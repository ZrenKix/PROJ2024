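; Moving platform actor that travels between its start position and an offset, either from BeginPlay or when StartPlatform is called.
; A looping timeline, with play rate scaled by TravelTime, lerps the location without sweep.
; A separate ColorChange timeline animates the Stone material's AlphaBlend parameter.
; BeginPlay requests a load from BP_GameInstance, and save/load events persist StartInMoveState under a Guid generated in the construction script.
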(event Custom|ColorChange
  (bind _newtrack_0 (Timeline|Timeline_0 Play)
    (:Update
      (Rendering|Material|SetScalarParameterValueonMaterials (Variables|Default|GetStone) "AlphaBlend" _newtrack_0))))

(event Custom|StartPlatform
  (bind _startpos (Variables|Default|GetStartPos))
  (Components|Timeline|SetLooping (Variables|Default|GetTimeline) true)
  (Components|Timeline|SetPlayRate (Variables|Default|GetTimeline) (/ 1.0 (Variables|Default|GetTravelTime)))
  (bind _alpha (Timeline|Timeline Play)
    (:Update
      (Transformation|SetActorLocation (Math|Vector|Lerp(Vector) _startpos (+ _startpos (Variables|Default|GetMoveToPos)) _alpha) false false))))

(event EventBeginPlay
  ;[1 1 1] Request load
  (bind _asbp_game_instance (Utilities|Casting|CastToBP_GameInstance (Game|GetGameInstance)))
  (Default|RequestLoad _asbp_game_instance self)
  (Variables|Default|SetStartPos (Transformation|GetActorLocation))
  (if (Variables|Default|GetStartInMoveState)
    (Components|Timeline|SetLooping (Variables|Default|GetTimeline) true)
    (Components|Timeline|SetPlayRate (Variables|Default|GetTimeline) (/ 1.0 (Variables|Default|GetTravelTime)))
    (bind _alpha (Timeline|Timeline Play)
      (:Update
        (Transformation|SetActorLocation (Math|Vector|Lerp(Vector) (Variables|Default|GetStartPos) (+ (Variables|Default|GetStartPos) (Variables|Default|GetMoveToPos)) _alpha) false false)))))

(event EventLoadData
  (params (SaveGameRef :type BP%20Save%20Game%20Object%20Reference))
  (bind _guid (Variables|Default|GetGuid))
  (bind _spawnableactors (Variables|/Game/Assets/Save/BP_SaveGame.BP_SaveGame_C|GetSpawnableActors SaveGameRef))
  (bind (_value _returnvalue) (Utilities|Map|Find _spawnableactors _guid))
  ;[1 1 1] Load Data
  (if _returnvalue
    (Variables|Default|SetStartInMoveState _value)))

(event EventSaveData
  (params (SaveGameRef :type BP%20Save%20Game%20Object%20Reference))
  ;[1 1 1] Save Data
  (Utilities|Map|Add (Variables|/Game/Assets/Save/BP_SaveGame.BP_SaveGame_C|GetSpawnableActors SaveGameRef) (Variables|Default|GetGuid) (Variables|Default|GetStartInMoveState)))

(event EventTick
  (params (DeltaSeconds :type Float%20%28single-precision%29)))

(fn ConstructionScript
  (CallFunction|HandleGUID))

(fn HandleGUID
  (if (not (Guid|IsValidGuid (Variables|Default|GetGuid)))
    (Variables|Default|SetGuid (Guid|NewGuid))))