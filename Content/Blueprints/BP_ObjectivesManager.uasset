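; Objectives manager that steps the player through a bedtime sequence: close wardrobe, turn off lights, go to sleep, turn on bed light, sleep again.
; Step functions mark objectives complete, delay the next objective text, and toggle bed access and light interactability.
; LightOff checks every light's intensity to detect completion.
; The first bed attempt briefly freezes movement with placeholder scares, while the sleep cutscene clears widgets and has the GameMode fade to black.
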(event Custom|UpdateObjectiveText
  (params (NewObjective :type Text))
  ;[1 1 1] Update objective text
  (Utilities|FlowControl|Delay (Variables|Default|GetUpdateObjectiveDelay))
  (Variables|Default|SetCurrentObjective NewObjective)
  (Variables|Default|SetObjectiveComplete false))

(event EventBeginPlay
  ;[1 1 1] Begin Play
  (Variables|Default|SetCurrentObjective "Close wardrobe")
  (bind _asbp_player_hero (Utilities|Casting|CastToBP_PlayerHero (Game|GetPlayerCharacter 0)))
  (Variables|Default|SetPlayerRef _asbp_player_hero))

(event Collision|EventActorBeginOverlap
  (params (OtherActor :type Actor%20Object%20Reference)))

(fn ConstructionScript)

(fn WardrobeDone
  (Variables|Default|SetObjectiveComplete true)
  (CallFunction|UpdateObjectiveText "Turn off the lights")
  (Utilities|Time|SetTimerbyFunctionName 0 "EnableLights" (Variables|Default|GetUpdateObjectiveDelay))
  (CallFunction|EnableLights))

(fn LightOff
  (for _array_element (Variables|Default|GetLights)
    (if (not (<= (Variables|/Script/Engine.LightComponentBase|GetIntensity (Variables|/Game/Blueprints/Interaction/BP_Lamp.BP_Lamp_C|GetPointLight _array_element)) 0.0))
      (LocalVariables|SetLightIsOff false)))
  (if (LocalVariables|GetLightIsOff)
    (Development|PrintString "all lights off")
    (CallFunction|AllLightsDone)
    (else
      (Development|PrintString "all lights not off"))))

(fn FirstTimeBed
  (Variables|Default|SetObjectiveComplete true)
  (Variables|Default|SetCanGoToBed false)
  (CallFunction|DisablePlayerMovement)
  (Development|PrintString "Play scary effects" true true "(R=1.000000,G=0.000000,B=0.772319,A=1.000000)")
  (Utilities|Time|SetTimerbyFunctionName 0 "EnablePlayerMovement" 2.0)
  (Utilities|Time|SetTimerbyFunctionName 0 "TurnOnBedLight" 2.0))

(fn DisablePlayerMovement
  (Pawn|Components|CharacterMovement|DisableMovement (Variables|/Script/Engine.Character|GetCharacterMovement (Game|GetPlayerCharacter 0))))

(fn EnablePlayerMovement
  (Pawn|Components|CharacterMovement|SetMovementMode (Variables|/Script/Engine.Character|GetCharacterMovement (Game|GetPlayerCharacter 0)) "MOVE_Walking" 0)
  (Development|PrintString "You can walk again" true true "(R=1.000000,G=0.000000,B=0.771030,A=1.000000)"))

(fn TurnonBedLight
  (CallFunction|UpdateObjectiveText "Turn on the bed light")
  (for _array_element (Variables|Default|GetLights)
    (if (Actor|ActorHasTag _array_element "BedLight")
      (Variables|/Game/Blueprints/Interaction/BP_Lamp.BP_Lamp_C|SetisInteractable? _array_element true))))

(fn AllLightsDone
  (Variables|Default|SetObjectiveComplete true)
  (Variables|Default|SetCanGoToBed true)
  (CallFunction|UpdateObjectiveText "Go to sleep."))

(fn EnableLights
  (for _array_element (Variables|Default|GetLights)
    (Variables|/Game/Blueprints/Interaction/BP_Lamp.BP_Lamp_C|SetisInteractable? _array_element true)))

(fn BedLightDone
  (Variables|Default|SetObjectiveComplete true)
  (Variables|Default|SetCanGoToBed true)
  (CallFunction|UpdateObjectiveText "Go to sleep."))

(fn StartSleepCutscene
  (CallFunction|DisablePlayerMovement)
  (Viewport|RemoveAllWidgets)
  (bind _asbp_tutorial_game_mode (Utilities|Casting|CastToBP_TutorialGameMode (Game|GetGameMode)))
  (Default|FadetoBlack _asbp_tutorial_game_mode))