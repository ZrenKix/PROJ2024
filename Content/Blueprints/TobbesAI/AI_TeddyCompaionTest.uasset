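; AI_TeddyCompaionTest is a test AI companion that follows the player hero.
; BeginPlay caches the player's BP_PlayerHero and its own BP_AIController, which receives the follow actor and companion state.
; Follow ignores its FollowTarget input in favour of the cached hero, while Wait only switches the state.
; Tick calls Follow every frame, so any Wait state is overwritten on the next tick.
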(event Custom|Follow
  (params (FollowTarget :type Actor%20Object%20Reference))
  (Default|SetFollowActor (Variables|Default|GetAs%20BP%20AIController) (Variables|Default|GetAs%20BP%20Player%20Hero))
  (Default|SetCompanionState (Variables|Default|GetAs%20BP%20AIController) "NewEnumerator1"))

(event Custom|Wait
  (Default|SetCompanionState (Variables|Default|GetAs%20BP%20AIController) "NewEnumerator0"))

(event EventBeginPlay
  (Utilities|FlowControl|Sequence
    (:then_0
      (bind _asbp_player_hero (Utilities|Casting|CastToBP_PlayerHero (Game|GetPlayerCharacter 0)))
      (Variables|Default|SetAs%20BP%20Player%20Hero _asbp_player_hero))
    (:then_1
      (bind _asbp_aicontroller (Utilities|Casting|CastToBP_AIController (AI|GetAIController self)))
      (Variables|Default|SetAs%20BP%20AIController _asbp_aicontroller))))

(event EventTick
  (params (DeltaSeconds :type Float%20%28single-precision%29))
  (CallFunction|Follow))

(fn ConstructionScript)