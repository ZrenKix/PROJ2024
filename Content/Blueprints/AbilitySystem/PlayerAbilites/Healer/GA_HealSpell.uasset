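; GA_HealSpell is a healer ability that casts a healing spell on a clicked hero unit in turn-based play.
; On input press, a mouse-cursor trace repeats until it hits a HeroUnit, which is flagged as having attacked and receives GE_AOEHeal.
; The owner's mana changes by ManaCost as Niagara, montage and sound play.
; A montage gameplay event, after a short delay, ends the controller's action and the ability.
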(event Ability|EventActivateAbility
  (bind _returnvalue (Game|GetPlayerController 0))
  (bind (_worldlocation _worlddirection) (Game|Player|ConvertMouseLocationToWorldSpace _returnvalue))
  (Ability|Tasks|WaitInputPress false :!label _label
    (:OnPress
      (bind _outhit (Collision|LineTraceByChannel _worldlocation (+ _worldlocation (* _worlddirection 1e+04)) "TraceTypeQuery1" false 0 "None"))
      (bind _ashero_unit (Utilities|Casting|CastToHeroUnit (.HitActor (Collision|BreakHitResult _outhit)))
        (:then
          (Class|HeroUnit|SetHasAttackedThisTurn _ashero_unit true)
          (|ChangeMana_2)
          (Class|UnitBase|ApplyEffecttoSelf _ashero_unit "/Game/Blueprints/AbilitySystem/PlayerAbilites/Healer/GE_AOEHeal.GE_AOEHeal_C" 1.0)
          (Niagara|SpawnSystematLocation "/Game/VFX/Niagara/Systems/Attacks/Artist/NS_Healing.NS_Healing" (+ (Transformation|GetActorLocation (.HitActor (Collision|BreakHitResult _outhit))) (Math|Vector|MakeVector (Variables|Default|GetHealLocX) 25.0 (Variables|Default|GetHealLocZ))))
          (|PlayMontageandWaitProxy "None" "/Game/Assets/Animations/Vincent/Animations/AM_VincentHealingAbility.AM_VincentHealingAbility" 1.0 "None" true 1.0 0.0 false
            (:then
              (Class|FMODBlueprintStatics|PlayEvent2D "/Game/FMOD/Events/Combat/PartyAbilities/Healer/Heal.Heal")
              (Ability|Tasks|WaitGameplayEvent "(TagName=\"Event.Montage.HealerAbility\")" 0
                (:EventReceived
                  (Utilities|FlowControl|Delay 0.2)
                  (bind _asarena_player_controller (Utilities|Casting|CastToArenaPlayerController (Game|GetPlayerController 0)))
                  (Class|ArenaPlayerController|OnActionEnd _asarena_player_controller)
                  (Ability|EndAbility))))))
        (:CastFailed
          (goto _label))))))

(event Ability|EventOnEndAbility
  (params (bWasCancelled :type Boolean)))