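; Healer player ability (GA_ChainHeal) that targets every HeroUnit in the level with a healing effect.
; It applies the mana cost, then loops over heroes, spawning Niagara effects and starting the montage and sound inside the loop.
; Each montage event spawns BP_Potion at the shared Hero variable, which holds the last hero by then.
; After a short delay it signals action end to the ArenaPlayerController and ends the ability.
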(event Ability|EventActivateAbility
  (|ChangeMana)
  (bind _outactors (Actor|GetAllActorsOfClass "/Script/PROJ.HeroUnit"))
  (for _array_element _outactors
    (bind _output_get (Variables|Default|SetHero _array_element))
    (Niagara|SpawnSystematLocation "/Game/VFX/Niagara/Systems/Attacks/Artist/NS_Healing.NS_Healing" (+ (Transformation|GetActorLocation _output_get) (Math|Vector|MakeVector (Variables|Default|GetHealingLocation) 0.0 85.0)))
    (|PlayMontageandWaitProxy "None" "/Game/Assets/Animations/Vincent/Animations/AM_HealingAbility.AM_HealingAbility" 1.0 "None" true 1.0 0.0 false
      (:then
        (Class|FMODBlueprintStatics|PlayEvent2D "/Game/FMOD/Events/Combat/PartyAbilities/Healer/Heal.Heal")
        (Ability|Tasks|WaitGameplayEvent "(TagName=\"Event.Montage.HealerAbility\")" 0
          (:EventReceived
            (Game|SpawnActorfromClass "/Game/Blueprints/Testing/BP_Potion.BP_Potion_C" (Math|Conversions|ToTransform(Vector) (Transformation|GetActorLocation _output_get)) "AlwaysSpawn" "MultiplyWithRoot" 0 0)
            (Utilities|FlowControl|Delay 0.2)
            (bind _asarena_player_controller (Utilities|Casting|CastToArenaPlayerController (Game|GetPlayerController 0)))
            (Class|ArenaPlayerController|OnActionEnd _asarena_player_controller)
            (Ability|EndAbility)))))))

(event Ability|EventOnEndAbility
  (params (bWasCancelled :type Boolean)))