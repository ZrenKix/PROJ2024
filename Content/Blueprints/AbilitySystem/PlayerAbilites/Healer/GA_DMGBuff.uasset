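; Healer gameplay ability that grants a damage buff to a HeroUnit picked with the mouse.
; On input press it line-traces under the cursor, re-arming until it hits a HeroUnit, then starts the target's buff effect and the buff montage.
; The montage's gameplay event spends the owner's mana; after a short delay it applies GE_DMGBuff, flags the target as having attacked, notifies ArenaPlayerController and ends.
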(event Ability|EventOnEndAbility
  (params (bWasCancelled :type Boolean)))

(event Ability|EventActivateAbility
  (Ability|Tasks|WaitInputPress false :!label _label
    (:OnPress
      (bind (_worldlocation _returnvalue) (CallFunction|GetMouseLocation))
      (bind _outhit (Collision|LineTraceByChannel _worldlocation _returnvalue "TraceTypeQuery1" false 0 "None" false))
      (bind _ashero_unit (Utilities|Casting|CastToHeroUnit (.HitActor (Collision|BreakHitResult _outhit)))
        (:then
          (Class|HeroUnit|StartDMGBuffEffect _ashero_unit)
          (|PlayMontageandWaitProxy "None" "/Game/Assets/Animations/Vincent/Animations/AM_Buff.AM_Buff" 1.0 "None" true 1.0 0.0 false
            (:then
              (Ability|Tasks|WaitGameplayEvent "(TagName=\"Event.Montage.Buff\")" 0
                (:then
                  (|ChangeMana_2)
                  (Utilities|FlowControl|Delay 2.0)
                  (CallFunction|AddBuffTag (.HitActor (Collision|BreakHitResult _outhit))))))))
        (:CastFailed
          (goto _label))))))

(fn GetMouseLocation
  (bind _returnvalue (Game|GetPlayerController 0))
  (bind (_worldlocation _worlddirection) (Game|Player|ConvertMouseLocationToWorldSpace _returnvalue))
  (return _worldlocation (+ _worldlocation (* _worlddirection 1e+04))))

(fn AddBuffTag
  (params (Object :type Object%20Object%20Reference))
  (bind _ashero_unit (Utilities|Casting|CastToHeroUnit Object))
  (Class|HeroUnit|SetHasAttackedThisTurn _ashero_unit true)
  (GameplayEffects|ApplyGameplayEffectToTarget (Ability|TargetData|AbilityTargetDatafromActor _ashero_unit) "/Game/Blueprints/AbilitySystem/GameplayEffects/GE_DMGBuff.GE_DMGBuff_C" 1 1)
  (bind _asarena_player_controller (Utilities|Casting|CastToArenaPlayerController (Game|GetPlayerController 0)))
  (Class|ArenaPlayerController|OnActionEnd _asarena_player_controller)
  (Ability|EndAbility))