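; Archer gameplay ability Rain of Arrows that hits every BP_Enemy actor in the level.
; On activation it loops over those enemies, spawning the arrow-rain Niagara effect at each and applying the damage gameplay effect.
; A short Delay and EndAbility sit inside the loop body, so the ability only ends when an enemy exists.
; Unconnected leftovers hold a mouse-targeted magic circle with debug-drawn ground points and a SetByCaller fire damage spec.
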(event Ability|EventActivateAbility
  (bind _outactors (Actor|GetAllActorsOfClass "/Game/Blueprints/Characters/Enemies/BP_Enemy.BP_Enemy_C"))
  (for _array_element _outactors
    (bind _output_get (Variables|Default|SetArray%20Element _array_element))
    (Niagara|SpawnSystematLocation "/Game/VFX/Niagara/Systems/Attacks/NS_RainOfArrows.NS_RainOfArrows" (Transformation|GetActorLocation _output_get))
    (GameplayEffects|ApplyGameplayEffectToTarget (Ability|TargetData|AbilityTargetDatafromActor _output_get) (Variables|Default|GetDamageEffectClass) 1 1)
    (Utilities|FlowControl|Delay 0.2)
    (Ability|EndAbility)))

(event Ability|EventOnEndAbility
  (params (bWasCancelled :type Boolean)))