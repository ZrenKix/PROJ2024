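; GA_SmallSingle is an Archer gameplay ability that lets a small shadow unit strike its single target hero.
; On activation it spawns the rain-of-arrows Niagara effect at the hero and applies the damage gameplay effect.
; After a short delay it notifies the arena player controller that the action ended, then prints the hero's health and ends.
; Failed avatar or controller casts only print, leaving the ability unended.
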(event Ability|EventActivateAbility
  (Development|PrintString "Start")
  (bind _asbp_small_shadow_unit (Utilities|Casting|CastToBP_SmallShadowUnit (Ability|GetAvatarActorfromActorInfo))
    (:then
      (Niagara|SpawnSystematLocation "/Game/VFX/Niagara/Systems/Attacks/Archer/NS_RainOfArrows.NS_RainOfArrows" (Transformation|GetActorLocation (Variables|/Script/PROJ.SmallShadowUnit|GetTargetHero _asbp_small_shadow_unit)))
      (GameplayEffects|ApplyGameplayEffectToTarget (Ability|TargetData|AbilityTargetDatafromActor (Variables|/Script/PROJ.SmallShadowUnit|GetTargetHero _asbp_small_shadow_unit)) (Variables|Default|GetDamageEffectClass) 1 1)
      (Utilities|FlowControl|Delay 0.5)
      (Development|PrintString "delayed and ending ability")
      (bind _asarena_player_controller (Utilities|Casting|CastToArenaPlayerController (Game|GetPlayerController 0))
        (:then
          (Class|ArenaPlayerController|OnActionEnd _asarena_player_controller)
          (Development|PrintString "called on action end")
          (Development|PrintString "ended ability")
          (Utilities|FlowControl|Delay 0.2)
          (bind _returnvalue (GameplayAttributes|GetAttributeSet (Ability|GetAbilitySystemComponent (Variables|/Script/PROJ.SmallShadowUnit|GetTargetHero _asbp_small_shadow_unit)) "/Script/PROJ.ProjAttributeSet"))
          (bind _asproj_attribute_set (Utilities|Casting|CastToProjAttributeSet _returnvalue))
          (Development|PrintString "New health")
          (Development|PrintString (Utilities|String|ToString(Float) (.CurrentValue (Utilities|Struct|BreakGameplayAttributeData (Variables|/Script/PROJ.ProjAttributeSet|GetHealth _asproj_attribute_set)))))
          (Ability|EndAbility))
        (:CastFailed
          (Development|PrintString "cast failed???"))))
    (:CastFailed
      (Development|PrintString "Faliled cast"))))

(event Ability|EventOnEndAbility
  (params (bWasCancelled :type Boolean)))