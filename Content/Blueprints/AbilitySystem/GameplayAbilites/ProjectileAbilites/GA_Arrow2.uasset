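; GA_Arrow2 is a projectile Gameplay Ability for a turn-based hero's basic attack, using Edith's montage.
; It waits for input, traces under the cursor and re-arms until the hit actor implements TargetInterface.
; It then flags the hero as having attacked and plays the montage.
; The montage's gameplay event spawns the projectile, changes mana, removes the damage buff and, after a delay, ends the action and ability.
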(event Ability|EventActivateAbility
  (bind _returnvalue (Game|GetPlayerController 0))
  (bind (_worldlocation _worlddirection) (Game|Player|ConvertMouseLocationToWorldSpace _returnvalue))
  (Ability|Tasks|WaitInputPress false :!label _label
    (:OnPress
      (Development|PrintString "doing the bear attack")
      (bind _outhit (Collision|LineTraceByChannel _worldlocation (+ _worldlocation (* _worlddirection 1e+04)) "TraceTypeQuery1" false 0 "None"))
      (if (Utilities|DoesObjectImplementInterface (.HitActor (Collision|BreakHitResult _outhit)) "/Script/PROJ.TargetInterface")
        (bind _ashero_unit (Utilities|Casting|CastToHeroUnit (Pawn|GetControlledPawn _returnvalue)))
        (Class|HeroUnit|SetHasAttackedThisTurn _ashero_unit true)
        (Variables|Default|SetProjectileTargetLocation (.Location (Collision|BreakHitResult _outhit)))
        (|PlayMontageandWaitProxy "None" "/Game/Assets/Animations/Edith/AnimationMontages/AM_EdithBasic.AM_EdithBasic" 1.0 "None" true 1.0 0.0 false
          (:then
            (Ability|Tasks|WaitGameplayEvent "(TagName=\"Event.Montage.EdithBA\")" 0
              (:EventReceived
                (Class|DBProjectileSpell|SpawnProjectile (Variables|Default|GetProjectileTargetLocation))
                (|ChangeMana)
                (Class|HeroUnit|RemoveDMGBuff _ashero_unit)
                (Utilities|FlowControl|Delay 0.5)
                (bind _asarena_player_controller (Utilities|Casting|CastToArenaPlayerController (Game|GetPlayerController 0)))
                (Class|ArenaPlayerController|OnActionEnd _asarena_player_controller)
                (Ability|EndAbility)))))
        (else
          (goto _label))))))

(event Ability|EventOnEndAbility
  (params (bWasCancelled :type Boolean))
  (Development|PrintString "Ability Ended"))