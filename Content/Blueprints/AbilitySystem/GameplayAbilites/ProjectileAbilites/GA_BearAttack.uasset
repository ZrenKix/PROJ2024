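; Gameplay ability for the Teddy hero's bear attack, a projectile attack on a target picked with the mouse.
; On input press, a cursor trace accepts actors implementing TargetInterface, flags the hero as having attacked this turn and sets an aim rotation on ABP_Teddy.
; The montage's notify spawns the projectile toward the hit point.
; Montage callbacks also apply mana cost, remove the damage buff, end the action and reset the aim.
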(event Ability|EventActivateAbility
  (bind _returnvalue (Game|GetPlayerController 0))
  (bind _returnvalue_2 (Pawn|GetControlledPawn _returnvalue))
  (bind (_worldlocation _worlddirection) (Game|Player|ConvertMouseLocationToWorldSpace _returnvalue))
  (Ability|Tasks|WaitInputPress false
    (:OnPress
      (Development|PrintString "doing the bear attack")
      (bind _outhit (Collision|LineTraceByChannel _worldlocation (+ _worldlocation (* _worlddirection 1e+04)) "TraceTypeQuery1" false 0 "None"))
      (if (Utilities|DoesObjectImplementInterface (.HitActor (Collision|BreakHitResult _outhit)) "/Script/PROJ.TargetInterface")
        (bind _ashero_unit (Utilities|Casting|CastToHeroUnit _returnvalue_2))
        (Class|HeroUnit|SetHasAttackedThisTurn _ashero_unit true)
        (bind _output_get (Variables|Default|SetProjectileTargetLocation (.Location (Collision|BreakHitResult _outhit))))
        (Development|PrintString "still doing the bear attack")
        (bind (_mesh _asabp_teddy) (|SetRotationTeddy _returnvalue_2 (.ReturnValue (|CalculateRotation (stale _mesh) _output_get)) (.ReturnValue2 (|CalculateRotation (stale _mesh) _output_get)) (.ReturnValue3 (|CalculateRotation (stale _mesh) _output_get)))
          (:then
            _)
          (:then2
            _))
        (bind _notifyname (Animation|Montage|PlayMontage _mesh "/Game/Assets/Animations/Teddy/Animations/AM_TeddyBasic.AM_TeddyBasic")
          (:then
            (|ChangeMana)
            (Class|HeroUnit|RemoveDMGBuff _ashero_unit))
          (:OnBlendOut
            (bind _asarena_player_controller (Utilities|Casting|CastToArenaPlayerController (Game|GetPlayerController 0)))
            (Class|ArenaPlayerController|OnActionEnd _asarena_player_controller)
            (Variables|/Game/Assets/Animations/Teddy/ABP_Teddy.ABP_Teddy_C|SetTargetRotation _asabp_teddy "0, 0, 0")
            (Ability|EndAbility))
          (:OnNotifyBegin
            (switch name _notifyname
              (:Attack
                (Class|DBProjectileSpell|SpawnProjectile (Variables|Default|GetProjectileTargetLocation))
                (Development|PrintString "did the bear attack")))))
        (else
          (Development|PrintString "actor does not implement interface")
          (Ability|EndAbility))))))

(event Ability|EventOnEndAbility
  (params (bWasCancelled :type Boolean))
  (Development|PrintString "Ability Ended"))