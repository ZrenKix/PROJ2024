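; Gameplay ability that lets the player taunt a clicked shadow unit, using the Teddy taunt montage.
; On input press it traces under the cursor, cancelling if the hit lacks TargetInterface.
; A BP_SmallShadowUnit hit receives the taunt effect, Taunted tag and Niagara burst.
; The caster's montage starts, mana changes via ManaCost, and blend-out notifies the arena controller of action end and ends the ability.
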(event Ability|EventActivateAbility
  (bind _returnvalue (Game|GetPlayerController 0))
  (bind (_worldlocation _worlddirection) (Game|Player|ConvertMouseLocationToWorldSpace _returnvalue))
  (Ability|Tasks|WaitInputPress true
    (:OnPress
      (bind _outhit (Collision|LineTraceByChannel _worldlocation (+ _worldlocation (* _worlddirection 1e+04)) "TraceTypeQuery1" false 0 "None"))
      (if (Utilities|DoesObjectImplementInterface (.HitActor (Collision|BreakHitResult _outhit)) "/Script/PROJ.TargetInterface")
        (bind _asbp_small_shadow_unit (Utilities|Casting|CastToBP_SmallShadowUnit (.HitActor (Collision|BreakHitResult _outhit))))
        (GameplayEffects|ApplyGameplayEffectToTarget (Ability|TargetData|AbilityTargetDatafromActor (.HitActor (Collision|BreakHitResult _outhit))) "/Game/Blueprints/AbilitySystem/GameplayEffects/GE_TauntEffect.GE_TauntEffect_C" 1 1)
        (GameplayTags|AddGameplayTag (Variables|/Game/Blueprints/Arena/Units/Enemies/BP_SmallShadowUnit.BP_SmallShadowUnit_C|GetGameplayTags _asbp_small_shadow_unit) "(TagName=\"States.Taunted\")" :!class /Script/GameplayTags.BlueprintGameplayTagLibrary)
        (Niagara|SpawnSystematLocation "/Game/VFX/Niagara/Systems/Attacks/Bear/NS_TauntHit.NS_TauntHit" (.Location (Collision|BreakHitResult _outhit)))
        (bind _ascharacter (Utilities|Casting|CastToCharacter (Pawn|GetControlledPawn _returnvalue)))
        (bind _notifyname (Animation|Montage|PlayMontage (Variables|/Script/Engine.Character|GetMesh _ascharacter) "/Game/Assets/Animations/Teddy/Animations/AS_TeddyTaunt_Anim_Montage.AS_TeddyTaunt_Anim_Montage")
          (:then
            (|ChangeMana))
          (:OnBlendOut
            (bind _asarena_player_controller (Utilities|Casting|CastToArenaPlayerController (Game|GetPlayerController 0)))
            (Class|ArenaPlayerController|OnActionEnd _asarena_player_controller)
            (Ability|EndAbility))
          (:OnNotifyBegin
            (switch name _notifyname)))
        (else
          (Ability|CancelAbility)
          (Ability|EndAbility))))))

(event Ability|EventOnEndAbility
  (params (bWasCancelled :type Boolean)))