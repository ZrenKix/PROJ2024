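; GA_Arrow is a gameplay ability that fires a projectile at the point the player targets with the mouse cursor.
; On activation it waits for an input press, line traces from the deprojected cursor and passes the hit location to SpawnProjectile.
; It then commits the cooldown, briefly delays, notifies the ArenaPlayerController that the action ended and ends itself.
; A TargetInterface check on the hit actor is present but disconnected.
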(event Ability|EventActivateAbility
  (bind _returnvalue (Game|GetPlayerController 0))
  (bind (_worldlocation _worlddirection) (Game|Player|ConvertMouseLocationToWorldSpace _returnvalue))
  (Ability|Tasks|WaitInputPress false
    (:OnPress
      (bind _outhit (Collision|LineTraceByChannel _worldlocation (+ _worldlocation (* _worlddirection 1e+04)) "TraceTypeQuery1" false 0 "None"))
      (Variables|Default|SetProjectileTargetLocation (.Location (Collision|BreakHitResult _outhit)))
      (Class|DBProjectileSpell|SpawnProjectile (Variables|Default|GetProjectileTargetLocation))
      (Ability|CommitAbilityCooldown false true)
      (Utilities|FlowControl|Delay 0.5)
      (bind _asarena_player_controller (Utilities|Casting|CastToArenaPlayerController (Game|GetPlayerController 0)))
      (Class|ArenaPlayerController|OnActionEnd _asarena_player_controller)
      (Ability|EndAbility))))

(event Ability|EventOnEndAbility
  (params (bWasCancelled :type Boolean))
  (Development|PrintString "Ability Ended"))