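; Gameplay ability for the healer's basic projectile spell, aimed with the mouse.
; On input press it traces under the cursor, requires a TargetInterface actor, pitches the Vincent anim blueprint toward the hit using the clamped X offset, and plays the attack montage.
; The Attack notify spawns the projectile, applies the mana cost and commits cooldown, then after a short delay signals action end, resets rotation and ends the ability.
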(event Ability|EventActivateAbility
  (bind _returnvalue (Game|GetPlayerController 0))
  (bind (_worldlocation _worlddirection) (Game|Player|ConvertMouseLocationToWorldSpace _returnvalue))
  (Ability|Tasks|WaitInputPress false
    (:OnPress
      (bind _outhit (Collision|LineTraceByChannel _worldlocation (+ _worldlocation (* _worlddirection 1e+04)) "TraceTypeQuery1" false 0 "None"))
      (if (Utilities|DoesObjectImplementInterface (.HitActor (Collision|BreakHitResult _outhit)) "/Script/PROJ.TargetInterface")
        (bind _output_get (Variables|Default|SetProjectileTargetLocation (.Location (Collision|BreakHitResult _outhit))))
        (bind _ascharacter (Utilities|Casting|CastToCharacter (Pawn|GetControlledPawn _returnvalue)))
        (bind _asabp_vincent (Utilities|Casting|CastToABP_Vincent (Components|SkeletalMesh|GetAnimInstance (Variables|/Script/Engine.Character|GetMesh _ascharacter))))
        (Development|PrintString (Utilities|String|ToString(Float) (- (.X (Math|Vector|BreakVector (Transformation|GetSocketLocation (Variables|/Script/Engine.Character|GetMesh _ascharacter) "bodySocket"))) (.X (Math|Vector|BreakVector _output_get)))))
        (if (<= (Math|Float|Absolute(Float) (- (.X (Math|Vector|BreakVector (Transformation|GetSocketLocation (Variables|/Script/Engine.Character|GetMesh _ascharacter) "bodySocket"))) (.X (Math|Vector|BreakVector _output_get)))) 1.5e+02)
          (Variables|/Game/Assets/Animations/Vincent/ABP_Vincent.ABP_Vincent_C|SetTargetRotatin _asabp_vincent (Math|Rotator|MakeRotator 0.0 (Math|Float|Clamp(Float) (- (.X (Math|Vector|BreakVector (Transformation|GetSocketLocation (Variables|/Script/Engine.Character|GetMesh _ascharacter) "bodySocket"))) (.X (Math|Vector|BreakVector _output_get))) 0.0 0.0) 0.0))
          (else
            (Variables|/Game/Assets/Animations/Vincent/ABP_Vincent.ABP_Vincent_C|SetTargetRotatin _asabp_vincent (Math|Rotator|MakeRotator 0.0 (Math|Float|Clamp(Float) (- (.X (Math|Vector|BreakVector (Transformation|GetSocketLocation (Variables|/Script/Engine.Character|GetMesh _ascharacter) "bodySocket"))) (.X (Math|Vector|BreakVector _output_get))) -5e+01 5e+01) 0.0))))
        (bind _notifyname (Animation|Montage|PlayMontage (Variables|/Script/Engine.Character|GetMesh _ascharacter) "/Game/Assets/Animations/Vincent/Animations/AM_VincentBasic.AM_VincentBasic")
          (:OnNotifyBegin
            (if (== _notifyname "Attack")
              (Class|DBProjectileSpell|SpawnProjectile (Variables|Default|GetProjectileTargetLocation))
              (|ChangeMana)
              (Ability|CommitAbilityCooldown false true)
              (Utilities|FlowControl|Delay 0.5)
              (bind _asarena_player_controller (Utilities|Casting|CastToArenaPlayerController (Game|GetPlayerController 0)))
              (Class|ArenaPlayerController|OnActionEnd _asarena_player_controller)
              (Variables|/Game/Assets/Animations/Vincent/ABP_Vincent.ABP_Vincent_C|SetTargetRotatin _asabp_vincent "0, 0, 0")
              (Ability|EndAbility))))
        (else
          (Development|PrintString "actor does not implement interface")
          (Ability|EndAbility))))))

(event Ability|EventOnEndAbility
  (params (bWasCancelled :type Boolean))
  (Development|PrintString "Ability Ended"))