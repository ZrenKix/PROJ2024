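; Gameplay ability for the Dark Bob unit's single-target basic attack on its TargetHero.
; On activation it spawns a mini Niagara effect at the hero and immediately applies the damage gameplay effect, with no projectile spawned.
; After short delays it notifies the ArenaPlayerController that the action ended, prints the hero's Health from ProjAttributeSet, then ends the ability.
; Debug prints trace each step and failed cast.
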(event Ability|EventActivateAbility
  (Development|PrintString "Start")
  (bind _asbp_dark_bob_unit (Utilities|Casting|CastToBP_DarkBobUnit (Ability|GetAvatarActorfromActorInfo))
    (:then
      _)
    (:CastFailed
      (Development|PrintString "Faliled cast")))
  (Niagara|SpawnSystematLocation "/Game/VFX/Niagara/Systems/Mini_Boss/NG_BasicAttack_Mini.NG_BasicAttack_Mini" (Transformation|GetActorLocation (Variables|/Script/PROJ.DarkBobUnit|GetTargetHero _asbp_dark_bob_unit)))
  (GameplayEffects|ApplyGameplayEffectToTarget (Ability|TargetData|AbilityTargetDatafromActor (Variables|/Script/PROJ.DarkBobUnit|GetTargetHero _asbp_dark_bob_unit)) (Variables|Default|GetDamageEffectClass) 1 1)
  (Utilities|FlowControl|Delay 0.5)
  (Development|PrintString "delayed and ending ability")
  (bind _asarena_player_controller (Utilities|Casting|CastToArenaPlayerController (Game|GetPlayerController 0))
    (:then
      (Class|ArenaPlayerController|OnActionEnd _asarena_player_controller)
      (Development|PrintString "called on action end")
      (Development|PrintString "ended ability")
      (Utilities|FlowControl|Delay 0.2)
      (bind _returnvalue (GameplayAttributes|GetAttributeSet (Ability|GetAbilitySystemComponent (Variables|/Script/PROJ.DarkBobUnit|GetTargetHero _asbp_dark_bob_unit)) "/Script/PROJ.ProjAttributeSet"))
      (bind _asproj_attribute_set (Utilities|Casting|CastToProjAttributeSet _returnvalue))
      (Development|PrintString "New health")
      (Development|PrintString (Utilities|String|ToString(Float) (.CurrentValue (Utilities|Struct|BreakGameplayAttributeData (Variables|/Script/PROJ.ProjAttributeSet|GetHealth _asproj_attribute_set)))))
      (Ability|EndAbility))
    (:CastFailed
      (Development|PrintString "cast failed???"))))