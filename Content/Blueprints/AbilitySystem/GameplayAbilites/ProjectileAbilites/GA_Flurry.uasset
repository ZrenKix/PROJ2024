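; GA_Flurry is a hero ability that collects clicked targets up to TargetLimit for a flurry attack.
; Chained input waits trace under the mouse, adding and highlighting TargetInterface actors.
; Only completion on the third click spends mana, marks the hero as having attacked, and applies set-by-caller fire damage on a montage event.
; Earlier completions only play VFX and montage before ending the turn; a fourth click triggers nothing further.
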(event Ability|EventActivateAbility
  (Ability|Tasks|WaitInputPress false :!label _label
    (:OnPress
      (bind _actoradded (CallFunction|AddActortoList))
      (if _actoradded
        (bind _targetcomplete (CallFunction|CheckAbilityState))
        (if _targetcomplete
          (CallFunction|SpawnVFX)
          (Animation|Montage|PlayMontage 0 "/Game/Assets/Animations/Teddy/Animations/AM_TeddyBasic.AM_TeddyBasic"
            (:OnBlendOut
              (CallFunction|EndTurn)))
          (else
            (Utilities|FlowControl|Delay 0.1)
            (Ability|Tasks|WaitInputPress false :!label _label_2
              (:OnPress
                (bind _actoradded_2 (CallFunction|AddActortoList))
                (if _actoradded_2
                  (bind _targetcomplete_2 (CallFunction|CheckAbilityState))
                  (if _targetcomplete_2
                    (CallFunction|SpawnVFX)
                    (Animation|Montage|PlayMontage 0 "/Game/Assets/Animations/Teddy/Animations/AM_TeddyBasic.AM_TeddyBasic"
                      (:OnBlendOut
                        (CallFunction|EndTurn)))
                    (else
                      (Utilities|FlowControl|Delay 0.1)
                      (Ability|Tasks|WaitInputPress false :!label _label_3
                        (:OnPress
                          (bind _actoradded_3 (CallFunction|AddActortoList))
                          (if _actoradded_3
                            (bind _targetcomplete_3 (CallFunction|CheckAbilityState))
                            (if _targetcomplete_3
                              (bind _ashero_unit (Utilities|Casting|CastToHeroUnit (Game|Player|GetPlayerPawn 0)))
                              (Class|HeroUnit|SetHasAttackedThisTurn _ashero_unit true)
                              (|ChangeMana_2)
                              (|PlayMontageandWaitProxy "None" "/Game/Assets/Animations/Teddy/Animations/AM_TeddyBasic.AM_TeddyBasic" 1.0 "None" true 1.0 0.0 false
                                (:then
                                  (Ability|Tasks|WaitGameplayEvent "(TagName=\"Event.Montage.Flurry\")" 0
                                    (:EventReceived
                                      (CallFunction|SpawnVFX)
                                      (for _array_element (Variables|Default|GetTargetList)
                                        (bind _returnvalue (Ability|GameplayEffect|AssignTagSetbyCallerMagnitude (Ability|MakeOutgoingGameplayEffectSpec (Variables|Default|GetDamageEffectClass)) "(TagName=\"Damage.Fire\")" 3.0))
                                        (GameplayEffects|ApplyGameplayEffectSpecToTarget _returnvalue (Ability|TargetData|AbilityTargetDatafromActor _array_element))
                                        (Camera|PlayWorldCameraShake "/Game/Blueprints/Camera/BP_CamShakeFlurry.BP_CamShakeFlurry_C" (Transformation|GetActorLocation (Game|Player|GetPlayerPawn 0)) 0.0 5e+04 1.0 true)
                                        (bind _asunit_paper_base (Utilities|Casting|CastToUnitPaperBase _array_element))
                                        (Class|UnitPaperBase|ClearTarget _asunit_paper_base)
                                        (Class|HeroUnit|RemoveDMGBuff _ashero_unit)
                                        (Utilities|FlowControl|Delay 0.2)
                                        (CallFunction|EndTurn))))))
                              (else
                                (Utilities|FlowControl|Delay 0.1)
                                (Ability|Tasks|WaitInputPress false :!label _label_4
                                  (:OnPress
                                    (bind _actoradded_4 (CallFunction|AddActortoList))
                                    (if _actoradded_4
                                      (CallFunction|CheckAbilityState)
                                      (else
                                        (goto _label_4)))))))
                            (else
                              (goto _label_3)))))))
                  (else
                    (goto _label_2)))))))
        (else
          (goto _label))))))

(event Ability|EventOnEndAbility
  (params (bWasCancelled :type Boolean)))

(fn AddActortoList
  (bind _returnvalue (Game|GetPlayerController 0))
  (bind (_worldlocation _worlddirection) (Game|Player|ConvertMouseLocationToWorldSpace _returnvalue))
  (bind _outhit (Collision|LineTraceByChannel _worldlocation (+ _worldlocation (* _worlddirection 1e+04)) "TraceTypeQuery1" false 0 "None"))
  (if (Utilities|DoesObjectImplementInterface (.HitActor (Collision|BreakHitResult _outhit)) "/Script/PROJ.TargetInterface")
    (Development|PrintString "actor does implement")
    (bind _result (Math|Integer|IncrementInt (Variables|Default|GetTargetsClicked))
      (:%20%20
        (Development|PrintString (Utilities|String|ToString(Integer) _result))
        (Utilities|Array|Add (Variables|Default|GetTargetList) (.HitActor (Collision|BreakHitResult _outhit)))
        (bind _asunit_paper_base (Utilities|Casting|CastToUnitPaperBase (.HitActor (Collision|BreakHitResult _outhit))))
        (Class|UnitPaperBase|OnTargetSet _asunit_paper_base)
        (return true)))
    (else
      (return false))))

(fn CheckAbilityState
  (return (== (Variables|Default|GetTargetsClicked) (Variables|Default|GetTargetLimit))))

(fn SpawnVFX
  (for _array_element (Variables|Default|GetTargetList)
    (Niagara|SpawnSystematLocation "/Game/VFX/Niagara/Systems/Attacks/Bear/NS_BearAttack.NS_BearAttack" (Transformation|GetActorLocation _array_element))))

(fn EndTurn
  (bind _asarena_player_controller (Utilities|Casting|CastToArenaPlayerController (Game|GetPlayerController 0)))
  (Class|ArenaPlayerController|OnActionEnd _asarena_player_controller)
  (Ability|EndAbility))