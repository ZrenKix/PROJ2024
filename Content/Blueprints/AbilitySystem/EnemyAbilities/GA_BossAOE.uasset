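; Boss area-attack gameplay ability that hits every HeroUnit in the level.
; On activation it spawns a rain-of-arrows Niagara effect at each hero and applies the damage GameplayEffect to them.
; A half-second Delay inside the loop leads to the arena player controller's OnActionEnd and EndAbility, with debug prints.
; A ChangeMana helper applies ManaCost to the owning unit but is never called.
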(event Ability|EventActivateAbility
  (bind _outactors (Actor|GetAllActorsOfClass "/Script/PROJ.HeroUnit"))
  (for _array_element _outactors
    (Niagara|SpawnSystematLocation "/Game/VFX/Niagara/Systems/Attacks/Archer/NS_RainOfArrows.NS_RainOfArrows" (Transformation|GetActorLocation _array_element))
    (GameplayEffects|ApplyGameplayEffectToTarget (Ability|TargetData|AbilityTargetDatafromActor _array_element) (Variables|Default|GetDamageEffectClass) 1 1)
    (Utilities|FlowControl|Delay 0.5)
    (Development|PrintString "delayed and ending ability")
    (bind _asarena_player_controller (Utilities|Casting|CastToArenaPlayerController (Game|GetPlayerController 0))
      (:then
        (Class|ArenaPlayerController|OnActionEnd _asarena_player_controller)
        (Development|PrintString "called on action end")
        (Ability|EndAbility)
        (Development|PrintString "ended ability"))
      (:CastFailed
        (Development|PrintString "cast failed???")))))

(event Ability|EventOnEndAbility
  (params (bWasCancelled :type Boolean)))