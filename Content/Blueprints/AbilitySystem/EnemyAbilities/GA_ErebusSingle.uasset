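; Gameplay ability for Erebus's single-target attack, used by the small shadow unit enemy in a turn-based fight.
; On activation it casts the avatar to BP_SmallShadowUnit, spawns a Niagara hit effect at its TargetHero and applies the damage effect class to that hero.
; It then prints the hero's new health from ProjAttributeSet for debugging, tells the unit its turn is finished and ends the ability.
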(event Ability|EventActivateAbility
  (Development|PrintString "Start")
  (bind _asbp_small_shadow_unit (Utilities|Casting|CastToBP_SmallShadowUnit (Ability|GetAvatarActorfromActorInfo))
    (:then
      (Niagara|SpawnSystematLocation "/Game/VFX/Niagara/Systems/LastBoss/NG_BasicAttack_Ere.NG_BasicAttack_Ere" (Transformation|GetActorLocation (Variables|/Script/PROJ.SmallShadowUnit|GetTargetHero _asbp_small_shadow_unit)))
      (GameplayEffects|ApplyGameplayEffectToTarget (Ability|TargetData|AbilityTargetDatafromActor (Variables|/Script/PROJ.SmallShadowUnit|GetTargetHero _asbp_small_shadow_unit)) (Variables|Default|GetDamageEffectClass) 1 1)
      (bind _returnvalue (GameplayAttributes|GetAttributeSet (Ability|GetAbilitySystemComponent (Variables|/Script/PROJ.SmallShadowUnit|GetTargetHero _asbp_small_shadow_unit)) "/Script/PROJ.ProjAttributeSet"))
      (bind _asproj_attribute_set (Utilities|Casting|CastToProjAttributeSet _returnvalue))
      (Development|PrintString "New health")
      (Development|PrintString (Utilities|String|ToString(Float) (.CurrentValue (Utilities|Struct|BreakGameplayAttributeData (Variables|/Script/PROJ.ProjAttributeSet|GetHealth _asproj_attribute_set)))))
      (Class|SmallShadowUnit|FinishedTurn _asbp_small_shadow_unit)
      (Ability|EndAbility))
    (:CastFailed
      (Development|PrintString "Faliled cast"))))

(event Ability|EventOnEndAbility
  (params (bWasCancelled :type Boolean)))