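; Trigger actor that plays a Level Sequence cutscene when the player hero overlaps its box, until it is marked done.
; When the sequence finishes, it disables the box collision, reveals the hidden Companion and sets CutsceneDone.
; It requests loading through the GameInstance on BeginPlay and persists CutsceneDone in the save game's Cutscenes map, keyed by GetSequenceName.
; Both save and load print the map's values for debugging.
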(event OnComponentBeginOverlap(Box)
  (params (OverlappedComponent :type Primitive%20Component%20Object%20Reference) (OtherActor :type Actor%20Object%20Reference) (OtherComp :type Primitive%20Component%20Object%20Reference) (OtherBodyIndex :type Integer) (bFromSweep :type Boolean) (SweepResult :type Hit%20Result%20Structure%20%28by%20ref%29))
  (bind _levelsequencer (Variables|Default|GetLevelSequencer))
  (bind _sequenceplayer (Variables|/Script/LevelSequence.LevelSequenceActor|GetSequencePlayer _levelsequencer))
  (if (not (Variables|Default|GetCutsceneDone))
    (Utilities|Casting|CastToBP_PlayerHero OtherActor)
    (Sequencer|Player|Play _sequenceplayer :!class /Script/MovieScene.MovieSceneSequencePlayer)
    (EventDispatchers|BindEventtoOnFinished _sequenceplayer (delegate Custom|CutsceneFinished))))

(event Custom|CutsceneFinished
  (Collision|SetCollisionEnabled (Variables|Default|GetBox) "NoCollision")
  (Rendering|SetActorHiddenInGame (Variables|Default|GetCompanion) false)
  (Variables|Default|SetCutsceneDone true))

(event EventSaveData
  (params (SaveGameRef :type BP%20Save%20Game%20Object%20Reference))
  ;[1 1 1] Save data
  (Utilities|Map|Add (Variables|/Game/Assets/Save/BP_SaveGame.BP_SaveGame_C|GetCutscenes SaveGameRef) (Utilities|GetSequenceName) (Variables|Default|GetCutsceneDone))
  ;[1 1 1] Load data
  (bind _values (Utilities|Map|Values (Variables|/Game/Assets/Save/BP_SaveGame.BP_SaveGame_C|GetCutscenes (stale EventLoadData SaveGameRef))))
  (for _array_element _values
    (Development|PrintString (Utilities|String|ToString(Boolean) _array_element) true true "(R=0.920018,G=1.000000,B=0.000000,A=1.000000)")))

(event EventLoadData
  (params (SaveGameRef :type BP%20Save%20Game%20Object%20Reference))
  ;[1 1 1] Load data
  (Variables|Default|SetCutsceneDone (.Value (Utilities|Map|Find (Variables|/Game/Assets/Save/BP_SaveGame.BP_SaveGame_C|GetCutscenes SaveGameRef) (Utilities|GetSequenceName))))
  (bind _values (Utilities|Map|Values (Variables|/Game/Assets/Save/BP_SaveGame.BP_SaveGame_C|GetCutscenes SaveGameRef)))
  (for _array_element _values
    (Development|PrintString (Utilities|String|ToString(Boolean) _array_element) true true "(R=0.920018,G=1.000000,B=0.000000,A=1.000000)")))

(event EventBeginPlay
  ;[1 1 1] BeginPlay
  (Class|BPIPersistence|RequestLoad(Message) (Game|GetGameInstance) self))

(fn ConstructionScript)