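; AI controller for a companion that follows the player character.
; On BeginPlay it caches the player character as its follow target and starts a looping half-second timer instead of using Tick.
; Each timer call checks the controller's distance to the target and, beyond a fixed threshold, issues a simple move-to-actor toward it and prints a debug message.
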(event EventBeginPlay
  (Variables|Default|SetFollow%20Target (Game|GetPlayerCharacter 0))
  (Utilities|Time|SetTimerbyFunctionName 0 "Follow Player" 0.5 true))

(event EventTick
  (params (DeltaSeconds :type Float%20%28single-precision%29)))

(fn ConstructionScript)

(fn FollowPlayer
  (if (> (Transformation|GetDistanceTo (Variables|Default|GetFollow%20Target)) 3e+02)
    (AI|Navigation|SimpleMovetoActor self (Variables|Default|GetFollow%20Target))
    (Development|PrintString "moving")))