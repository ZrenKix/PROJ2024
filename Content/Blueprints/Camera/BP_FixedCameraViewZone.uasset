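; Trigger actor that switches the player to its own fixed camera while the player pawn is inside the zone.
; Begin and end overlap blend the view target over time to this actor and back to the controlled pawn, with outgoing view locked.
; Each switch aligns control rotation to the destination camera.
; Two cross-resetting DoOnce gates make entry and exit alternate, blocking repeat triggers.
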(event Collision|EventActorBeginOverlap
  (params (OtherActor :type Actor%20Object%20Reference))
  (bind _returnvalue (Game|GetPlayerController 0))
  (bind _returnvalue_2 (Game|GetPlayerController 0))
  (bind _returnvalue_3 (Pawn|GetControlledPawn _returnvalue))
  (if (== OtherActor (Game|Player|GetPlayerPawn 0))
    (Utilities|FlowControl|DoOnce false
      (:Completed
        (Game|Player|SetViewTargetwithBlend _returnvalue_2 self 2.0 "VTBlend_Linear" 0.0 true)
        (Pawn|SetControlRotation _returnvalue_2 (Transformation|GetWorldRotation (Variables|Default|GetCamera)))
        (Utilities|FlowControl|DoOnce false) ; enters at Reset
      ))))

(event Collision|EventActorEndOverlap
  (params (OtherActor :type Actor%20Object%20Reference))
  (bind _returnvalue (Game|GetPlayerController 0))
  (bind _returnvalue_2 (Game|GetPlayerController 0))
  (bind _returnvalue_3 (Pawn|GetControlledPawn _returnvalue))
  (if (== OtherActor (Game|Player|GetPlayerPawn 0))
    (Utilities|FlowControl|DoOnce false
      (:Completed
        (Game|Player|SetViewTargetwithBlend _returnvalue _returnvalue_3 2.0 "VTBlend_Linear" 0.0 true)
        (Pawn|SetControlRotation _returnvalue (Transformation|GetWorldRotation (Actor|GetComponentbyClass _returnvalue_3 "/Script/Engine.CameraComponent")))
        (Utilities|FlowControl|DoOnce false) ; enters at Reset
      ))))

(fn ConstructionScript)