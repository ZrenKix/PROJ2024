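; BP_MoveableStair is a stair puzzle piece that moves vertically while its linked Button is pressed.
; Button press events start a fast looping timer on MoveStair and swap the mesh material, and release events clear the timer and restore the default.
; MoveStair offsets the mesh's world Z by a fraction of Speed per tick, flipping direction through top and bottom position checks to oscillate between the two markers.
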(event Custom|isPressed_Event
  (Utilities|Time|SetTimerbyFunctionName 0 "MoveStair" 0.001 true)
  (Rendering|Material|SetMaterial (Variables|Default|GetStaticMesh) 0 "/Game/VFX/Test_Animations/standardSurface1.standardSurface1"))

(event Custom|isNotPressed_Event
  (Utilities|Time|ClearTimerbyFunctionName 0 "MoveStair")
  (Rendering|Material|SetMaterial (Variables|Default|GetStaticMesh) 0 (Variables|Default|GetDefaultMat)))

(event EventBeginPlay
  (Variables|Default|SetDefaultMat (Rendering|Material|GetMaterial (Variables|Default|GetStaticMesh) 0))
  (EventDispatchers|AssignIsPressed (Variables|Default|GetButton) (delegate Custom|isPressed_Event))
  (EventDispatchers|AssignIsNotPressed (Variables|Default|GetButton) (delegate Custom|isNotPressed_Event)))

(fn ConstructionScript)

(fn MoveStair
  (if (Variables|Default|GetSwitchDirection)
    (Variables|Default|SetSpeed (* (Variables|Default|GetSpeed) -1.0))
    (Variables|Default|SetSwitchDirection false)
    (else
      (CallFunction|UpdateLocation)
      (if (or (|CheckTopPosition) (|CheckBottomPosition))
        (Variables|Default|SetSwitchDirection true)))))

(fn UpdateLocation
  (bind _staticmesh (Variables|Default|GetStaticMesh))
  (bind _returnvalue (Transformation|GetWorldLocation _staticmesh))
  (Transformation|SetWorldLocation (Variables|Default|GetStaticMesh) (Math|Vector|MakeVector (.x _returnvalue) (.y _returnvalue) (+ (.z _returnvalue) (/ (Variables|Default|GetSpeed) 1e+01))) false false))