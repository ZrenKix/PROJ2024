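; Edith's pressure platform in the stair puzzle, which triggers the final Erebus boss fight.
; Player overlap swaps its material and sinks it via looping timers, then freezes and turns the hero while blending to the final camera.
; A timer raises Erebus and shakes the camera with decaying intensity, then after a delay the game mode creates the combat arena.
; When combat finishes, the end-of-game widget appears.
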(event OnComponentBeginOverlap(Box)
  (params (OverlappedComponent :type Primitive%20Component%20Object%20Reference) (OtherActor :type Actor%20Object%20Reference) (OtherComp :type Primitive%20Component%20Object%20Reference) (OtherBodyIndex :type Integer) (bFromSweep :type Boolean) (SweepResult :type Hit%20Result%20Structure%20%28by%20ref%29))
  (if (Utilities|DoesObjectImplementInterface OtherActor "/Game/Blueprints/Interface/BPI_PlayerInterface.BPI_PlayerInterface_C")
    (Default|CallIsPressed)
    (Rendering|Material|SetMaterial (Variables|Default|GetCube) 0 (Variables|Default|GetPressedMat))
    (Utilities|Time|SetTimerbyFunctionName 0 "UpdateLocation" 0.001 true)
    (|IsVincentAndTeddyOnPlatforms)
    (bind _asbp_player_hero (Utilities|Casting|CastToBP_PlayerHero OtherActor))
    (Utilities|FlowControl|Delay 0.7)
    (Pawn|Components|CharacterMovement|SetMovementMode (Variables|/Script/Engine.Character|GetCharacterMovement _asbp_player_hero) "MOVE_None" 0)
    (Game|Player|SetViewTargetwithBlend (Game|GetPlayerController 0) (Variables|Default|GetFinalCamera) 5.0 "VTBlend_Linear" 0.0 false)
    (Variables|Default|SetbFuckoff true)
    (bind _returnvalue (Utilities|Time|SetTimerbyEvent (delegate Custom|CameraShake) 0.05 (Variables|Default|GetLooping)))))

(event OnComponentEndOverlap(Box)
  (params (OverlappedComponent :type Primitive%20Component%20Object%20Reference) (OtherActor :type Actor%20Object%20Reference) (OtherComp :type Primitive%20Component%20Object%20Reference) (OtherBodyIndex :type Integer))
  (if (Utilities|DoesObjectImplementInterface OtherActor "/Game/Blueprints/Interface/BPI_PlayerInterface.BPI_PlayerInterface_C")
    (Default|CallIsNotPressed)
    (Rendering|Material|SetMaterial (Variables|Default|GetCube) 0 (Variables|Default|GetDefaultMat))
    (Utilities|Time|SetTimerbyFunctionName 0 "ResetLocation" 0.001 true)))

(event Custom|CameraShake
  (|MoveErebus)
  (|CameraShakeCalculations (stale OnComponentBeginOverlap(Box) _returnvalue)))

(event EventBeginPlay
  (Variables|Default|SetDefaultPosition (Transformation|GetActorLocation))
  (Variables|Default|SetDefaultMat (Rendering|Material|GetMaterial (Variables|Default|GetCube) 0))
  (|SetErebusIslandVariables))

(event EventTick
  (params (DeltaSeconds :type Float%20%28single-precision%29))
  (if (Variables|Default|GetbFuckoff)
    (Transformation|SetActorRotation (stale OnComponentBeginOverlap(Box) _asbp_player_hero) (|CalculateRotation (stale OnComponentBeginOverlap(Box) _asbp_player_hero)))))

(fn ConstructionScript)

(fn ResetLocation
  (bind _returnvalue (Transformation|GetActorLocation))
  (if (Utilities|Operators|EqualEqual (Transformation|GetActorLocation) (Variables|Default|GetDefaultPosition) 0.0)
    (Utilities|Time|ClearTimerbyFunctionName 0 "ResetLocation")
    (else
      (Transformation|SetActorLocation (Math|Vector|MakeVector (.x _returnvalue) (.y _returnvalue) (+ (.z _returnvalue) (Variables|Default|GetOffset))) false false))))

(fn UpdateLocation
  (bind _returnvalue (Transformation|GetActorLocation))
  (bind _defaultposition (Variables|Default|GetDefaultPosition))
  (if (Utilities|Operators|EqualEqual (Transformation|GetActorLocation) (Math|Vector|MakeVector (.x _defaultposition) (.y _defaultposition) (- (.z _defaultposition) (Variables|Default|GetOffset))) 0.0)
    (Utilities|Time|ClearTimerbyFunctionName 0 "UpdateLocation")
    (else
      (Transformation|SetActorLocation (Math|Vector|MakeVector (.x _returnvalue) (.y _returnvalue) (- (.z _returnvalue) (Variables|Default|GetOffset))) false false))))

(event Custom|OnCombatFinished_Event
  (bind _returnvalue (UserInterface|CreateWidget "/Game/Blueprints/UI/WBP_TheEnd.WBP_TheEnd_C"))
  (UserInterface|Viewport|AddtoViewport _returnvalue 0))