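; Stair puzzle floor button that reacts to player overlap and can trigger the final Erebus sequence.
; Overlap calls press/release events, swaps the cube material and moves the button down or up through function timers.
; If the Vincent and Teddy buttons both report home on press, it disables hero movement and blends to FinalCamera.
; A CameraShake timer event then raises Erebus and jitters the camera with decreasing intensity.
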(event OnComponentBeginOverlap(Box)
  (params (OverlappedComponent :type Primitive%20Component%20Object%20Reference) (OtherActor :type Actor%20Object%20Reference) (OtherComp :type Primitive%20Component%20Object%20Reference) (OtherBodyIndex :type Integer) (bFromSweep :type Boolean) (SweepResult :type Hit%20Result%20Structure%20%28by%20ref%29))
  (if (Utilities|DoesObjectImplementInterface OtherActor "/Game/Blueprints/Interface/BPI_PlayerInterface.BPI_PlayerInterface_C")
    (Default|CallIsPressed)
    (Rendering|Material|SetMaterial (Variables|Default|GetCube) 0 (Variables|Default|GetPressedMat))
    (Utilities|Time|SetTimerbyFunctionName 0 "UpdateLocation" 0.001 true)
    (if (and (Variables|/Game/Blueprints/BP_FloorButtonVincent.BP_FloorButtonVincent_C|GetbVincentIsHome (Variables|Default|GetVincentFloor)) (Variables|/Game/Blueprints/BP_FloorButtonTeddy.BP_FloorButtonTeddy_C|GetbTeddyIsHome (Variables|Default|GetTeddyFloor)))
      (bind _asbp_player_hero (Utilities|Casting|CastToBP_PlayerHero OtherActor))
      (Utilities|FlowControl|Delay 0.7)
      (Pawn|Components|CharacterMovement|SetMovementMode (Variables|/Script/Engine.Character|GetCharacterMovement _asbp_player_hero) "MOVE_None" 0)
      (Game|Player|SetViewTargetwithBlend (Game|GetPlayerController 0) (Variables|Default|GetFinalCamera) 5.0 "VTBlend_Linear" 0.0 false)
      (Transformation|SetActorRotation _asbp_player_hero (Math|Interpolation|RInterpTo (Math|Rotator|MakeRotator 0.0 0.0 (.X (Math|Vector|BreakVector (Transformation|GetActorLocation _asbp_player_hero)))) (Math|Rotator|FindLookatRotation (Transformation|GetActorLocation _asbp_player_hero) (Transformation|GetActorLocation (Variables|Default|GetErebus))) (stale EventTick DeltaSeconds) 1.0))
      (bind _returnvalue (Utilities|Time|SetTimerbyEvent (delegate Custom|CameraShake) 0.05 (Variables|Default|GetLooping))))))

(event OnComponentEndOverlap(Box)
  (params (OverlappedComponent :type Primitive%20Component%20Object%20Reference) (OtherActor :type Actor%20Object%20Reference) (OtherComp :type Primitive%20Component%20Object%20Reference) (OtherBodyIndex :type Integer))
  (if (Utilities|DoesObjectImplementInterface OtherActor "/Game/Blueprints/Interface/BPI_PlayerInterface.BPI_PlayerInterface_C")
    (Default|CallIsNotPressed)
    (Rendering|Material|SetMaterial (Variables|Default|GetCube) 0 (Variables|Default|GetDefaultMat))
    (Utilities|Time|SetTimerbyFunctionName 0 "ResetLocation" 0.001 true)))

(event Custom|CameraShake
  (bind _erebus (Variables|Default|GetErebus))
  (bind _finalcameraoriginalpos (Variables|Default|GetFinalCameraOriginalPos))
  (bind _returnvalue (Transformation|GetActorLocation _erebus))
  (bind (_x _y _z) (Math|Vector|BreakVector _finalcameraoriginalpos))
  (bind (_x_2 _y_2 _z_2) (Math|Vector|BreakVector _returnvalue))
  (Transformation|SetActorLocation _erebus (Math|Vector|MakeVector _x_2 _y_2 (Math|Interpolation|FInterpTo _z_2 (.Z (Math|Vector|BreakVector "0.000000,0.000000,250.000000")) (stale EventTick DeltaSeconds) 1.0)) false false)
  (Transformation|SetActorLocation (Variables|Default|GetFinalCamera) (Math|Vector|MakeVector (+ _x (Math|Random|RandomFloatinRange (* (Variables|Default|GetCameraShakeIntensity) -1.0) (Variables|Default|GetCameraShakeIntensity))) (+ _y (Math|Random|RandomFloatinRange (* (Variables|Default|GetCameraShakeIntensity) -1.0) (Variables|Default|GetCameraShakeIntensity))) (+ _z (Math|Random|RandomFloatinRange (* (Variables|Default|GetCameraShakeIntensity) -1.0) (Variables|Default|GetCameraShakeIntensity)))) false false)
  (Variables|Default|SetCameraShakeIntensity (- (Variables|Default|GetCameraShakeIntensity) 0.2))
  (Utilities|FlowControl|Delay 4.0)
  (Variables|Default|SetLooping false)
  (Utilities|Time|ClearandInvalidateTimerbyHandle (stale OnComponentBeginOverlap(Box) _returnvalue)))

(event EventBeginPlay
  (Variables|Default|SetDefaultPosition (Transformation|GetActorLocation))
  (Variables|Default|SetDefaultMat (Rendering|Material|GetMaterial (Variables|Default|GetCube) 0))
  (bind _returnvalue (Actor|GetActorOfClass "/Game/Blueprints/BP_FloorButtonVincent.BP_FloorButtonVincent_C"))
  (bind _returnvalue_2 (Actor|GetActorOfClass "/Game/Blueprints/BP_FloorButtonTeddy.BP_FloorButtonTeddy_C"))
  (Variables|Default|SetVincentFloor _returnvalue)
  (Variables|Default|SetTeddyFloor _returnvalue_2)
  (Variables|Default|SetFinalCameraOriginalPos (Transformation|GetActorLocation (Variables|Default|GetFinalCamera))))

(event EventTick
  (params (DeltaSeconds :type Float%20%28single-precision%29)))

(fn ConstructionScript)

(fn ResetLocation
  (bind _returnvalue (Transformation|GetActorLocation))
  (if (Utilities|Operators|EqualEqual (Transformation|GetActorLocation) (Variables|Default|GetDefaultPosition) 0.0)
    (Utilities|Time|ClearTimerbyFunctionName 0 "ResetLocation")
    (else
      (Transformation|SetActorLocation (Math|Vector|MakeVector (.x _returnvalue) (.y _returnvalue) (+ (.z _returnvalue) (Variables|Default|GetOffset))) false false))))

(fn UpdateLocation
  (bind _returnvalue (Transformation|GetActorLocation))
  (bind _defaultposition (Variables|Default|GetDefaultPosition))
  (if (Utilities|Operators|EqualEqual (Transformation|GetActorLocation) (Math|Vector|MakeVector (.x _defaultposition) (.y _defaultposition) (- (.z _defaultposition) (Variables|Default|GetOffset))) 0.0)
    (Utilities|Time|ClearTimerbyFunctionName 0 "UpdateLocation")
    (else
      (Transformation|SetActorLocation (Math|Vector|MakeVector (.x _returnvalue) (.y _returnvalue) (- (.z _returnvalue) (Variables|Default|GetOffset))) false false))))