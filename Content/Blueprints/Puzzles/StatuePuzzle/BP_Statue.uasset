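; Interactable puzzle statue that shows a "Rotate" prompt and turns its mesh when used.
; Interact stores the current rotation, takes a target from Rotate90 and locks input while a timeline lerps between them, unlocking on finish.
; Rotate90's 90-degree yaw rotator appears unconnected to any output.
; ResetStatue snaps to the stored start rotation, which each interaction overwrites, and rotations are read in world space but set as relative.
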(event Custom|RotateMesh
  (bind _time (Timeline|UpdateLerp PlayFromStart)
    (:Update
      (Transformation|SetRelativeRotation (Variables|Default|GetObject) (Math|Rotator|Lerp(Rotator) (Variables|Default|GetStartRotation) (Variables|Default|GetTargetRotation) _time) false false))
    (:Finished
      (Variables|Default|SetisInteractable true))))

(event EventBeginPlay
  (Variables|Default|SetStartRotation (Transformation|GetWorldRotation (Variables|Default|GetObject))))

(fn ConstructionScript)

(fn ResetStatue
  (Transformation|SetRelativeRotation (Variables|Default|GetObject) (Variables|Default|GetStartRotation) false false))

(fn GetInteractPrompt
  (if (Variables|Default|GetisInteractable)
    (return "Rotate")
    (else
      (return ""))))

(fn Interact
  (if (Variables|Default|GetisInteractable)
    (Variables|Default|SetStartRotation (Transformation|GetWorldRotation (Variables|Default|GetObject)))
    (Variables|Default|SetTargetRotation (|Rotate90))
    (CallFunction|RotateMesh)
    (Variables|Default|SetisInteractable false)
    (return false)))