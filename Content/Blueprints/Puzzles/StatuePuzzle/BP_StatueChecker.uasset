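; Interactable checker for the statue puzzle that tests whether three statues face their goal yaw rotations.
; CheckStatues compares exact yaw per statue, fills CorrectStatues, derives AllCorrect, and shows the completion popup without branching on the result.
; Success opens bars, disables the blocking wall, activates lantern fires, and locks checker and statues.
; Failure resets the statues and shows a hint popup pointing back to the painting.
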(event EventBeginPlay)

(event Collision|EventActorBeginOverlap
  (params (OtherActor :type Actor%20Object%20Reference)))

(event EventTick
  (params (DeltaSeconds :type Float%20%28single-precision%29)))

(fn ConstructionScript)

(fn CheckStatues
  (for (_array_element _array_index) (Variables|Default|GetStatues)
    (switch int _array_index
      (:0
        (if (== (.yaw (Transformation|GetWorldRotation (Variables|/Game/Blueprints/Puzzles/StatuePuzzle/BP_Statue.BP_Statue_C|GetObject _array_element))) (Variables|Default|GetGoalRotation1))
          (Utilities|Array|SetArrayElem (Variables|Default|GetCorrectStatues) 0 true)))
      (:1
        (if (== (.yaw (Transformation|GetWorldRotation (Variables|/Game/Blueprints/Puzzles/StatuePuzzle/BP_Statue.BP_Statue_C|GetObject _array_element))) (Variables|Default|GetGoalRotation2))
          (Utilities|Array|SetArrayElem (Variables|Default|GetCorrectStatues) 1 true)))
      (:2
        (if (== (.yaw (Transformation|GetWorldRotation (Variables|/Game/Blueprints/Puzzles/StatuePuzzle/BP_Statue.BP_Statue_C|GetObject _array_element))) (Variables|Default|GetGoalRotation3))
          (Utilities|Array|SetArrayElem (Variables|Default|GetCorrectStatues) 2 true)))))
  (for _array_element_2 (Variables|Default|GetCorrectStatues)
    (if (not _array_element_2)
      (LocalVariables|SetAllCorrect false)))
  ;[1 1 1] Puzzle Complete
  (bind _returnvalue (UserInterface|CreateWidget "/Game/Blueprints/UI/Interaction/WBP_TextPopup.WBP_TextPopup_C" 0 "I did it! I should check the last painting piece." "Edith" "/Game/Assets/UI/NewUI/T_UI_Card_Character_Edith.T_UI_Card_Character_Edith"))
  (UserInterface|Viewport|AddtoViewport _returnvalue 0)
  (return (LocalVariables|GetAllCorrect)))

(fn HandleSuccess
  (Default|OpenBars (Variables|Default|GetBars))
  (Variables|Default|SetisInteractable false)
  (for _array_element (Variables|Default|GetStatues)
    (Variables|/Game/Blueprints/Puzzles/StatuePuzzle/BP_Statue.BP_Statue_C|SetisInteractable _array_element false))
  (Default|Disable (Variables|Default|GetBlockingWall))
  (for _array_element_2 (Variables|Default|GetLanterns)
    (Components|Activation|Activate (Variables|/Game/Blueprints/Enviroment/BP_Lantern.BP_Lantern_C|Getfire _array_element_2) false)))

(fn ResetStatues
  (for _array_element (Variables|Default|GetStatues)
    (Default|ResetStatue _array_element)))

(fn GetInteractPrompt
  (if (Variables|Default|GetisInteractable)
    (return "Check result")
    (else
      (return ""))))

(fn Interact
  (if (Variables|Default|GetisInteractable)
    (bind _success (CallFunction|CheckStatues))
    (if _success
      (CallFunction|HandleSuccess)
      (else
        (CallFunction|ResetStatues)
        (bind _returnvalue (UserInterface|CreateWidget "/Game/Blueprints/UI/Interaction/WBP_TextPopup.WBP_TextPopup_C" 0 "Hmm, that wasn't right. I should check that painting again." "Edith" "/Game/Assets/UI/NewUI/T_UI_Card_Character_Edith.T_UI_Card_Character_Edith"))
        (UserInterface|Viewport|AddtoViewport _returnvalue 0)))
    (return true)))