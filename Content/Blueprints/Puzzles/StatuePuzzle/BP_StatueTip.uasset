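; BP_StatueTip is a statue puzzle interactable that shows a "Look at" prompt while it is enabled.
; Interacting disables it, creates a WBP_StatueCorrect widget with itself as owning actor, and adds that widget to the viewport.
; An external SetInteractable event toggles whether it can be used again.
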(event EventBeginPlay)

(event Collision|EventActorBeginOverlap
  (params (OtherActor :type Actor%20Object%20Reference)))

(event EventTick
  (params (DeltaSeconds :type Float%20%28single-precision%29)))

(event EventSetInteractable
  (params (bIsInteractable :type Boolean))
  (Variables|Default|SetisInteractable bIsInteractable))

(fn ConstructionScript)

(fn GetInteractPrompt
  (if (Variables|Default|GetisInteractable)
    (return "Look at")
    (else
      (return ""))))

(fn Interact
  (if (Variables|Default|GetisInteractable)
    (Variables|Default|SetisInteractable false)
    (bind _returnvalue (UserInterface|CreateWidget "/Game/Blueprints/Puzzles/StatuePuzzle/WBP_StatueCorrect.WBP_StatueCorrect_C"))
    (Variables|/Game/Blueprints/Puzzles/StatuePuzzle/WBP_StatueCorrect.WBP_StatueCorrect_C|SetOwningActor _returnvalue self)
    (UserInterface|Viewport|AddtoViewport _returnvalue 0)
    (return true)))