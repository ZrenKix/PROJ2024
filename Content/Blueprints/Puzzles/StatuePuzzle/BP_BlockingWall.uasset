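; Blocking wall for the statue puzzle that can be removed, with its removed state persisting through the save game.
; Disable turns off mesh and box collision, hides the actor and clears ShouldSpawn rather than destroying it.
; Save and load events store that flag in the SpawnableActors map, keyed by ActorGuid.
; On BeginPlay it requests a load from BP_GameInstance, then destroys itself if the flag is false.
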(event EventBeginPlay
  (bind _asbp_game_instance (Utilities|Casting|CastToBP_GameInstance (Game|GetGameInstance)))
  (Default|RequestLoad _asbp_game_instance self)
  (if (not (Variables|Default|GetShouldSpawn))
    (Actor|DestroyActor)))

(event EventSaveData
  (params (SaveGameRef :type BP%20Save%20Game%20Object%20Reference))
  (Utilities|Map|Add (Variables|/Game/Assets/Save/BP_SaveGame.BP_SaveGame_C|GetSpawnableActors SaveGameRef) (Variables|Default|GetActorGuid) (Variables|Default|GetShouldSpawn)))

(event EventLoadData
  (params (SaveGameRef :type BP%20Save%20Game%20Object%20Reference))
  (bind _spawnableactors (Variables|/Game/Assets/Save/BP_SaveGame.BP_SaveGame_C|GetSpawnableActors SaveGameRef))
  (bind _actorguid (Variables|Default|GetActorGuid))
  (bind (_value _returnvalue) (Utilities|Map|Find _spawnableactors _actorguid))
  (if _returnvalue
    (Variables|Default|SetShouldSpawn _value)))

(fn ConstructionScript)

(fn Disable
  (Collision|SetCollisionEnabled (Variables|Default|GetStaticMesh) "NoCollision")
  (Rendering|SetActorHiddenInGame true)
  (Variables|Default|SetShouldSpawn false))