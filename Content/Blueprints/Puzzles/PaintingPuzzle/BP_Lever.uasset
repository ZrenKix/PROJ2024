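; Interactable color source for the painting puzzle that feeds its own color into a linked ResultColor to be mixed.
; On BeginPlay it reads MyColor from the FirstColor parameter of its mesh material and randomizes its rotation speed.
; The "Mix" interaction fills ResultColor's first slot if still white, otherwise the second, then disables further interaction.
; CheckResult simply forwards to ResultColor.
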(event EventBeginPlay
  (bind _returnvalue (Rendering|Material|CreateDynamicMaterialInstance (Rendering|Material|GetMaterial (Variables|Default|GetStaticMesh) 1) "None" "None" :!class /Script/Engine.KismetMaterialLibrary))
  (bind _returnvalue_2 (Rendering|Material|GetVectorParameterValue _returnvalue "FirstColor" :!class /Script/Engine.MaterialInstanceDynamic))
  (Variables|Default|SetMyColor _returnvalue_2)
  (Variables|/Script/Engine.RotatingMovementComponent|SetRotationRate (Variables|Default|GetRotatingMovement) (Math|Rotator|MakeRotator 0.0 0.0 (Math|Random|RandomFloatinRange 25.0 45.0))))

(fn ConstructionScript)

(fn CheckResult
  (Default|CheckResult (Variables|Default|GetResultColor)))

(fn GetInteractPrompt
  (if (Variables|Default|GetisInteractable)
    (return "Mix")
    (else
      (return ""))))

(fn Interact
  (bind _resultcolor (Variables|Default|GetResultColor))
  (if (Variables|Default|GetisInteractable)
    (if (== (Variables|/Game/Blueprints/Puzzles/PaintingPuzzle/BP_ResultColor.BP_ResultColor_C|GetFirstColor (Variables|Default|GetResultColor)) "(R=1.000000,G=1.000000,B=1.000000,A=1.000000)")
      (Variables|/Game/Blueprints/Puzzles/PaintingPuzzle/BP_ResultColor.BP_ResultColor_C|SetFirstColor (Variables|Default|GetResultColor) (Variables|Default|GetMyColor))
      (Default|SetValues (Variables|Default|GetResultColor) (Variables|Default|GetMyColor))
      (else
        (Variables|/Game/Blueprints/Puzzles/PaintingPuzzle/BP_ResultColor.BP_ResultColor_C|SetSecondColor (Variables|Default|GetResultColor) (Variables|Default|GetMyColor))
        (Default|SetValues _resultcolor (Variables|/Game/Blueprints/Puzzles/PaintingPuzzle/BP_ResultColor.BP_ResultColor_C|GetFirstColor _resultcolor) (Variables|Default|GetMyColor))))
    (Variables|Default|SetisInteractable false)))