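; A one-shot trigger that shows a hard-coded color-mixing hint from Edith when the player enters its box.
; On overlap by an actor implementing BPI_PlayerInterface, it adds a WBP_TextPopup to the viewport, disables the box collision and clears ShouldSpawn.
; Save and load events persist ShouldSpawn by ActorGuid in the save game's SpawnableActors map.
; BeginPlay destroys the actor if that flag is false.
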(event OnComponentBeginOverlap(Box)
  (params (OverlappedComponent :type Primitive%20Component%20Object%20Reference) (OtherActor :type Actor%20Object%20Reference) (OtherComp :type Primitive%20Component%20Object%20Reference) (OtherBodyIndex :type Integer) (bFromSweep :type Boolean) (SweepResult :type Hit%20Result%20Structure%20%28by%20ref%29))
  (if (Utilities|DoesObjectImplementInterface OtherActor "/Game/Blueprints/Interface/BPI_PlayerInterface.BPI_PlayerInterface_C")
    (bind _returnvalue (UserInterface|CreateWidget "/Game/Blueprints/UI/Interaction/WBP_TextPopup.WBP_TextPopup_C" 0 "Hmm, seems like I have to mix the right color." "Edith" "/Game/Assets/UI/NewUI/T_UI_Card_Character_Edith.T_UI_Card_Character_Edith"))
    (UserInterface|Viewport|AddtoViewport _returnvalue 0)
    (Collision|SetCollisionEnabled (Variables|Default|GetBox) "NoCollision")
    (Variables|Default|SetShouldSpawn false)))

(event EventBeginPlay
  (if (not (Variables|Default|GetShouldSpawn))
    (Actor|DestroyActor)))

(event EventLoadData
  (params (SaveGameRef :type BP%20Save%20Game%20Object%20Reference))
  (bind _actorguid (Variables|Default|GetActorGuid))
  (bind _spawnableactors (Variables|/Game/Assets/Save/BP_SaveGame.BP_SaveGame_C|GetSpawnableActors SaveGameRef))
  (bind (_value _returnvalue) (Utilities|Map|Find _spawnableactors _actorguid))
  (if _returnvalue
    (Variables|Default|SetShouldSpawn _value)))

(event EventSaveData
  (params (SaveGameRef :type BP%20Save%20Game%20Object%20Reference))
  (Utilities|Map|Add (Variables|/Game/Assets/Save/BP_SaveGame.BP_SaveGame_C|GetSpawnableActors SaveGameRef) (Variables|Default|GetActorGuid) (Variables|Default|GetShouldSpawn)))

(fn ConstructionScript)