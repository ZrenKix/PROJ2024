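; Enemy encounter trigger that starts an arena when the player's pawn overlaps its collision component.
; It asks the ArenaManager to create the arena scene from its enemy and hero classes, with no boss type.
; After a short delay it destroys its referenced sprite actors and plays a level sequence.
; The sequence-finished handler is empty, and the trigger neither destroys itself nor guards against repeat overlaps.
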(event OnComponentBeginOverlap(CollisionComponent)
  (params (OverlappedComponent :type Primitive%20Component%20Object%20Reference) (OtherActor :type Actor%20Object%20Reference) (OtherComp :type Primitive%20Component%20Object%20Reference) (OtherBodyIndex :type Integer) (bFromSweep :type Boolean) (SweepResult :type Hit%20Result%20Structure%20%28by%20ref%29))
  (bind _sequencer (Variables|Default|GetSequencer))
  (bind _sequenceplayer (Variables|/Script/LevelSequence.LevelSequenceActor|GetSequencePlayer _sequencer))
  (if (== OtherActor (Game|Player|GetPlayerPawn 0))
    (Class|ArenaManager|CreateArena (Subsystems|GetArenaManager) (Variables|Default|GetEnemy%20Classes) (Variables|Default|GetHero%20Classes) "ArenaScene" "None" 3)
    (Utilities|FlowControl|Delay 1.0)
    (for _array_element (Variables|Default|GetSprites)
      (Actor|DestroyActor _array_element))
    (Sequencer|Player|Play _sequenceplayer :!class /Script/MovieScene.MovieSceneSequencePlayer)
    (EventDispatchers|AssignOnFinished _sequenceplayer (delegate Custom|OnFinished_Event))))

(event Custom|OnFinished_Event)

(event EventBeginPlay)

(event Collision|EventActorBeginOverlap
  (params (OtherActor :type Actor%20Object%20Reference)))

(event EventTick
  (params (DeltaSeconds :type Float%20%28single-precision%29)))

(fn ConstructionScript)