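; One-shot enemy encounter trigger that sends the player into arena combat, then plays a post-combat sequence and dialogue.
; Player overlap disables movement, plays the encounter flipbook and sound, then asks BP_DreamboundGameMode to create the arena with combat dialogue.
; When the arena with the matching UID closes, it removes sprites, reveals the chair, starts the sequencer and opens the dialogue widget.
; Tick restores movement once the last entry is reached and the widget is hidden.
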(event OnComponentBeginOverlap(CollisionComponent)
  (params (OverlappedComponent :type Primitive%20Component%20Object%20Reference) (OtherActor :type Actor%20Object%20Reference) (OtherComp :type Primitive%20Component%20Object%20Reference) (OtherBodyIndex :type Integer) (bFromSweep :type Boolean) (SweepResult :type Hit%20Result%20Structure%20%28by%20ref%29))
  (bind _hero_classes (Variables|Default|GetHero%20Classes))
  (if (== OtherActor (Game|Player|GetPlayerPawn 0))
    (Utilities|FlowControl|DoOnce false
      (:Completed
        (Components|Activation|SetActive (Pawn|GetMovementComponent (Game|GetPlayerCharacter 0)) false false)
        (|EncounterTransition)
        (Class|FMODAudioComponent|Stop (stale EventBeginPlay _returnvalue))
        (bind _asbp_dreambound_game_mode (Utilities|Casting|CastToBP_DreamboundGameMode (Game|GetGameMode)))
        (bind _uid (Default|CreateArena _asbp_dreambound_game_mode _hero_classes (Variables|Default|GetEnemy%20Classes) (Variables|Default|GetBossfight%20Type) (Utilities|Array|Length _hero_classes) (Variables|Default|GetDialogue%20Under%20Combat) (Variables|Default|GetArena%20Scene)))
        (EventDispatchers|AssignCloseArena _asbp_dreambound_game_mode (delegate Custom|CloseArena_Event))))))

(event Custom|OnFinished_Event)

(event Custom|CloseArena_Event
  (params (UID :type Integer))
  (bind _sequencer (Variables|Default|GetSequencer))
  (bind _sequenceplayer (Variables|/Script/LevelSequence.LevelSequenceActor|GetSequencePlayer _sequencer))
  (if (== (stale OnComponentBeginOverlap(CollisionComponent) _uid) UID)
    (Sprite|SetFlipbook (Variables|Default|GetPaperFlipbook1))
    (Utilities|FlowControl|Delay 1.0)
    (for _array_element (Variables|Default|GetSprites%20To%20Remove)
      (Actor|DestroyActor _array_element))
    (Rendering|SetActorHiddenInGame (Variables|Default|GetChair) false)
    (Sequencer|Player|Play _sequenceplayer :!class /Script/MovieScene.MovieSceneSequencePlayer)
    (EventDispatchers|AssignOnFinished _sequenceplayer (delegate Custom|OnFinished_Event))
    (Components|Activation|SetActive (Pawn|GetMovementComponent (Game|GetPlayerCharacter 0)) false false)
    (bind _returnvalue (UserInterface|CreateWidget "/Game/Blueprints/Arena/Widgets/WBP_DialogueOpenWorld.WBP_DialogueOpenWorld_C"))
    (UserInterface|Viewport|AddtoViewport _returnvalue 0)
    (Widget|SetVisibility _returnvalue "Visible")
    (bind _returnvalue_2 (Game|ConstructObjectfromClass (Variables|Default|GetDialogue%20After%20Combat)))
    (bind _asdialogue_data_asset (Utilities|Casting|CastToDialogueDataAsset _returnvalue_2))
    (Default|DisplayEntry _returnvalue 0 "/Game/Assets/UI/Card/T_UI_Card_Character_Bear.T_UI_Card_Character_Bear" _asdialogue_data_asset)
    (else
      (Development|PrintString "Wrong UID"))))

(event EventBeginPlay
  (bind _returnvalue (Class|FMODBlueprintStatics|PlayEventAttached "/Game/FMOD/Events/Combat/Enemies/EnemyEncounter/EnemeyEncounter_Idle.EnemeyEncounter_Idle" (Variables|Default|GetPaperFlipbook1) "None" "0, 0, 0" "KeepRelativeOffset"))
  (Rendering|SetActorHiddenInGame (Variables|Default|GetChair) true))

(event Collision|EventActorBeginOverlap
  (params (OtherActor :type Actor%20Object%20Reference)))

(event EventTick
  (params (DeltaSeconds :type Float%20%28single-precision%29))
  ;[0.4562 1 0.5145] Enable Input after dialogue
  (Utilities|IsValid (stale Custom|CloseArena_Event _returnvalue)
    (:Is%20Valid
      (if (>= (Variables|/Game/Blueprints/Arena/Widgets/WBP_DialogueOpenWorld.WBP_DialogueOpenWorld_C|GetCurrentEntry (stale Custom|CloseArena_Event _returnvalue)) (- (Utilities|Array|Length (Variables|/Script/PROJ.DialogueDataAsset|GetDialogueEntries (stale Custom|CloseArena_Event _asdialogue_data_asset))) 1))
        (bind _output_get (Variables|Default|SetAt%20Last%20Entry (>= (Variables|/Game/Blueprints/Arena/Widgets/WBP_DialogueOpenWorld.WBP_DialogueOpenWorld_C|GetCurrentEntry (stale Custom|CloseArena_Event _returnvalue)) (- (Utilities|Array|Length (Variables|/Script/PROJ.DialogueDataAsset|GetDialogueEntries (stale Custom|CloseArena_Event _asdialogue_data_asset))) 1)))))
      (if _output_get
        (if (not (Widget|IsVisible (stale Custom|CloseArena_Event _returnvalue)))
          (Utilities|FlowControl|DoOnce false
            (:Completed
              (Components|Activation|SetActive (Pawn|GetMovementComponent (Game|GetPlayerCharacter 0)) true false))))))))

(fn ConstructionScript)