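; BP_TriggerNG is a trigger actor that ignites two referenced lanterns when BP_PlayerHero overlaps it.
; BeginPlay deactivates both lanterns' Fire components and hides their point lights.
; Overlap activates Lantern1's fire, then a DoOnce gates the attached FireWithIgnite audio events and Lantern2's fire, so they happen only once.
; The nodes that would unhide the point lights are unconnected, so those lights stay hidden.
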(event EventBeginPlay
  (bind _lantern1 (Variables|Default|GetLantern1))
  (bind _lantern2 (Variables|Default|GetLantern2))
  (Components|Activation|Deactivate (Variables|/Game/Blueprints/Enviroment/BP_Lantern.BP_Lantern_C|Getfire _lantern1))
  (Components|Activation|Deactivate (Variables|/Game/Blueprints/Enviroment/BP_Lantern.BP_Lantern_C|Getfire _lantern2))
  (Development|SetHiddeninGame (Variables|/Game/Blueprints/Enviroment/BP_Lantern.BP_Lantern_C|GetPointLight _lantern2) true false)
  (Development|SetHiddeninGame (Variables|/Game/Blueprints/Enviroment/BP_Lantern.BP_Lantern_C|GetPointLight _lantern1) true false))

(event Collision|EventActorBeginOverlap
  (params (OtherActor :type Actor%20Object%20Reference))
  (bind _lantern1 (Variables|Default|GetLantern1))
  (bind _lantern2 (Variables|Default|GetLantern2))
  (bind _fire (Variables|/Game/Blueprints/Enviroment/BP_Lantern.BP_Lantern_C|Getfire _lantern2))
  (bind _fire_2 (Variables|/Game/Blueprints/Enviroment/BP_Lantern.BP_Lantern_C|Getfire _lantern1))
  (Utilities|Casting|CastToBP_PlayerHero OtherActor)
  (Components|Activation|Activate _fire_2 false)
  (Utilities|FlowControl|DoOnce false
    (:Completed
      (Class|FMODBlueprintStatics|PlayEventAttached "/Game/FMOD/Events/Misc/FireWithIgnite.FireWithIgnite" _fire_2 "None" "0, 0, 0" "KeepRelativeOffset")
      (Components|Activation|Activate _fire false)
      (Utilities|FlowControl|DoOnce false
        (:Completed
          (Class|FMODBlueprintStatics|PlayEventAttached "/Game/FMOD/Events/Misc/FireWithIgnite.FireWithIgnite" _fire "None" "0, 0, 0" "KeepRelativeOffset"))))))

(fn ConstructionScript)