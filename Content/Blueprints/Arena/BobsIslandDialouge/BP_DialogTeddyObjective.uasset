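; One-shot trigger actor that plays the Teddy dialogue and advances that objective.
; When the player overlaps TriggerZone, it disables character movement and shows WBP_DialogueOpenWorld with the bear portrait and DialougeClass entries.
; Tick polls until the last entry is reached and the widget hidden, then restores movement and calls TalkToTeddy on BP_ObjectivesManager.
; ShouldSpawn saves under a construction-generated GUID, so a used trigger destroys itself on BeginPlay.
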(event OnComponentBeginOverlap(TriggerZone)
  (params (OverlappedComponent :type Primitive%20Component%20Object%20Reference) (OtherActor :type Actor%20Object%20Reference) (OtherComp :type Primitive%20Component%20Object%20Reference) (OtherBodyIndex :type Integer) (bFromSweep :type Boolean) (SweepResult :type Hit%20Result%20Structure%20%28by%20ref%29))
  (bind _returnvalue (Game|GetPlayerCharacter 0))
  (if (and (== OtherActor _returnvalue) (Variables|Default|GetShouldSpawn))
    (Components|Activation|SetActive (Pawn|GetMovementComponent _returnvalue) false false)
    (bind _returnvalue_2 (UserInterface|CreateWidget "/Game/Blueprints/Arena/Widgets/WBP_DialogueOpenWorld.WBP_DialogueOpenWorld_C"))
    (UserInterface|Viewport|AddtoViewport _returnvalue_2 0)
    (Widget|SetVisibility _returnvalue_2 "Visible")
    (bind _returnvalue_3 (Game|ConstructObjectfromClass (Variables|Default|GetDialougeClass)))
    (bind _asdialogue_data_asset (Utilities|Casting|CastToDialogueDataAsset _returnvalue_3))
    (Default|DisplayEntry _returnvalue_2 0 "/Game/Assets/UI/Card/T_UI_Card_Character_Bear.T_UI_Card_Character_Bear" _asdialogue_data_asset)
    (Variables|Default|SetShouldSpawn false)))

(event Custom|Isdone
  (if true
    _))

(event EventBeginPlay
  (bind _asbp_game_instance (Utilities|Casting|CastToBP_GameInstance (Game|GetGameInstance)))
  (Default|RequestLoad _asbp_game_instance self)
  (bind _returnvalue (Actor|GetActorOfClass "/Game/Blueprints/ObjectiveManager/BP_ObjectivesManager.BP_ObjectivesManager_C"))
  (Variables|Default|SetObjectiveManager _returnvalue)
  (if (not (Variables|Default|GetShouldSpawn))
    (Actor|DestroyActor)))

(event EventSaveData
  (params (SaveGameRef :type BP%20Save%20Game%20Object%20Reference))
  ;[1 1 1] Save Data
  (Utilities|Map|Add (Variables|/Game/Assets/Save/BP_SaveGame.BP_SaveGame_C|GetSpawnableActors SaveGameRef) (Variables|Default|GetGuid) (Variables|Default|GetShouldSpawn)))

(event EventLoadData
  (params (SaveGameRef :type BP%20Save%20Game%20Object%20Reference))
  (bind _spawnableactors (Variables|/Game/Assets/Save/BP_SaveGame.BP_SaveGame_C|GetSpawnableActors SaveGameRef))
  (bind _guid (Variables|Default|GetGuid))
  (bind (_value _returnvalue) (Utilities|Map|Find _spawnableactors _guid))
  ;[1 1 1] Load Data
  (if _returnvalue
    (Variables|Default|SetShouldSpawn _value)))

(event EventTick
  (params (DeltaSeconds :type Float%20%28single-precision%29))
  ;[0.4562 1 0.5145] Enable Input after dialogue
  (Utilities|IsValid (stale OnComponentBeginOverlap(TriggerZone) _returnvalue_2)
    (:Is%20Valid
      (if (>= (Variables|/Game/Blueprints/Arena/Widgets/WBP_DialogueOpenWorld.WBP_DialogueOpenWorld_C|GetCurrentEntry (stale OnComponentBeginOverlap(TriggerZone) _returnvalue_2)) (- (Utilities|Array|Length (Variables|/Script/PROJ.DialogueDataAsset|GetDialogueEntries (stale OnComponentBeginOverlap(TriggerZone) _asdialogue_data_asset))) 1))
        (bind _output_get (Variables|Default|SetAt%20Last%20Entry (>= (Variables|/Game/Blueprints/Arena/Widgets/WBP_DialogueOpenWorld.WBP_DialogueOpenWorld_C|GetCurrentEntry (stale OnComponentBeginOverlap(TriggerZone) _returnvalue_2)) (- (Utilities|Array|Length (Variables|/Script/PROJ.DialogueDataAsset|GetDialogueEntries (stale OnComponentBeginOverlap(TriggerZone) _asdialogue_data_asset))) 1)))))
      (if _output_get
        (if (not (Widget|IsVisible (stale OnComponentBeginOverlap(TriggerZone) _returnvalue_2)))
          (Utilities|FlowControl|DoOnce false
            (:Completed
              (Components|Activation|SetActive (Pawn|GetMovementComponent (Game|GetPlayerCharacter 0)) true false)
              (Default|TalktoTeddy (Variables|Default|GetObjectiveManager)))))))))

(fn ConstructionScript
  (CallFunction|HandleGUID))

(fn HandleGUID
  (if (not (Guid|IsValidGuid (Variables|Default|GetGuid)))
    (Variables|Default|SetGuid (Guid|NewGuid))))