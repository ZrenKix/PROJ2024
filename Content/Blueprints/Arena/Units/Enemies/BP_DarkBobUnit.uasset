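; Dark Bob miniboss enemy unit for the arena, tagged Enemy, with Charge, Ground Slam and Basic Attack actions.
; The two attacks activate GAS abilities, while Charge only plays effects; all play override animations and timed announcement widgets, with camera shake on Charge and Slam.
; Tick mirrors the Taunted tag to a sprite, and a successful Basic Attack clears it after a delay.
; Death sets lifespan from animation length.
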(event EventBeginPlay
  (GameplayTags|AddGameplayTag (Variables|Default|GetGameplay%20Tags) "(TagName=\"enemy\")" :!class /Script/GameplayTags.BlueprintGameplayTagLibrary))

(event Collision|EventActorBeginOverlap
  (params (OtherActor :type Actor%20Object%20Reference)))

(event EventBasicAttack
  (bind _gameplay_tags (Variables|Default|GetGameplay%20Tags))
  ;[1 1 1] Basic Attack
  (Development|PrintString "Basic Attack")
  (bind _returnvalue (Abilities|TryActivateAbilitybyClass (Ability|GetAbilitySystemComponent self) "/Game/Blueprints/AbilitySystem/GameplayAbilites/ProjectileAbilites/GA_BobSingle.GA_BobSingle_C" true))
  (if _returnvalue
    (Development|PrintString "success")
    (bind _animationlength (Class|PaperZDAnimInstance|PlayAnimationOverride (Variables|/Script/PaperZD.PaperZDAnimationComponent|GetAnimInstance (Variables|Default|GetAnimationComponent)) "/Game/Assets/Animations/Enemy_Miniboss/AnimSequences/AS_Enemy_Miniboss_BA.AS_Enemy_Miniboss_BA" "DefaultSlot" 1.0 0.0))
    (bind _returnvalue_2 (UserInterface|CreateWidget "/Game/Blueprints/UI/AttackExplanation/WBP_AttackExplain.WBP_AttackExplain_C"))
    (Variables|/Script/UMG.TextBlock|SetText (Variables|/Game/Blueprints/UI/AttackExplanation/WBP_AttackExplain.WBP_AttackExplain_C|GetActionText _returnvalue_2) "Dark Bob used 'Basic Attack'")
    (UserInterface|Viewport|AddtoViewport _returnvalue_2 0)
    (Utilities|FlowControl|Delay (+ _animationlength 1.0))
    (Widget|RemovefromParent _returnvalue_2)
    (if (GameplayTags|HasTag _gameplay_tags "(TagName=\"States.Taunted\")")
      (Utilities|FlowControl|Delay 2.0)
      (GameplayTags|RemoveGameplayTag _gameplay_tags "(TagName=\"States.Taunted\")" :!class /Script/GameplayTags.BlueprintGameplayTagLibrary))
    (else
      (Development|PrintString "fail"))))

(event EventCharge
  ;[1 0.04868 0] Charge
  (Development|PrintString "Charfe")
  (bind _animationlength (Class|PaperZDAnimInstance|PlayAnimationOverride (Variables|/Script/PaperZD.PaperZDAnimationComponent|GetAnimInstance (Variables|Default|GetAnimationComponent)) "/Game/Assets/Animations/Enemy_Miniboss/AnimSequences/AS_Enemy_Miniboss_Charge.AS_Enemy_Miniboss_Charge" "DefaultSlot" 1.0 0.0))
  (Niagara|SpawnSystematLocation "/Game/VFX/Niagara/Systems/LastBoss/NG_Charge_Bob.NG_Charge_Bob" (Transformation|GetActorLocation) (Transformation|GetActorRotation) "2.000000,2.000000,2.000000")
  (bind _returnvalue (UserInterface|CreateWidget "/Game/Blueprints/UI/AttackExplanation/WBP_AttackExplain.WBP_AttackExplain_C"))
  (Variables|/Script/UMG.TextBlock|SetText (Variables|/Game/Blueprints/UI/AttackExplanation/WBP_AttackExplain.WBP_AttackExplain_C|GetActionText _returnvalue) "Dark Bob used 'Charge'")
  (UserInterface|Viewport|AddtoViewport _returnvalue 0)
  (Camera|PlayWorldCameraShake "/Game/Blueprints/Camera/BP_CamShakeCharge.BP_CamShakeCharge_C" (Transformation|GetActorLocation (Game|Player|GetPlayerPawn 0)) 0.0 5e+04)
  (Utilities|FlowControl|Delay (+ _animationlength 1.0))
  (Widget|RemovefromParent _returnvalue))

(event EventDarkBobSpecial
  ;[1 0.9334 0] Special Attack
  (Development|PrintString "Special Attack")
  (bind _returnvalue (Abilities|TryActivateAbilitybyClass (Ability|GetAbilitySystemComponent self) "/Game/Blueprints/AbilitySystem/EnemyAbilities/GA_BobAOE.GA_BobAOE_C" true))
  (if _returnvalue
    (Development|PrintString "success")
    (bind _animationlength (Class|PaperZDAnimInstance|PlayAnimationOverride (Variables|/Script/PaperZD.PaperZDAnimationComponent|GetAnimInstance (Variables|Default|GetAnimationComponent)) "/Game/Assets/Animations/Enemy_Miniboss/AnimSequences/AS_Enemy_Miniboss_Ability.AS_Enemy_Miniboss_Ability" "DefaultSlot" 1.0 0.0))
    (Camera|PlayWorldCameraShake "/Game/Blueprints/Camera/BP_CamShakeROA.BP_CamShakeROA_C" (Transformation|GetActorLocation (Game|Player|GetPlayerPawn 0)) 0.0 5e+04)
    (bind _returnvalue_2 (UserInterface|CreateWidget "/Game/Blueprints/UI/AttackExplanation/WBP_AttackExplain.WBP_AttackExplain_C"))
    (Variables|/Script/UMG.TextBlock|SetText (Variables|/Game/Blueprints/UI/AttackExplanation/WBP_AttackExplain.WBP_AttackExplain_C|GetActionText _returnvalue_2) "Dark Bob used 'Ground Slam'")
    (UserInterface|Viewport|AddtoViewport _returnvalue_2 0)
    (Utilities|FlowControl|Delay (+ _animationlength 1.0))
    (Widget|RemovefromParent _returnvalue_2)
    (else
      (Development|PrintString "fail"))))

(event EventTick
  (params (DeltaSeconds :type Float%20%28single-precision%29))
  (if (GameplayTags|HasTag (Variables|Default|GetGameplay%20Tags) "(TagName=\"States.Taunted\")" true)
    (bind _output_get (Variables|Default|SetbIsTaunted true))
    (Rendering|SetVisibility (Variables|Default|GetPaperSprite) _output_get false)
    (else
      (bind _output_get_2 (Variables|Default|SetbIsTaunted false))
      (Rendering|SetVisibility (Variables|Default|GetPaperSprite) _output_get_2 false))))

(event EventPlayDeathAnimation
  (bind _animationlength (Class|PaperZDAnimInstance|PlayAnimationOverride (Variables|/Script/PaperZD.PaperZDAnimationComponent|GetAnimInstance (Variables|Default|GetAnimationComponent)) "/Game/Assets/Animations/Enemy_Miniboss/AnimSequences/AS_Enemy_Miniboss_Death.AS_Enemy_Miniboss_Death" "DefaultSlot" 1.0 0.0))
  (Actor|SetLifeSpan (- _animationlength 0.2)))

(fn ConstructionScript)