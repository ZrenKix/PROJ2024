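; Small shadow enemy unit for the arena, built on gameplay tags and the Gameplay Ability System.
; It adds the Enemy tag on BeginPlay and polls its tags every Tick to mirror States.Taunted into IsTaunted.
; The Attack event tries to activate the GA_SmallSingle ability through the ability system component and prints debug text on success or failure.
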(event EventBeginPlay
  (GameplayTags|AddGameplayTag (Variables|Default|GetGameplayTags) "(TagName=\"enemy\")" :!class /Script/GameplayTags.BlueprintGameplayTagLibrary))

(event Collision|EventActorBeginOverlap
  (params (OtherActor :type Actor%20Object%20Reference)))

(event EventTick
  (params (DeltaSeconds :type Float%20%28single-precision%29))
  (if (GameplayTags|HasTag (Variables|Default|GetGameplayTags) "(TagName=\"States.Taunted\")" true)
    (Variables|Default|SetbIsTaunted true)
    (else
      (Variables|Default|SetbIsTaunted false))))

(event EventAttack
  (bind _returnvalue (Ability|GetAbilitySystemComponent 0))
  (Utilities|IsValid _returnvalue
    (:Is%20Valid
      (bind _returnvalue_2 (Abilities|TryActivateAbilitybyClass _returnvalue "/Game/Blueprints/AbilitySystem/EnemyAbilities/GA_SmallSingle.GA_SmallSingle_C" false))
      (if _returnvalue_2
        (Development|PrintString "Casted spell")
        (else
          (Development|PrintString "Coudlnt cast spell"))))
    (:Is%20Not%20Valid
      (Development|PrintString "No valid component"))))

(fn ConstructionScript)