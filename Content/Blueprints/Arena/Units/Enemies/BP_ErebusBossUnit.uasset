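; Erebus boss enemy unit for the arena, tagged Enemy on BeginPlay, with Charge, AoE, basic attack and cooldown action events.
; AoE and basic attacks activate GAS abilities, then on success play an override animation and show a timed attack-name widget.
; Charge shows the same feedback without an ability, and CoolDown only replays the charge animation.
; Tick checks the Taunted tag but sets IsTaunted true in both branches.
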(event EventBeginPlay
  (GameplayTags|AddGameplayTag (Variables|Default|GetGameplay%20Tags) "(TagName=\"enemy\")" :!class /Script/GameplayTags.BlueprintGameplayTagLibrary))

(event Collision|EventActorBeginOverlap
  (params (OtherActor :type Actor%20Object%20Reference)))

(event EventTick
  (params (DeltaSeconds :type Float%20%28single-precision%29))
  (if (GameplayTags|HasTag (Variables|Default|GetGameplay%20Tags) "(TagName=\"States.Taunted\")" true)
    (Variables|Default|SetbIsTaunted true)
    (else
      (Variables|Default|SetbIsTaunted true))))

(event EventCoolDown
  ;[0 0.9923 1] COOLDOWN
  (Development|PrintString "Cooldown")
  (bind _animationlength (Class|PaperZDAnimInstance|PlayAnimationOverride (Variables|/Script/PaperZD.PaperZDAnimationComponent|GetAnimInstance (Variables|Default|GetAnimationComponent)) "/Game/Assets/Animations/Enemy_Boss/AnimSequences/AS_Enemy_Boss_Charge.AS_Enemy_Boss_Charge" "DefaultSlot" 1.0 0.0))
  (Utilities|FlowControl|Delay _animationlength))

(event EventBasicAttack
  ;[0 1 0.05902] Basic attack
  (Development|PrintString "BA")
  (bind _returnvalue (Abilities|TryActivateAbilitybyClass (Ability|GetAbilitySystemComponent self) "/Game/Blueprints/AbilitySystem/EnemyAbilities/GA_ErebusSingle.GA_ErebusSingle_C" true))
  (if _returnvalue
    (Development|PrintString "failed activation")
    (bind _animationlength (Class|PaperZDAnimInstance|PlayAnimationOverride (Variables|/Script/PaperZD.PaperZDAnimationComponent|GetAnimInstance (Variables|Default|GetAnimationComponent)) "/Game/Assets/Animations/Enemy_Boss/AnimSequences/AS_Enemy_Boss_BA.AS_Enemy_Boss_BA" "DefaultSlot" 1.0 0.0))
    (bind _returnvalue_2 (UserInterface|CreateWidget "/Game/Blueprints/UI/AttackExplanation/WBP_AttackExplain.WBP_AttackExplain_C"))
    (Variables|/Script/UMG.TextBlock|SetText (Variables|/Game/Blueprints/UI/AttackExplanation/WBP_AttackExplain.WBP_AttackExplain_C|GetActionText _returnvalue_2) "Erebus used 'Basic Attack'")
    (UserInterface|Viewport|AddtoViewport _returnvalue_2 0)
    (Utilities|FlowControl|Delay (+ _animationlength 1.0))
    (Widget|RemovefromParent _returnvalue_2)
    (else
      (Development|PrintString "Activation succeed" true true "(R=1.000000,G=0.381021,B=0.097409,A=1.000000)"))))

(event EventAoeAttack
  ;[1 0 0.75] AOE ATTACK
  (bind _returnvalue (Abilities|TryActivateAbilitybyClass (Ability|GetAbilitySystemComponent self) "/Game/Blueprints/AbilitySystem/EnemyAbilities/GA_ErebusAOE.GA_ErebusAOE_C" true))
  (if _returnvalue
    (Development|PrintString "failed activation")
    (bind _animationlength (Class|PaperZDAnimInstance|PlayAnimationOverride (Variables|/Script/PaperZD.PaperZDAnimationComponent|GetAnimInstance (Variables|Default|GetAnimationComponent)) "/Game/Assets/Animations/Enemy_Boss/AnimSequences/AS_Enemy_Boss_Ability.AS_Enemy_Boss_Ability" "DefaultSlot" 1.0 0.0))
    (bind _returnvalue_2 (UserInterface|CreateWidget "/Game/Blueprints/UI/AttackExplanation/WBP_AttackExplain.WBP_AttackExplain_C"))
    (Variables|/Script/UMG.TextBlock|SetText (Variables|/Game/Blueprints/UI/AttackExplanation/WBP_AttackExplain.WBP_AttackExplain_C|GetActionText _returnvalue_2) "Erebus used 'Special Attack'")
    (UserInterface|Viewport|AddtoViewport _returnvalue_2 0)
    (Utilities|FlowControl|Delay (+ _animationlength 1.0))
    (Widget|RemovefromParent _returnvalue_2)
    (else
      (Development|PrintString "Activation succeed"))))

(event EventCharge
  ;[0.1611 1 0.08185] Charge
  (Development|PrintString "Charfe")
  (bind _animationlength (Class|PaperZDAnimInstance|PlayAnimationOverride (Variables|/Script/PaperZD.PaperZDAnimationComponent|GetAnimInstance (Variables|Default|GetAnimationComponent)) "/Game/Assets/Animations/Enemy_Boss/AnimSequences/AS_Enemy_Boss_Charge.AS_Enemy_Boss_Charge" "DefaultSlot" 1.0 0.0))
  (bind _returnvalue (UserInterface|CreateWidget "/Game/Blueprints/UI/AttackExplanation/WBP_AttackExplain.WBP_AttackExplain_C"))
  (Variables|/Script/UMG.TextBlock|SetText (Variables|/Game/Blueprints/UI/AttackExplanation/WBP_AttackExplain.WBP_AttackExplain_C|GetActionText _returnvalue) "Erebus used 'Charge'")
  (UserInterface|Viewport|AddtoViewport _returnvalue 0)
  (Utilities|FlowControl|Delay (+ _animationlength 1.0))
  (Widget|RemovefromParent _returnvalue))

(fn ConstructionScript)