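; Overworld enemy encounter trigger that starts an arena fight when a player-interface actor overlaps its box.
; Overlap clears ShouldSpawn, disables collision and asks BP_DreamboundGameMode to create the arena from its Enemies and Heroes.
; When combat finishes, the triggered encounter reveals its optional PaintingPiece as interactable and destroys itself.
; ShouldSpawn persists by ActorGuid through save/load requested on BeginPlay, hiding the flipbook and disabling collision for spent encounters.
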(event OnComponentBeginOverlap(Box)
  (params (OverlappedComponent :type Primitive%20Component%20Object%20Reference) (OtherActor :type Actor%20Object%20Reference) (OtherComp :type Primitive%20Component%20Object%20Reference) (OtherBodyIndex :type Integer) (bFromSweep :type Boolean) (SweepResult :type Hit%20Result%20Structure%20%28by%20ref%29))
  (if (Utilities|DoesObjectImplementInterface OtherActor "/Game/Blueprints/Interface/BPI_PlayerInterface.BPI_PlayerInterface_C")
    (Variables|Default|SetShouldSpawn? false)
    (bind _gamemoderef (Variables|Default|GetGameModeRef)
      (:then
        (Default|CreateArena _gamemoderef (Variables|Default|GetEnemies) (Variables|Default|GetHeroes) "None" 2)
        (Variables|Default|SetisActive false)
        (Collision|SetCollisionEnabled (Variables|Default|GetBox) "NoCollision")
        (Development|PrintString (Utilities|String|ToString(Boolean) (Variables|Default|GetShouldSpawn?))))
      (:else))))

(event Custom|HandleDestroy
  (if (not (Variables|Default|GetisActive))
    (Utilities|FlowControl|Delay 0.3)
    (bind _paintingpiece (Variables|Default|GetPaintingPiece)
      (:then
        (Rendering|SetActorHiddenInGame _paintingpiece false)
        (Variables|/Game/Blueprints/Interaction/BP_PaintingPiece.BP_PaintingPiece_C|SetisInteractable (Variables|Default|GetPaintingPiece) true)
        (Actor|DestroyActor))
      (:else
        (Actor|DestroyActor)))))

(event EventBeginPlay
  (bind _asbp_game_instance (Utilities|Casting|CastToBP_GameInstance (Game|GetGameInstance)))
  (Default|RequestLoad _asbp_game_instance self)
  (bind _asbp_dreambound_game_mode (Utilities|Casting|CastToBP_DreamboundGameMode (Game|GetGameMode)))
  (Variables|Default|SetGameModeRef _asbp_dreambound_game_mode)
  (bind _spawn (CallFunction|HandleSpawn))
  (if _spawn
    (EventDispatchers|BindEventtoOnCombatFinished (Subsystems|GetArenaManager) (delegate Custom|HandleDestroy))))

(event EventSaveData
  (params (SaveGameRef :type BP%20Save%20Game%20Object%20Reference))
  (bind _shouldspawn_ (Variables|Default|GetShouldSpawn?))
  (Utilities|Map|Add (Variables|/Game/Assets/Save/BP_SaveGame.BP_SaveGame_C|GetEnemyEncounters SaveGameRef) (Variables|Default|GetActorGuid) _shouldspawn_)
  (Development|PrintString (Utilities|String|ToString(Boolean) _shouldspawn_) true true "(R=0.000000,G=1.000000,B=0.029325,A=1.000000)"))

(event EventLoadData
  (params (SaveGameRef :type BP%20Save%20Game%20Object%20Reference))
  (bind _actorguid (Variables|Default|GetActorGuid))
  (bind _enemyencounters (Variables|/Game/Assets/Save/BP_SaveGame.BP_SaveGame_C|GetEnemyEncounters SaveGameRef))
  (bind (_value _returnvalue) (Utilities|Map|Find _enemyencounters _actorguid))
  (if _returnvalue
    (bind _output_get (Variables|Default|SetShouldSpawn? _value))
    (Development|PrintString (Utilities|String|ToString(Boolean) _output_get))))

(fn ConstructionScript)

(fn HandleSpawn
  (if (Variables|Default|GetShouldSpawn?)
    (return (Variables|Default|GetShouldSpawn?))
    (else
      (Collision|SetCollisionEnabled (Variables|Default|GetBox) "NoCollision")
      (Development|SetHiddeninGame (Variables|Default|GetPaperFlipbook) true false))))