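; Temporary interactable actor that offers a "Start Combat" prompt to launch an arena fight.
; On interact, it asks the Dreambound game mode, cached at BeginPlay, to create an arena from its enemy and hero lists with no bossfight type.
; It then binds to the arena manager's combat-finished event and, if DropPiece is set, immediately replaces itself with a BP_PaintingPiece at its transform.
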(event EventBeginPlay
  (bind _asbp_dreambound_game_mode (Utilities|Casting|CastToBP_DreamboundGameMode (Game|GetGameMode)))
  (Variables|Default|SetGameModeRef _asbp_dreambound_game_mode))

(event EventTick
  (params (DeltaSeconds :type Float%20%28single-precision%29)))

(fn ConstructionScript)

(fn DropPaintingPiece
  (Actor|DestroyActor)
  (Game|SpawnActorfromClass "/Game/Blueprints/Interaction/BP_PaintingPiece.BP_PaintingPiece_C" (Transformation|GetActorTransform) "Undefined" "MultiplyWithRoot" 0 0))

(fn GetInteractPrompt
  (return "Start Combat"))

(fn Interact
  (bind _gamemoderef (Variables|Default|GetGameModeRef)
    (:then
      (Default|CreateArena _gamemoderef (Variables|Default|GetEnemies) (Variables|Default|GetHeros) "None")
      (EventDispatchers|BindEventtoOnCombatFinished (Subsystems|GetArenaManager) (EventDispatchers|CreateEvent :!event K2DestroyActor))
      (if (Variables|Default|GetDropPiece)
        (CallFunction|DropPaintingPiece)
        (return false)
        (else
          (return false))))
    (:else)))