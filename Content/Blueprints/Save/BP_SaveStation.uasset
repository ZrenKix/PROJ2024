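; BP_SaveStation is an interactable save point that lets the player save the game.
; On Interact it binds a completion callback to BP_GameInstance's game-saved event and calls RequestSaveMessage, leaving the save itself outside this Blueprint.
; When saving completes, it prints a green "Saved!" debug string and re-enables interaction on BP_PlayerHero.
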(event Custom|SavingCompleted
  (params (SaveGameRef :type BP%20Save%20Game%20Object%20Reference))
  ;[1 1 1] Interaction / Save game
  (Development|PrintString "Saved!" true true "(R=0.112619,G=1.000000,B=0.000000,A=1.000000)" 1.0)
  (|LetPlayerInteractAgain))

(event EventBeginPlay)

(event Collision|EventActorBeginOverlap
  (params (OtherActor :type Actor%20Object%20Reference)))

(event EventTick
  (params (DeltaSeconds :type Float%20%28single-precision%29)))

(event EventInteract
  ;[1 1 1] Interaction / Save game
  (bind _asbp_game_instance (Utilities|Casting|CastToBP_GameInstance (Game|GetGameInstance)))
  (EventDispatchers|BindEventtoGameSaved _asbp_game_instance (delegate Custom|SavingCompleted))
  (Class|BPIPersistence|RequestSave(Message) _asbp_game_instance true))

(fn ConstructionScript)