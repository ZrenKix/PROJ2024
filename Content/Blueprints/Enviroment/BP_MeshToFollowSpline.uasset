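; BP_MeshToFollowSpline is an interactable floating object that travels along a spline while spinning.
; On BeginPlay it finds a BP_SplineForObjectsToFollow actor, and a timeline scaled by TimeToComplete moves it along that spline's length.
; RerollRotator gives RotatingMovement one random rate on all three axes, rerolling near-zero values.
; Interacting shows a text popup with Edith's portrait remarking on the floating, and returns false.
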(event Custom|MoveObject
  (Components|Timeline|SetPlayRate (Variables|Default|GetMoveObjectT) (/ 1.0 (Variables|Default|GetTimeToComplete)))
  (bind _movetrack (Timeline|MoveObjectT Play)
    (:Update
      (Transformation|SetActorLocation (Spline|GetLocationatDistanceAlongSpline (Variables|/Game/Blueprints/Enviroment/BP_SplineForObjectsToFollow.BP_SplineForObjectsToFollow_C|GetSpline (Variables|Default|GetSplineRef)) (Math|Float|Lerp 0.0 (Spline|GetSplineLength (Variables|/Game/Blueprints/Enviroment/BP_SplineForObjectsToFollow.BP_SplineForObjectsToFollow_C|GetSpline (Variables|Default|GetSplineRef))) _movetrack) "World") false false))))

(event EventBeginPlay
  (bind _returnvalue (Actor|GetActorOfClass "/Game/Blueprints/Enviroment/BP_SplineForObjectsToFollow.BP_SplineForObjectsToFollow_C"))
  (Variables|Default|SetSplineRef _returnvalue)
  (CallFunction|MoveObject)
  (bind _outrotator (CallFunction|RerollRotator))
  (Variables|/Script/Engine.RotatingMovementComponent|SetRotationRate (Variables|Default|GetRotatingMovement) _outrotator))

(fn ConstructionScript
  (Variables|Default|SetSplineRef 0))

(fn RerollRotator
  (bind _output_get (LocalVariables|SetRandomFloat (Math|Random|RandomFloatinRange -5e+01 5e+01)))
  (while (and (>= _output_get -5.0) (<= _output_get 5.0))
    (LocalVariables|SetRandomFloat (Math|Random|RandomFloatinRange -25.0 25.0)))
  (bind _output_get_2 (Variables|Default|SetRandomizedRotator (Math|Rotator|MakeRotator (LocalVariables|GetRandomFloat) (LocalVariables|GetRandomFloat) (LocalVariables|GetRandomFloat))))
  (return _output_get_2))

(fn GetInteractPrompt
  (return ""))

(fn Interact
  (bind _returnvalue (UserInterface|CreateWidget "/Game/Blueprints/UI/Interaction/WBP_TextPopup.WBP_TextPopup_C" 0 "Thats weird, why is it floating?" "Edith" "/Game/Assets/UI/NewUI/T_UI_Card_Character_Edith.T_UI_Card_Character_Edith"))
  (UserInterface|Viewport|AddtoViewport _returnvalue 0)
  (return false))