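; BP_TrippyObject is an environment actor whose scale animates from the moment play begins.
; A Timeline scale curve multiplies the stored original scale on each update, and the result is also printed as debug output.
; An unused RerollRotator function builds a random roll and pitch rotator from one shared value.
; Its reroll loop draws from the same narrow band it rejects, so it cannot exit once entered.
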(event EventBeginPlay
  (Variables|Default|SetOrginalScale (Transformation|GetActorScale3D))
  (bind _scalecurve (Timeline|Timeline Play)
    (:Update
      (Development|PrintString (Utilities|String|ToString(Vector) (* _scalecurve (Variables|Default|GetOrginalScale))))
      (Transformation|SetActorScale3D (* _scalecurve (Variables|Default|GetOrginalScale))))))

(fn ConstructionScript)

(fn RerollRotator
  (bind _output_get (LocalVariables|SetRandomFloat (Math|Random|RandomFloatinRange -25.0 25.0)))
  (while (and (>= _output_get -5.0) (<= _output_get 5.0))
    (LocalVariables|SetRandomFloat (Math|Random|RandomFloatinRange -5.0 5.0)))
  (bind _output_get_2 (Variables|Default|SetRandomizedRotator (Math|Rotator|MakeRotator (LocalVariables|GetRandomFloat) (LocalVariables|GetRandomFloat) 0.0)))
  (return _output_get_2))