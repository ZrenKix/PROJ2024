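; BP_TextTrigger is a one-shot trigger box that shows a text popup when the player hero walks into it.
; On overlap it disables the hero's movement and creates a WBP_TextPopup with hardcoded text.
; The popup's OnDone callback turns off box collision and marks the trigger completed, but does not restore movement here.
; Completion is saved by object name, and BeginPlay asks the GameInstance to load it.
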(event OnComponentBeginOverlap(Box)
  (params (OverlappedComponent :type Primitive%20Component%20Object%20Reference) (OtherActor :type Actor%20Object%20Reference) (OtherComp :type Primitive%20Component%20Object%20Reference) (OtherBodyIndex :type Integer) (bFromSweep :type Boolean) (SweepResult :type Hit%20Result%20Structure%20%28by%20ref%29))
  ;[1 1 1] Handle Player trigger
  (if (not (Variables|Default|GethasCompleted?))
    (bind _asbp_player_hero (Utilities|Casting|CastToBP_PlayerHero OtherActor))
    (Pawn|Components|CharacterMovement|DisableMovement (Variables|/Script/Engine.Character|GetCharacterMovement _asbp_player_hero))
    (bind _returnvalue (UserInterface|CreateWidget "/Game/Blueprints/UI/Interaction/WBP_TextPopup.WBP_TextPopup_C" 0 "Where am I?"))
    (bind _output_get (Variables|Default|SetTextWidget _returnvalue))
    (UserInterface|Viewport|AddtoViewport _output_get 0)
    (EventDispatchers|AssignOnDone (Variables|Default|GetTextWidget) (delegate Custom|OnDone_Event))))

(event Custom|OnDone_Event
  ;[1 1 1] Handle Player trigger
  (Collision|SetCollisionEnabled (Variables|Default|GetBox) "NoCollision")
  (Variables|Default|SethasCompleted? true))

(event EventBeginPlay
  ;[1 1 1] BeginPlay
  (Class|BPIPersistence|RequestLoad(Message) (Game|GetGameInstance) self))

(event EventLoadData
  (params (SaveGameRef :type BP%20Save%20Game%20Object%20Reference))
  ;[1 1 1] Load data
  (Variables|Default|SethasCompleted? (.Value (Utilities|Map|Find (Variables|/Game/Assets/Save/BP_SaveGame.BP_SaveGame_C|GetTextTriggers SaveGameRef) (Utilities|GetObjectName self)))))

(event EventSaveData
  (params (SaveGameRef :type BP%20Save%20Game%20Object%20Reference))
  ;[1 1 1] Save data
  (Utilities|Map|Add (Variables|/Game/Assets/Save/BP_SaveGame.BP_SaveGame_C|GetTextTriggers SaveGameRef) (Utilities|GetObjectName self) (Variables|Default|GethasCompleted?)))

(fn ConstructionScript)