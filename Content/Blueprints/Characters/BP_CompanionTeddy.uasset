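; Teddy companion that can be talked to and follows the player pawn once unlocked.
; In TheHub, the first interaction shows its intro dialogue and sets CanFollow; any other interaction calls Yeet.
; CanFollow persists in the save game by ActorGuid; BeginPlay requests a load from the game instance, then starts following if it is set.
; Interact does not start following itself, and the arena combat-finished binding never runs.
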(event Custom|FollowPlayerHero
  (Class|CompanionCharacter|FollowTargetActor (Game|Player|GetPlayerPawn 0)))

(event EventBeginPlay
  (Variables|Default|SetfollowDistanceThreshold 1e+02)
  (Variables|Default|SetMovementSpeed 5e+02)
  (bind _asbp_game_instance (Utilities|Casting|CastToBP_GameInstance (Game|GetGameInstance)))
  (Default|RequestLoad _asbp_game_instance self)
  (if (Variables|Default|GetbCanFollow)
    (CallFunction|FollowPlayerHero)))

(event Collision|EventActorBeginOverlap
  (params (OtherActor :type Actor%20Object%20Reference)))

(event EventTick
  (params (DeltaSeconds :type Float%20%28single-precision%29)))

(event EventSaveData
  (params (SaveGameRef :type BP%20Save%20Game%20Object%20Reference))
  ;[1 1 1] Save data
  (Utilities|Map|Add (Variables|/Game/Assets/Save/BP_SaveGame.BP_SaveGame_C|GetSpawnableActors SaveGameRef) (Variables|Default|GetActorGuid) (Variables|Default|GetbCanFollow)))

(event EventLoadData
  (params (SaveGameRef :type BP%20Save%20Game%20Object%20Reference))
  (bind _actorguid (Variables|Default|GetActorGuid))
  (bind _spawnableactors (Variables|/Game/Assets/Save/BP_SaveGame.BP_SaveGame_C|GetSpawnableActors SaveGameRef))
  (bind (_value _returnvalue) (Utilities|Map|Find _spawnableactors _actorguid))
  ;[1 1 1] Load data
  (if _returnvalue
    (Variables|Default|SetbCanFollow _value)))

(fn ConstructionScript)

(fn Interact
  (bind _returnvalue (Game|GetCurrentLevelName true))
  (if (and (Utilities|Enum|Equal(Enum) _returnvalue (Variables|Default|GetTheHub)) (Variables|Default|GetisInteractable))
    (bind _returnvalue_2 (Game|ConstructObjectfromClass "/Game/Blueprints/Arena/BP_TeddyIntro.BP_TeddyIntro_C"))
    (bind _returnvalue_3 (UserInterface|CreateWidget "/Game/Blueprints/Arena/Widgets/WBP_DialogueOpenWorld.WBP_DialogueOpenWorld_C"))
    (UserInterface|Viewport|AddtoViewport _returnvalue_3 0)
    (Widget|SetVisibility _returnvalue_3 "Visible")
    (Default|DisplayEntry _returnvalue_3 0 "/Game/Assets/UI/Card/T_UI_Card_Character_Bear.T_UI_Card_Character_Bear" _returnvalue_2)
    (Variables|Default|SetisInteractable false)
    (Variables|Default|SetbCanFollow true)
    (else
      (Class|CompanionCharacter|Yeet)))
  (return false))

(fn GetInteractPrompt
  (return "Talk to Teddy"))