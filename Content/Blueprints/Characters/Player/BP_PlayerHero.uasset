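; Player hero Blueprint that lets the character interact with world objects and shows their prompts.
; IA_Interact has two handlers, messaging the first overlapping interface implementer or the interactable hit by a line trace.
; A shared LineTrace helper casts a debug-drawn Visibility ray along the actor's forward vector.
; Tick uses it to show the targeted InteractableBase's prompt, hiding the last one's when none is hit.
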(event Input|EnhancedActionEvents|EnhancedInputActionIA_Interact
  (params (ActionValue :type Boolean) (ElapsedSeconds :type Float%20%28double-precision%29) (TriggeredSeconds :type Float%20%28double-precision%29) (InputAction :type Input%20Action%20Object%20Reference :default "/Game/Blueprints/Input/InputActions/IA_Interact.IA_Interact"))
  ;[1 1 1] Interaction via line trace
  (:Started
    (bind _hitactor (CallFunction|LineTrace))
    (if (Utilities|DoesObjectImplementInterface _hitactor "/Script/PROJ.InteractableInterface")
      (Class|InteractableInterface|Interact(Message) _hitactor))))

(event Input|EnhancedActionEvents|EnhancedInputActionIA_Interact
  (params (ActionValue :type Boolean) (ElapsedSeconds :type Float%20%28double-precision%29) (TriggeredSeconds :type Float%20%28double-precision%29) (InputAction :type Input%20Action%20Object%20Reference :default "/Game/Blueprints/Input/InputActions/IA_Interact.IA_Interact"))
  ;[1 1 1] Interaction via overlapping
  (:Started
    (bind _array_element (Utilities|Array|ForEachLoopwithBreak (Collision|GetOverlappingActors "/Script/Engine.Actor" :!class /Script/Engine.Actor) :!label _label)
      (:LoopBody
        (if (Utilities|DoesObjectImplementInterface _array_element 0)
          (Class|InteractableInterface|Interact(Message) _array_element)
          (goto _label Break))))))

(event EventBeginPlay)

(event Collision|EventActorBeginOverlap
  (params (OtherActor :type Actor%20Object%20Reference)))

(event EventTick
  (params (DeltaSeconds :type Float%20%28single-precision%29))
  (bind _hitactor (CallFunction|LineTrace))
  (bind _asinteractable_base (Utilities|Casting|CastToInteractableBase _hitactor)
    (:then
      (Variables|Default|SetLast%20Interactable _asinteractable_base)
      (Class|InteractableBase|ShowPromptText _asinteractable_base))
    (:CastFailed
      (bind _last_interactable (Variables|Default|GetLast%20Interactable)
        (:then
          (Class|InteractableBase|HidePromptText _last_interactable))
        (:else)))))

(fn ConstructionScript)

(fn LineTrace
  (bind _returnvalue (Transformation|GetActorLocation))
  (bind (_outhit _returnvalue_2) (Collision|LineTraceByChannel _returnvalue (+ _returnvalue (* (Transformation|GetActorForwardVector) (LocalVariables|GetLine%20Trace%20Range))) "TraceTypeQuery1" false 0 "ForOneFrame"))
  (return _returnvalue_2 (.HitActor (Collision|BreakHitResult _outhit))))