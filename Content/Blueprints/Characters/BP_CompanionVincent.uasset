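; BP_CompanionVincent is the Vincent companion character, with follow movement and a comfort interaction.
; BeginPlay sets its follow distance threshold and movement speed, and the FollowPlayerHero event calls FollowTargetActor on TeddyFollow.
; The binding of that event to the arena manager's combat-finished event is disconnected, and Tick is empty.
; Interact prints a debug message, sets IsComforted and returns false.
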(event Custom|FollowPlayerHero
  (Class|CompanionCharacter|FollowTargetActor (Variables|Default|GetTeddyFollow)))

(event Custom|CustomEvent
  (params (DeltaSeconds :type Float%20%28single-precision%29)))

(event EventBeginPlay
  (Variables|Default|SetfollowDistanceThreshold 1e+02)
  (Variables|Default|SetMovementSpeed 5e+02))

(event EventTick
  (params (DeltaSeconds :type Float%20%28single-precision%29)))

(fn ConstructionScript)

(fn Interact
  (Development|PrintString "Interact with Vincent")
  (Variables|Default|SetbIsComforted true)
  (return false))