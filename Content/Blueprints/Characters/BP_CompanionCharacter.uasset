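; Companion character Blueprint with unfinished logic for following the player hero after arena combat.
; On BeginPlay it binds FollowPlayerHero to the arena manager's combat-finished event, but that handler only waits through a delay.
; Disconnected nodes would register the companion with BP_PlayerHero and move it via AI controller, but never run.
; Interaction is stubbed out, returning false and an empty prompt.
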(event Custom|FollowPlayerHero
  (Utilities|FlowControl|Delay 2.0))

(event EventBeginPlay
  (EventDispatchers|BindEventtoOnCombatFinished (Subsystems|GetArenaManager) (delegate Custom|FollowPlayerHero)))

(event Collision|EventActorBeginOverlap
  (params (OtherActor :type Actor%20Object%20Reference)))

(event EventTick
  (params (DeltaSeconds :type Float%20%28single-precision%29)))

(fn ConstructionScript)

(fn Interact
  (return false))

(fn GetInteractPrompt
  (return ""))