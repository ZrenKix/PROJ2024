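; BP_ResetColor is a painting puzzle interactable that, despite its name, prompts "Check color" and triggers a check of the puzzle's result.
; Interact calls CheckResult on its ResultColor reference and returns false.
; On BeginPlay it creates a dynamic instance of mesh material slot 1 and caches its BaseColor in MyColor, which is not used elsewhere in these graphs.
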(event EventBeginPlay
  (bind _returnvalue (Rendering|Material|CreateDynamicMaterialInstance (Rendering|Material|GetMaterial (Variables|Default|GetStaticMesh) 1) "None" "None" :!class /Script/Engine.KismetMaterialLibrary))
  (bind _returnvalue_2 (Rendering|Material|GetVectorParameterValue _returnvalue "BaseColor" :!class /Script/Engine.MaterialInstanceDynamic))
  (Variables|Default|SetMyColor _returnvalue_2))

(fn ConstructionScript)

(fn GetInteractPrompt
  (return "Check color"))

(fn Interact
  (Default|CheckResult (Variables|Default|GetResultColor))
  (return false))