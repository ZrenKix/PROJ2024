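; Interactable lever in the painting puzzle that feeds its own color into a ResultColor object for mixing.
; On BeginPlay it reads MyColor from the BaseColor parameter of its mesh's second material, via a dynamic instance.
; When interactable it shows a "Mix" prompt, and Interact writes MyColor into ResultColor's first or second slot, treating white as empty, then calls MixColors.
; If both slots are filled, interaction changes nothing.
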(event EventBeginPlay
  (bind _returnvalue (Rendering|Material|CreateDynamicMaterialInstance (Rendering|Material|GetMaterial (Variables|Default|GetStaticMesh) 1) "None" "None" :!class /Script/Engine.KismetMaterialLibrary))
  (bind _returnvalue_2 (Rendering|Material|GetVectorParameterValue _returnvalue "BaseColor" :!class /Script/Engine.MaterialInstanceDynamic))
  (Variables|Default|SetMyColor _returnvalue_2))

(fn ConstructionScript)

(fn GetInteractPrompt
  (if (Variables|Default|GetisInteractable)
    (return "Mix")
    (else
      (return ""))))

(fn Interact
  (if (Variables|Default|GetisInteractable)
    (if (== (Variables|/Game/Blueprints/PaintingPuzzle/BP_ResultColor.BP_ResultColor_C|GetFirstColor (Variables|Default|GetResultColor)) "(R=1.000000,G=1.000000,B=1.000000,A=1.000000)")
      (Variables|/Game/Blueprints/PaintingPuzzle/BP_ResultColor.BP_ResultColor_C|SetFirstColor (Variables|Default|GetResultColor) (Variables|Default|GetMyColor))
      (Default|MixColors (Variables|Default|GetResultColor) :!label _label)
      (elif (== (Variables|/Game/Blueprints/PaintingPuzzle/BP_ResultColor.BP_ResultColor_C|GetSecondColor (Variables|Default|GetResultColor)) "(R=1.000000,G=1.000000,B=1.000000,A=1.000000)")
        (Variables|/Game/Blueprints/PaintingPuzzle/BP_ResultColor.BP_ResultColor_C|SetSecondColor (Variables|Default|GetResultColor) (Variables|Default|GetMyColor))
        (goto _label)))))