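; Painting puzzle actor that displays the mix of two colors on its mesh and checks it against a goal color.
; SetValues feeds two dynamic material parameters, hard-coding yellow mixes as orange or green, and disables the linked levers once two colors are in.
; CheckResult compares the material's first color with GoalColor, then either unlocks the bars or resets the colors and levers for another try.
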(event EventBeginPlay
  (bind _staticmesh (Variables|Default|GetStaticMesh))
  (bind _returnvalue (Rendering|Material|CreateDynamicMaterialInstance _staticmesh 1 (Rendering|Material|GetMaterial _staticmesh 1) "None" :!class /Script/Engine.PrimitiveComponent))
  (bind _output_get (Variables|Default|SetDynamicMaterial _returnvalue))
  (bind _returnvalue_2 (Rendering|Material|GetVectorParameterValue _output_get "FirstColor" :!class /Script/Engine.MaterialInstanceDynamic))
  (bind _output_get_2 (Variables|Color|SetStartingColor _returnvalue_2))
  (CallFunction|SetValues _output_get_2))

(fn ConstructionScript)

(fn SetValues
  (params (FirstColor :type Linear%20Color%20Structure) (SecondColor :type Linear%20Color%20Structure))
  (Variables|Color|SetFirstColor FirstColor)
  (Variables|Color|SetSecondColor SecondColor)
  (if (== (Variables|Color|GetFirstColor) "(R=1.000000,G=1.000000,B=0.000000,A=1.000000)")
    (CallFunction|FirstColorYellow)
    (elif (== (Variables|Color|GetSecondColor) "(R=1.000000,G=1.000000,B=0.000000,A=1.000000)")
      (CallFunction|SecondColorYellow)
      (else
        (Rendering|Material|SetVectorParameterValue (Variables|Default|GetDynamicMaterial) "FirstColor" (Variables|Color|GetFirstColor) :!class /Script/Engine.MaterialInstanceDynamic)
        (Rendering|Material|SetVectorParameterValue (Variables|Default|GetDynamicMaterial) "SecondColor" (Variables|Color|GetSecondColor) :!class /Script/Engine.MaterialInstanceDynamic)
        (if (not (== (Variables|Color|GetSecondColor) ""))
          (CallFunction|StopLeverInteraction))))))

(fn NormalizeColor
  (params (Color :type Linear%20Color%20Structure))
  (bind (_r _g _b) (Math|Color|BreakColor Color))
  (bind _output_get (Variables|Default|SetMaxChannelValue (Class|KismetMathLibrary|LinearColorGetMax Color)))
  (return (Utilities|Struct|MakeLinearColor (/ _r _output_get) (/ _g _output_get) (/ _b _output_get) 1.0)))

(fn CheckResult
  (bind _returnvalue (Rendering|Material|GetVectorParameterValue (Variables|Default|GetDynamicMaterial) "FirstColor" :!class /Script/Engine.MaterialInstanceDynamic))
  (if (== _returnvalue (Variables|Color|GetGoalColor))
    (Development|PrintString "You did it!")
    (Default|UnlockBars (Variables|Default|GetBars))
    (else
      (Development|PrintString "Try again!")
      (Rendering|Material|SetVectorParameterValue (Variables|Default|GetDynamicMaterial) "FirstColor" "(R=1.000000,G=1.000000,B=1.000000,A=1.000000)" :!class /Script/Engine.MaterialInstanceDynamic)
      (Rendering|Material|SetVectorParameterValue (Variables|Default|GetDynamicMaterial) "SecondColor" "(R=0.000000,G=0.000000,B=0.000000,A=1.000000)" :!class /Script/Engine.MaterialInstanceDynamic)
      (Variables|Color|SetStartingColor "(R=1.000000,G=1.000000,B=1.000000,A=1.000000)")
      (CallFunction|ResetLevers)
      (Variables|Default|SetActiveLevers 0)
      (Variables|Color|SetFirstColor "(R=1.000000,G=1.000000,B=1.000000,A=1.000000)")
      (Variables|Color|SetSecondColor "(R=1.000000,G=1.000000,B=1.000000,A=1.000000)"))))

(fn ResetLevers
  (for _array_element (Variables|Default|GetLevers)
    (Variables|/Game/Blueprints/PaintingPuzzle/BP_Lever.BP_Lever_C|SetisInteractable _array_element true)))

(fn SetColortoYellow
  (Rendering|Material|SetVectorParameterValue (Variables|Default|GetDynamicMaterial) "FirstColor" "(R=1.000000,G=1.000000,B=0.000000,A=1.000000)" :!class /Script/Engine.MaterialInstanceDynamic))

(fn FirstColorYellow
  (if (== (Variables|Color|GetSecondColor) "")
    (Rendering|Material|SetVectorParameterValue (Variables|Default|GetDynamicMaterial) "FirstColor" "(R=1.000000,G=1.000000,B=0.000000,A=1.000000)" :!class /Script/Engine.MaterialInstanceDynamic)
    (else
      (if (== (Variables|Color|GetSecondColor) "(R=1.000000,G=0.000000,B=0.000000,A=1.000000)")
        (Rendering|Material|SetVectorParameterValue (Variables|Default|GetDynamicMaterial) "FirstColor" "(R=1.000000,G=0.500000,B=0.000000,A=1.000000)" :!class /Script/Engine.MaterialInstanceDynamic)
        (else
          (Rendering|Material|SetVectorParameterValue (Variables|Default|GetDynamicMaterial) "FirstColor" "(R=0.000000,G=1.000000,B=0.000000,A=1.000000)" :!class /Script/Engine.MaterialInstanceDynamic)))
      (Rendering|Material|SetVectorParameterValue :self (Variables|Default|GetDynamicMaterial) :ParameterName "SecondColor" :!class /Script/Engine.MaterialInstanceDynamic)
      (CallFunction|StopLeverInteraction))))

(fn StopLeverInteraction
  (for _array_element (Variables|Default|GetLevers)
    (Variables|/Game/Blueprints/PaintingPuzzle/BP_Lever.BP_Lever_C|SetisInteractable _array_element false)))

(fn SecondColorYellow
  (if (== (Variables|Color|GetFirstColor) "(R=1.000000,G=0.000000,B=0.000000,A=1.000000)")
    (Rendering|Material|SetVectorParameterValue (Variables|Default|GetDynamicMaterial) "FirstColor" "(R=1.000000,G=0.500000,B=0.000000,A=1.000000)" :!class /Script/Engine.MaterialInstanceDynamic)
    (else
      (Rendering|Material|SetVectorParameterValue (Variables|Default|GetDynamicMaterial) "FirstColor" "(R=0.000000,G=1.000000,B=0.000000,A=1.000000)" :!class /Script/Engine.MaterialInstanceDynamic)))
  (Rendering|Material|SetVectorParameterValue :self (Variables|Default|GetDynamicMaterial) :ParameterName "SecondColor" :!class /Script/Engine.MaterialInstanceDynamic)
  (CallFunction|StopLeverInteraction))