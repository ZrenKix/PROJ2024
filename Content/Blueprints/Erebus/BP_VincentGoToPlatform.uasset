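; Trigger actor in Erebus that plays a dialogue when companion Vincent overlaps it, then sends him to the VincentGoTo target.
; BeginPlay caches the player and open-world dialogue widget after a short delay.
; Overlap rotates Vincent, disables both characters' movement and displays the dialogue.
; Tick polls the widget's entry index; at entry 1, after a delay, it retargets Vincent's follow with zero threshold and restores walking for both.
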(event EventBeginPlay
  (Utilities|FlowControl|Delay 1.0)
  (bind _returnvalue (Actor|GetActorOfClass "/Game/Blueprints/Characters/Player/BP_PlayerHero.BP_PlayerHero_C"))
  (Variables|Default|SetPlayer _returnvalue)
  (bind _foundwidgets (Widget|GetAllWidgetsOfClass "/Game/Blueprints/Arena/Widgets/WBP_DialogueOpenWorld.WBP_DialogueOpenWorld_C" true))
  (bind _array_element (Utilities|Array|ForEachLoopwithBreak _foundwidgets)))

(event Collision|EventActorBeginOverlap
  (params (OtherActor :type Actor%20Object%20Reference))
  (bind _asbp_companion_vincent (Utilities|Casting|CastToBP_CompanionVincent OtherActor))
  (bind _returnvalue (Game|ConstructObjectfromClass "/Game/Blueprints/Arena/BP_ErabusDialogueSecond.BP_ErabusDialogueSecond_C"))
  (Transformation|SetActorRotation _asbp_companion_vincent (Math|Rotator|MakeRotator 0.0 (.Y (Math|Vector|BreakVector (Transformation|GetActorLocation (Variables|Default|GetVincentGoTo)))) 0.0))
  (Pawn|Components|CharacterMovement|SetMovementMode (Variables|/Script/Engine.Character|GetCharacterMovement _asbp_companion_vincent) "MOVE_None" 0)
  (Pawn|Components|CharacterMovement|SetMovementMode (Variables|/Script/Engine.Character|GetCharacterMovement (Variables|Default|GetPlayer)) "MOVE_None" 0)
  (Utilities|FlowControl|Delay 0.5)
  (Default|DisplayEntry (stale EventBeginPlay _array_element) 0 "/Game/Assets/UI/Card/T_UI_Card_Character_Bear.T_UI_Card_Character_Bear" _returnvalue))

(event EventTick
  (params (DeltaSeconds :type Float%20%28single-precision%29))
  (if (not (== (Variables|/Game/Blueprints/Arena/Widgets/WBP_DialogueOpenWorld.WBP_DialogueOpenWorld_C|GetCurrentEntry (stale EventBeginPlay _array_element)) (Variables|Default|GetOldCurrentEntry)))
    (Variables|Default|SetOldCurrentEntry (Variables|/Game/Blueprints/Arena/Widgets/WBP_DialogueOpenWorld.WBP_DialogueOpenWorld_C|GetCurrentEntry (stale EventBeginPlay _array_element)))
    (switch int (Variables|/Game/Blueprints/Arena/Widgets/WBP_DialogueOpenWorld.WBP_DialogueOpenWorld_C|GetCurrentEntry (stale EventBeginPlay _array_element))
      (:1
        (Utilities|FlowControl|Delay 1.0)
        (Class|CompanionCharacter|SetFollowTarget (stale Collision|EventActorBeginOverlap _asbp_companion_vincent) (Variables|Default|GetVincentGoTo))
        (Variables|/Script/PROJ.CompanionCharacter|SetfollowDistanceThreshold (stale Collision|EventActorBeginOverlap _asbp_companion_vincent) 0.0)
        (Pawn|Components|CharacterMovement|SetMovementMode (Variables|/Script/Engine.Character|GetCharacterMovement (Variables|Default|GetPlayer)) "MOVE_Walking" 0)
        (Pawn|Components|CharacterMovement|SetMovementMode (Variables|/Script/Engine.Character|GetCharacterMovement (stale Collision|EventActorBeginOverlap _asbp_companion_vincent)) "MOVE_Walking" 0)))))

(fn ConstructionScript)