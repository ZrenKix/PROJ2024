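; BP_LowerSpeed is an overlap-triggered actor that sets movement speed for the player hero, with intended handling for Teddy and Vincent companions.
; On overlap it casts the same actor to hero, Teddy, then Vincent in one chain, so each companion step requires the previous casts to succeed.
; Successful casts set max walk speed from player or companion variables; companion steps also enable following, and the chain ends with debug speed prints.
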(event EventBeginPlay)

(event Collision|EventActorBeginOverlap
  (params (OtherActor :type Actor%20Object%20Reference))
  (bind _newcompanionspeed (Variables|Default|GetNewCompanionSpeed))
  (bind _asbp_player_hero (Utilities|Casting|CastToBP_PlayerHero OtherActor))
  (bind _output_get (Variables|/Script/Engine.CharacterMovementComponent|SetMaxWalkSpeed (Variables|/Script/Engine.Character|GetCharacterMovement _asbp_player_hero) (Variables|Default|GetNewPlayerSpeed)))
  (bind _asbp_companion_teddy (Utilities|Casting|CastToBP_CompanionTeddy OtherActor))
  (Variables|/Script/PROJ.CompanionCharacter|SetbCanFollow _asbp_companion_teddy true)
  (Variables|/Script/Engine.CharacterMovementComponent|SetMaxWalkSpeed (Variables|/Script/Engine.Character|GetCharacterMovement _asbp_companion_teddy) _newcompanionspeed)
  (bind _asbp_companion_vincent (Utilities|Casting|CastToBP_CompanionVincent OtherActor))
  (Variables|/Script/PROJ.CompanionCharacter|SetbCanFollow _asbp_companion_vincent true)
  (bind _output_get_2 (Variables|/Script/Engine.CharacterMovementComponent|SetMaxWalkSpeed (Variables|/Script/Engine.Character|GetCharacterMovement _asbp_companion_vincent) _newcompanionspeed))
  (Development|PrintString (Utilities|String|ToString(Float) _output_get_2))
  (Development|PrintString (Utilities|String|ToString(Float) _output_get)))

(event EventTick
  (params (DeltaSeconds :type Float%20%28single-precision%29)))

(fn ConstructionScript)