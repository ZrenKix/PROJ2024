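; BP_StoneTrigger is a trigger actor that stages a scripted stone movement when BP_PlayerHero overlaps it.
; The overlap disables the hero's movement and sets a flag that lets Tick interpolate Stone1's Z toward StoneTargetLocation while restarting a camera shake every frame.
; A Delay inside Tick restores walking after about five seconds and destroys the trigger, so it fires only once.
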(event EventBeginPlay)

(event Collision|EventActorBeginOverlap
  (params (OtherActor :type Actor%20Object%20Reference))
  (bind _asbp_player_hero (Utilities|Casting|CastToBP_PlayerHero OtherActor))
  (Variables|Default|SetShouldMove true)
  (Pawn|Components|CharacterMovement|SetMovementMode (Variables|/Script/Engine.Character|GetCharacterMovement _asbp_player_hero) "MOVE_None" 0))

(event EventTick
  (params (DeltaSeconds :type Float%20%28single-precision%29))
  (bind _stone1 (Variables|Default|GetStone1))
  (bind _returnvalue (Transformation|GetActorLocation _stone1))
  (bind (_x _y _z) (Math|Vector|BreakVector _returnvalue))
  (if (Variables|Default|GetShouldMove)
    (Transformation|SetActorLocation _stone1 (Math|Vector|MakeVector _x _y (Math|Interpolation|FInterpTo _z (.Z (Math|Vector|BreakVector (Variables|Default|GetStoneTargetLocation))) DeltaSeconds 0.8)) false false)
    (CameraShakes|StartCameraShake (Variables|/Script/Engine.PlayerController|GetPlayerCameraManager (Game|GetPlayerController 0)) "/Game/Blueprints/Camera/BP_CameraShake.BP_CameraShake_C" 1.0 "World" "0, 0, 0")
    (Utilities|FlowControl|Delay 5.0)
    (Pawn|Components|CharacterMovement|SetMovementMode (Variables|/Script/Engine.Character|GetCharacterMovement (stale Collision|EventActorBeginOverlap _asbp_player_hero)) "MOVE_Walking" 0)
    (Actor|DestroyActor)))

(fn ConstructionScript)