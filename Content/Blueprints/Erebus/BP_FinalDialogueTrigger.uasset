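; Trigger volume that stages the final Erebus dialogue and hands off to the closing cutscene level.
; On player overlap it stops movement, destroys the spotlight, repositions Teddy and Vincent, rotates the player, hides Erebus and shows the dialogue widget.
; Tick watches for the last entry, then once runs a black-screen fade, CallPlay and a delayed level load.
; The Erebus-death handler is empty and the white fade is unused.
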(event Custom|OnErebusDied_Event)

(event EventBeginPlay
  ;[1 1 1] BeginPlay
  (bind _asbp_dreambound_game_mode (Utilities|Casting|CastToBP_DreamboundGameMode (Game|GetGameMode)))
  (Variables|Default|SetGameModeRef _asbp_dreambound_game_mode)
  (Variables|/Script/Engine.PrimitiveComponent|SetbGenerateOverlapEvents (Variables|Default|GetCollisionComponent) true)
  (EventDispatchers|BindEventtoOnErebusDied (Subsystems|GetArenaManager) (delegate Custom|OnErebusDied_Event))
  (|GetPlayer))

(event Collision|EventActorBeginOverlap
  (params (OtherActor :type Actor%20Object%20Reference))
  (bind _asbp_player_hero (Utilities|Casting|CastToBP_PlayerHero OtherActor))
  (Pawn|Components|CharacterMovement|SetMovementMode (Variables|/Script/Engine.Character|GetCharacterMovement _asbp_player_hero) "MOVE_None" 0)
  (Actor|DestroyActor (Variables|Default|GetSpotLight))
  (|PositionPawns)
  (Rendering|SetActorHiddenInGame (Variables|Default|GetErebus) true)
  (Variables|Default|SetbShouldBeBright true)
  (Utilities|FlowControl|Delay 3.0)
  (Variables|/Script/Engine.PrimitiveComponent|SetbGenerateOverlapEvents (Variables|Default|GetCollisionComponent) true)
  (bind (_returnvalue _asdialogue_data_asset) (|DisplayDialogue (stale _returnvalue))))

(event EventTick
  (params (DeltaSeconds :type Float%20%28single-precision%29))
  ;[0.4562 1 0.5145] Enable Input after dialogue
  (Utilities|IsValid (stale Collision|EventActorBeginOverlap _returnvalue)
    (:Is%20Valid
      (if (>= (Variables|/Game/Blueprints/Arena/Widgets/WBP_DialogueOpenWorld.WBP_DialogueOpenWorld_C|GetCurrentEntry (stale Collision|EventActorBeginOverlap _returnvalue)) (- (Utilities|Array|Length (Variables|/Script/PROJ.DialogueDataAsset|GetDialogueEntries (stale Collision|EventActorBeginOverlap _asdialogue_data_asset))) 1))
        (bind _output_get (Variables|Default|SetAt%20Last%20Entry (>= (Variables|/Game/Blueprints/Arena/Widgets/WBP_DialogueOpenWorld.WBP_DialogueOpenWorld_C|GetCurrentEntry (stale Collision|EventActorBeginOverlap _returnvalue)) (- (Utilities|Array|Length (Variables|/Script/PROJ.DialogueDataAsset|GetDialogueEntries (stale Collision|EventActorBeginOverlap _asdialogue_data_asset))) 1)))))
      (if _output_get
        (if (Widget|IsVisible (stale Collision|EventActorBeginOverlap _returnvalue))
          (Utilities|FlowControl|DoOnce false
            (:Completed
              (Utilities|FlowControl|Delay 1.0)
              (bind _returnvalue (UserInterface|CreateWidget "/Game/Blueprints/Arena/Widgets/BP_Blackscreen.BP_Blackscreen_C"))
              (UserInterface|Viewport|AddtoViewport _returnvalue 0)
              (UserInterface|Animation|PlayAnimation _returnvalue (Variables|/Game/Blueprints/Arena/Widgets/BP_Blackscreen.BP_Blackscreen_C|GetFadeIn _returnvalue) 0.5 1 "Forward" 1.0 false)
              (Utilities|FlowControl|Delay 2.5)
              (Widget|RemovefromParent _returnvalue)
              (Default|CallPlay)
              (Utilities|FlowControl|Delay 6.5)
              (|FadeToFinalCutscene))))))))

(fn ConstructionScript)