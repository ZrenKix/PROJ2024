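; Trigger actor that runs the Erebus intro cutscene when the player overlaps it, freezing the hero, positioning Teddy and Vincent, and starting dialogue.
; Tick watches the dialogue widget's entry index to send Teddy toward a target on camera and trigger a camera shake.
; The shake is a timer jittering CameraActor2 with decaying intensity, then blending to a zoom-out view.
; A final entry restores camera and movement, resumes Vincent following, saves, and disables collision.
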(event Custom|CameraShake
  ;[1 1 1] Tick
  (|CameraShakeLogic (Game|GetPlayerController 0) (stale EventTick _returnvalue_2)))

(event EventBeginPlay
  (bind _teddy (Variables|Default|GetTeddy))
  ;[1 1 1] Beginplay
  (Variables|Default|SetNewCameraPos (Pawn|GetViewTarget (Game|GetPlayerController 0)))
  (Rendering|SetActorHiddenInGame (Variables|Default|GetPlane) true)
  (bind _returnvalue (UserInterface|CreateWidget "/Game/Blueprints/Arena/Widgets/WBP_DialogueOpenWorld.WBP_DialogueOpenWorld_C"))
  (UserInterface|Viewport|AddtoViewport _returnvalue 0)
  (Widget|SetVisibility _returnvalue "Hidden")
  (Variables|Default|SetOrginalLocationCamera2 (Transformation|GetActorLocation (Variables|Default|GetCameraActor2)))
  (Utilities|IsValid _teddy
    (:Is%20Valid
      (Variables|/Game/Blueprints/Characters/BP_CompanionTeddy.BP_CompanionTeddy_C|SetisInteractable _teddy false))))

(event Collision|EventActorBeginOverlap
  (params (OtherActor :type Actor%20Object%20Reference))
  (bind _teddy (|DisplayDialogue (stale EventBeginPlay _returnvalue) OtherActor)))

(event EventTick
  (params (DeltaSeconds :type Float%20%28single-precision%29))
  (bind _returnvalue (Game|GetPlayerController 0))
  ;[1 1 1] Tick
  (Utilities|FlowControl|Sequence
    (:then_0
      (bind _output_get (Variables|Default|SetTeddyIsHome (|IsTeddyHome (stale _teddygoto))))
      (if _output_get
        (Pawn|Components|CharacterMovement|SetMovementMode (Variables|/Script/Engine.Character|GetCharacterMovement (stale Collision|EventActorBeginOverlap _teddy)) "MOVE_None" 0)))
    (:then_1
      (if (not (== (Variables|/Game/Blueprints/Arena/Widgets/WBP_DialogueOpenWorld.WBP_DialogueOpenWorld_C|GetCurrentEntry (stale EventBeginPlay _returnvalue)) (Variables|Default|GetOld%20Current%20Entry)))
        (Variables|Default|SetOld%20Current%20Entry (Variables|/Game/Blueprints/Arena/Widgets/WBP_DialogueOpenWorld.WBP_DialogueOpenWorld_C|GetCurrentEntry (stale EventBeginPlay _returnvalue)))
        (switch int (Variables|/Game/Blueprints/Arena/Widgets/WBP_DialogueOpenWorld.WBP_DialogueOpenWorld_C|GetCurrentEntry (stale EventBeginPlay _returnvalue))
          (:2
            (bind _teddygoto (|TeddyGoToHoney (Game|GetPlayerController 0) (Variables|Default|GetTeddy))))
          (:20
            (Input|DisableInput _returnvalue 0)
            (bind _returnvalue_2 (Utilities|Time|SetTimerbyEvent (delegate Custom|CameraShake) 0.05 (Variables|Default|GetLooping))))
          (:22
            (|ResetCameraAndMovement _returnvalue (Variables|Default|GetNewCameraPos))))))))

(fn ConstructionScript)