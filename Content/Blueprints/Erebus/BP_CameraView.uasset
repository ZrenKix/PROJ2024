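; One-shot trigger for a scripted Erebus dialogue cutscene with Teddy and camera moves.
; Player overlap halts movement and companion following, then opens the open-world dialogue widget.
; Tick watches the dialogue entry index to send Teddy to a target under a new camera, start timer-driven random camera-location shake, and finally restore the original view.
; The shake blends to a zoom-out camera; the reset re-enables walking and Vincent's following, then destroys the actor.
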(event Custom|CameraShake
  (|CameraShakeLogic (Game|GetPlayerController 0) (stale EventTick _returnvalue)))

(event EventBeginPlay
  (bind _teddy (Variables|Default|GetTeddy))
  (Variables|Default|SetNewVar_0 (Pawn|GetViewTarget (Game|GetPlayerController 0)))
  (Rendering|SetActorHiddenInGame (Variables|Default|GetPlane) true)
  (bind _returnvalue (UserInterface|CreateWidget "/Game/Blueprints/Arena/Widgets/WBP_DialogueOpenWorld.WBP_DialogueOpenWorld_C"))
  (UserInterface|Viewport|AddtoViewport _returnvalue 0)
  (Widget|SetVisibility _returnvalue "Hidden")
  (Variables|Default|SetOrginalLocationCamera2 (Transformation|GetActorLocation (Variables|Default|GetCameraActor2)))
  (Utilities|IsValid _teddy
    (:Is%20Valid
      (Variables|/Game/Blueprints/Characters/BP_CompanionTeddy.BP_CompanionTeddy_C|SetisInteractable _teddy false))))

(event Collision|EventActorBeginOverlap
  (params (OtherActor :type Actor%20Object%20Reference))
  (bind _asbp_player_hero (Utilities|Casting|CastToBP_PlayerHero OtherActor))
  (Pawn|Components|CharacterMovement|SetMovementMode (Variables|/Script/Engine.Character|GetCharacterMovement _asbp_player_hero) "MOVE_None" 0)
  (Variables|/Script/PROJ.CompanionCharacter|SetbCanFollow (Variables|Default|GetTeddy) false)
  (Variables|/Script/PROJ.CompanionCharacter|SetbCanFollow (Variables|Default|GetVincent) false)
  (bind _returnvalue (Game|ConstructObjectfromClass "/Game/Blueprints/Arena/BP_ErabusDialogue.BP_ErabusDialogue_C"))
  (Utilities|FlowControl|Delay 1.0)
  (Default|DisplayEntry (stale EventBeginPlay _returnvalue) 0 "/Game/Assets/UI/Card/T_UI_Card_Character_Bear.T_UI_Card_Character_Bear" _returnvalue))

(event EventTick
  (params (DeltaSeconds :type Float%20%28single-precision%29))
  (Utilities|FlowControl|Sequence
    (:then_0
      (bind _output_get (Variables|Default|SetTeddyIsHome (|IsTeddyHome (stale _teddygoto))))
      (if _output_get
        (Pawn|Components|CharacterMovement|SetMovementMode (Variables|/Script/Engine.Character|GetCharacterMovement (Variables|Default|GetTeddy)) "MOVE_None" 0)))
    (:then_1
      (if (not (== (Variables|/Game/Blueprints/Arena/Widgets/WBP_DialogueOpenWorld.WBP_DialogueOpenWorld_C|GetCurrentEntry (stale EventBeginPlay _returnvalue)) (Variables|Default|GetOld%20Current%20Entry)))
        (Variables|Default|SetOld%20Current%20Entry (Variables|/Game/Blueprints/Arena/Widgets/WBP_DialogueOpenWorld.WBP_DialogueOpenWorld_C|GetCurrentEntry (stale EventBeginPlay _returnvalue)))
        (switch int (Variables|/Game/Blueprints/Arena/Widgets/WBP_DialogueOpenWorld.WBP_DialogueOpenWorld_C|GetCurrentEntry (stale EventBeginPlay _returnvalue))
          (:2
            (bind _teddygoto (|TeddyGoToHoney (Game|GetPlayerController 0) (Variables|Default|GetTeddy))))
          (:20
            (bind _returnvalue (Utilities|Time|SetTimerbyEvent (delegate Custom|CameraShake) 0.05 (Variables|Default|GetLooping))))
          (:22
            (|ResetCameraAndMovement (Game|GetPlayerController 0) (Variables|Default|GetNewVar_0))))))))

(fn ConstructionScript)