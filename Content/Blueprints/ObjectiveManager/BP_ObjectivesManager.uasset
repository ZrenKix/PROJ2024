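; Objective manager that tracks and saves the player's current objective through the Tutorial bedtime routine and The Hub's painting-piece and Vincent quest.
; Named step functions mark objectives complete and set the next text after a delay, with timers unlocking interactables or saving at key Hub steps.
; Bedtime steps also drive lights, decal fades, movement locks and the sleep fade.
; Level name picks the first objective, and combat's end re-shows the objective widget.
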(event Custom|OnCombatFinished_Event
  ;[1 1 1] Begin Play
  (bind _objectivewidget (Variables|Default|GetObjectiveWidget)
    (:then
      (Widget|SetVisibility _objectivewidget "Visible"))
    (:else)))

(event Custom|UpdateObjectiveText
  (params (NewObjective :type Text))
  ;[1 1 1] Update objective text
  (Utilities|FlowControl|Delay (Variables|Default|GetUpdateObjectiveDelay))
  (Variables|Default|SetCurrentObjective NewObjective)
  (Variables|Default|SetObjectiveComplete false))

(event EventBeginPlay
  ;[1 1 1] Begin Play
  (Class|BPIPersistence|RequestLoad(Message) (Game|GetGameInstance) self)
  (CallFunction|GetReferences)
  (EventDispatchers|AssignOnCombatFinished (Subsystems|GetArenaManager) (delegate Custom|OnCombatFinished_Event)))

(event Collision|EventActorBeginOverlap
  (params (OtherActor :type Actor%20Object%20Reference)))

(event EventLoadData
  (params (SaveGameRef :type BP%20Save%20Game%20Object%20Reference))
  ;[1 1 1] Load data
  (Variables|Default|SetPaintingPieceNr (Variables|/Game/Assets/Save/BP_SaveGame.BP_SaveGame_C|GetPaintingPieceNr SaveGameRef))
  (bind _output_get (Variables|Default|SetCurrentObjective (Variables|/Game/Assets/Save/BP_SaveGame.BP_SaveGame_C|GetCurrentObjective SaveGameRef)))
  (if (Variables|/Game/Assets/Save/BP_SaveGame.BP_SaveGame_C|GetFirstTimeLoadingLevel? SaveGameRef)
    (CallFunction|InitObjectives)
    (else
      (CallFunction|CreateWidget)
      (CallFunction|UpdateObjectiveText _output_get))))

(event EventSaveData
  (params (SaveGameRef :type BP%20Save%20Game%20Object%20Reference))
  ;[1 1 1] Save data
  (Variables|/Game/Assets/Save/BP_SaveGame.BP_SaveGame_C|SetCurrentObjective SaveGameRef (Variables|Default|GetCurrentObjective))
  (Variables|/Game/Assets/Save/BP_SaveGame.BP_SaveGame_C|SetObjectiveComplete SaveGameRef (Variables|Default|GetObjectiveComplete))
  (Variables|/Game/Assets/Save/BP_SaveGame.BP_SaveGame_C|SetPaintingPieceNr SaveGameRef (Variables|Default|GetPaintingPieceNr)))

(fn ConstructionScript)

(fn WardrobeDone
  (Variables|Default|SetObjectiveComplete true)
  (CallFunction|UpdateObjectiveText "Say goodnight to Teddy")
  (Utilities|Time|SetTimerbyFunctionName 0 "EnableTeddy" (Variables|Default|GetUpdateObjectiveDelay)))

(fn TeddyDone
  (Variables|Default|SetObjectiveComplete true)
  (CallFunction|UpdateObjectiveText "Turn off the lights")
  (Utilities|Time|SetTimerbyFunctionName 0 "EnableLights" (Variables|Default|GetUpdateObjectiveDelay)))

(fn LightOff
  (for _array_element (Variables|Tutorial|GetLights)
    (if (not (<= (Variables|/Script/Engine.LightComponentBase|GetIntensity (Variables|/Game/Blueprints/Interaction/BP_Lamp.BP_Lamp_C|GetPointLight _array_element)) 0.0))
      (LocalVariables|SetLightIsOff false)))
  (if (LocalVariables|GetLightIsOff)
    (Development|PrintString "all lights off")
    (Tutorial|AllLightsDone)
    (else
      (Development|PrintString "all lights not off"))))

(fn FirstTimeBed
  (Variables|Default|SetObjectiveComplete true)
  (Variables|Tutorial|SetCanGoToBed false)
  (Default|FadeinDecal (Variables|Default|GetDecalRef))
  (CallFunction|DisablePlayerMovement)
  (bind _returnvalue (UserInterface|CreateWidget "/Game/Blueprints/UI/Interaction/WBP_TextPopup.WBP_TextPopup_C" 0 "It's to scary! I will turn on my lamp" "Edith" "/Game/Assets/UI/NewUI/T_UI_Card_Character_Edith.T_UI_Card_Character_Edith"))
  (UserInterface|Viewport|AddtoViewport _returnvalue 0)
  (Utilities|Time|SetTimerbyFunctionName 0 "EnablePlayerMovement" 2.0)
  (Utilities|Time|SetTimerbyFunctionName 0 "TurnOnBedLight" 2.0))

(fn DisablePlayerMovement
  (Pawn|Components|CharacterMovement|DisableMovement (Variables|/Script/Engine.Character|GetCharacterMovement (Game|GetPlayerCharacter 0))))

(fn EnablePlayerMovement
  (Pawn|Components|CharacterMovement|SetMovementMode (Variables|/Script/Engine.Character|GetCharacterMovement (Game|GetPlayerCharacter 0)) "MOVE_Walking" 0)
  (Development|PrintString "You can walk again" true true "(R=1.000000,G=0.000000,B=0.771030,A=1.000000)"))

(fn TurnonBedLight
  (CallFunction|UpdateObjectiveText "Turn on the bed light")
  (for _array_element (Variables|Tutorial|GetLights)
    (if (Actor|ActorHasTag _array_element "BedLight")
      (Variables|/Game/Blueprints/Interaction/BP_Lamp.BP_Lamp_C|SetisInteractable? _array_element true))))

(fn AllLightsDone
  (Variables|Default|SetObjectiveComplete true)
  (Variables|Tutorial|SetCanGoToBed true)
  (CallFunction|UpdateObjectiveText "Go to sleep."))

(fn EnableLights
  (for _array_element (Variables|Tutorial|GetLights)
    (Variables|/Game/Blueprints/Interaction/BP_Lamp.BP_Lamp_C|SetisInteractable? _array_element true)))

(fn BedLightDone
  (Variables|Default|SetObjectiveComplete true)
  (Variables|Tutorial|SetCanGoToBed true)
  (CallFunction|UpdateObjectiveText "Go to sleep.")
  (Default|FadeOutDecal (Variables|Default|GetDecalRef)))

(fn StartSleepCutscene
  (CallFunction|DisablePlayerMovement)
  (Viewport|RemoveAllWidgets)
  (bind _asbp_tutorial_game_mode (Utilities|Casting|CastToBP_TutorialGameMode (Game|GetGameMode)))
  (Default|FadetoBlack _asbp_tutorial_game_mode))

(fn InitObjectives
  (bind _returnvalue (Game|GetCurrentLevelName true))
  (switch string _returnvalue
    (:Tutorial
      (Variables|Default|SetCurrentObjective "Close the wardrobe"))
    (:TheHub
      (bind _returnvalue_2 (UserInterface|CreateWidget "/Game/Blueprints/UI/Tutorial/WBP_Objective.WBP_Objective_C"))
      (bind _output_get (Variables|Default|SetObjectiveWidget _returnvalue_2))
      (UserInterface|Viewport|AddtoViewport _output_get 0)
      (Variables|Default|SetCurrentObjective "Explore your surroundings")
      (Default|ToggleCheckMark (Variables|Default|GetObjectiveWidget) false))))

(fn GetReferences
  (bind _asbp_player_hero (Utilities|Casting|CastToBP_PlayerHero (Game|GetPlayerCharacter 0)))
  (Variables|Default|SetPlayerRef _asbp_player_hero)
  (bind _asbp_dreambound_game_mode (Utilities|Casting|CastToBP_DreamboundGameMode (Game|GetGameMode)))
  (Variables|Default|SetGameModeRef _asbp_dreambound_game_mode))

(fn ExplorationDone
  (Variables|Default|SetObjectiveComplete true)
  (CallFunction|UpdateObjectiveText "Find the remaining pieces"))

(fn CreateWidget
  (bind _returnvalue (UserInterface|CreateWidget "/Game/Blueprints/UI/Tutorial/WBP_Objective.WBP_Objective_C"))
  (bind _output_get (Variables|Default|SetObjectiveWidget _returnvalue))
  (UserInterface|Viewport|AddtoViewport _output_get 0))

(fn EnableTeddy
  (Variables|/Game/Blueprints/Interaction/BP_TeddyInteract.BP_TeddyInteract_C|SetisInteractable (Variables|Tutorial|GetTeddy) true))

(fn UpdatePaintingPiece
  (bind _result (Math|Integer|IncrementInt (Variables|Default|GetPaintingPieceNr))
    (:%20%20
      (bind _output_get (Variables|Default|SetPaintingPieceNr _result))
      (if (>= _output_get 3)
        (Variables|Default|SetCurrentObjective (Utilities|Text|ToText(String) (Utilities|String|Append "Find painting pieces " (Utilities|String|ToString(Integer) _output_get) "/3")))
        (Utilities|Time|SetTimerbyFunctionName 0 "SetVincentObjective" 0.001)
        (else
          (Variables|Default|SetCurrentObjective (Utilities|Text|ToText(String) (Utilities|String|Append "Find painting pieces " (Utilities|String|ToString(Integer) _output_get) "/3"))))))))

(fn SetVincentObjective
  (Variables|Default|SetObjectiveComplete true)
  (CallFunction|UpdateObjectiveText "Find Vincent")
  (Utilities|Time|SetTimerbyFunctionName 0 "SaveGame" (+ (Variables|Default|GetUpdateObjectiveDelay) 0.05)))

(fn AfterVincentFight
  (Variables|Default|SetObjectiveComplete true)
  (CallFunction|UpdateObjectiveText "Find the portal")
  (CallFunction|CallSaveGame))

(fn CallSaveGame
  (Utilities|Time|SetTimerbyFunctionName 0 "SaveGame" (+ (Variables|Default|GetUpdateObjectiveDelay) 0.05)))

(fn SaveGame
  (Default|SaveGame (Variables|Default|GetGameModeRef) true))