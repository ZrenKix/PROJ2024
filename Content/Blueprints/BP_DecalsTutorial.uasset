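; Tutorial decal actor that groups three decal components, starts hidden, and can be faded in and out through events.
; FadeInDecal unhides the actor and fades all three decals in after a short delay.
; FadeOutDecal fades them out the same way and destroys the actor when the fade finishes.
; IsItDark is an empty stub, and nothing in this Blueprint triggers either fade.
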(event Custom|FadeInDecal
  (bind _output_get (Variables|Default|SetIsHidden false))
  (Rendering|SetActorHiddenInGame _output_get)
  (Rendering|Components|Decal|SetFadeIn (Variables|Default|GetDecal2) 1.0 1.0))

(event Custom|IsItDark)

(event Custom|FadeOutDecal
  (Rendering|Components|Decal|SetFadeOut (Variables|Default|GetDecal1) 1.0 1.0 true))

(event EventBeginPlay
  (bind _output_get (Variables|Default|SetIsHidden true))
  (Rendering|SetActorHiddenInGame _output_get))

(event Collision|EventActorBeginOverlap
  (params (OtherActor :type Actor%20Object%20Reference)))

(event EventTick
  (params (DeltaSeconds :type Float%20%28single-precision%29)))

(fn ConstructionScript)