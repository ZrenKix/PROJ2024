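; Floor button that responds only to the Vincent companion (BP_CompanionVincent) entering or leaving its trigger box.
; On entry it calls the IsPressed dispatcher, swaps to the pressed material and sets VincentIsHome, which this graph never clears.
; On exit it calls IsNotPressed and restores the original material.
; Looping function timers lower or raise the actor by Offset, stopping on exact position matches.
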(event OnComponentBeginOverlap(Box)
  (params (OverlappedComponent :type Primitive%20Component%20Object%20Reference) (OtherActor :type Actor%20Object%20Reference) (OtherComp :type Primitive%20Component%20Object%20Reference) (OtherBodyIndex :type Integer) (bFromSweep :type Boolean) (SweepResult :type Hit%20Result%20Structure%20%28by%20ref%29))
  (Utilities|Casting|CastToBP_CompanionVincent OtherActor)
  (Default|CallIsPressed)
  (Rendering|Material|SetMaterial (Variables|Default|GetCube) 0 (Variables|Default|GetPressedMat))
  (Utilities|Time|SetTimerbyFunctionName 0 "UpdateLocation" 0.001 true)
  (Variables|Default|SetbVincentIsHome true))

(event OnComponentEndOverlap(Box)
  (params (OverlappedComponent :type Primitive%20Component%20Object%20Reference) (OtherActor :type Actor%20Object%20Reference) (OtherComp :type Primitive%20Component%20Object%20Reference) (OtherBodyIndex :type Integer))
  (Utilities|Casting|CastToBP_CompanionVincent OtherActor)
  (Default|CallIsNotPressed)
  (Rendering|Material|SetMaterial (Variables|Default|GetCube) 0 (Variables|Default|GetDefaultMat))
  (Utilities|Time|SetTimerbyFunctionName 0 "ResetLocation" 0.001 true))

(event EventBeginPlay
  (Variables|Default|SetDefaultPosition (Transformation|GetActorLocation))
  (Variables|Default|SetDefaultMat (Rendering|Material|GetMaterial (Variables|Default|GetCube) 0)))

(fn ConstructionScript)

(fn ResetLocation
  (bind _returnvalue (Transformation|GetActorLocation))
  (if (Utilities|Operators|EqualEqual (Transformation|GetActorLocation) (Variables|Default|GetDefaultPosition) 0.0)
    (Utilities|Time|ClearTimerbyFunctionName 0 "ResetLocation")
    (else
      (Transformation|SetActorLocation (Math|Vector|MakeVector (.x _returnvalue) (.y _returnvalue) (+ (.z _returnvalue) (Variables|Default|GetOffset))) false false))))

(fn UpdateLocation
  (bind _returnvalue (Transformation|GetActorLocation))
  (bind _defaultposition (Variables|Default|GetDefaultPosition))
  (if (Utilities|Operators|EqualEqual (Transformation|GetActorLocation) (Math|Vector|MakeVector (.x _defaultposition) (.y _defaultposition) (- (.z _defaultposition) (Variables|Default|GetOffset))) 0.0)
    (Utilities|Time|ClearTimerbyFunctionName 0 "UpdateLocation")
    (else
      (Transformation|SetActorLocation (Math|Vector|MakeVector (.x _returnvalue) (.y _returnvalue) (- (.z _returnvalue) (Variables|Default|GetOffset))) false false))))