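; BP_PortalOtherLevel is a portal that saves the game and sends the player to another level.
; A capsule overlap with a player-interface actor activates it, binds LoadNextLevel to the game instance's saved event and requests a save.
; SaveData writes the destination and first-time-load flag when activated, and LoadNextLevel opens that level after a short delay.
; The construction script's scene-capture cubemap setup for the Niagara particle is disconnected and never runs.
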(event OnComponentBeginOverlap(Capsule)
  (params (OverlappedComponent :type Primitive%20Component%20Object%20Reference) (OtherActor :type Actor%20Object%20Reference) (OtherComp :type Primitive%20Component%20Object%20Reference) (OtherBodyIndex :type Integer) (bFromSweep :type Boolean) (SweepResult :type Hit%20Result%20Structure%20%28by%20ref%29))
  (if (Utilities|DoesObjectImplementInterface OtherActor "/Game/Blueprints/Interface/BPI_PlayerInterface.BPI_PlayerInterface_C")
    (Variables|Default|SetIsActivated true)
    (bind _asbp_game_instance (Utilities|Casting|CastToBP_GameInstance (Game|GetGameInstance)))
    (EventDispatchers|BindEventtoGameSaved _asbp_game_instance (delegate Custom|LoadNextLevel))
    (Class|BPIPersistence|RequestSave(Message) _asbp_game_instance false)))

(event Custom|LoadNextLevel
  (params (SaveGameRef :type BP%20Save%20Game%20Object%20Reference))
  (Utilities|FlowControl|Delay 2.0)
  (Game|OpenLevel(byObjectReference) (Variables|Default|GetLevelToGoTo)))

(event EventBeginPlay
  (bind _asbp_game_instance (Utilities|Casting|CastToBP_GameInstance (Game|GetGameInstance)))
  (Default|RequestLoad _asbp_game_instance self))

(event EventLoadData
  (params (SaveGameRef :type BP%20Save%20Game%20Object%20Reference)))

(event EventSaveData
  (params (SaveGameRef :type BP%20Save%20Game%20Object%20Reference))
  (if (Variables|Default|GetIsActivated)
    (Variables|/Game/Assets/Save/BP_SaveGame.BP_SaveGame_C|SetCurrentLevel SaveGameRef (Variables|Default|GetLevelToGoTo))
    (Variables|/Game/Assets/Save/BP_SaveGame.BP_SaveGame_C|SetFirstTimeLoadingLevel? SaveGameRef true)
    (Development|PrintString (Utilities|String|Append "portal first time: " (Utilities|String|ToString(Boolean) (Variables|/Game/Assets/Save/BP_SaveGame.BP_SaveGame_C|GetFirstTimeLoadingLevel? SaveGameRef))) true true "(R=0.000000,G=1.000000,B=0.017425,A=1.000000)")))

(fn ConstructionScript)