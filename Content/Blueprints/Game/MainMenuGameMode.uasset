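; Game mode for the main menu that sets up the menu UI and a hidden debug option.
; On BeginPlay it creates WBP_MainMenu, adds it to the viewport, focuses it with Game and UI input, and shows a cursor locked to the viewport.
; Tick polls the Section (§) key and, once only, reveals the widget's debug buttons for test map, hub and save creation or deletion.
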(event EventBeginPlay
  (bind _returnvalue (Game|GetPlayerController 0))
  ;[1 1 1] Setup widget and mouse cursor
  (bind _returnvalue_2 (UserInterface|CreateWidget "/Game/Blueprints/UI/Menus/WBP_MainMenu.WBP_MainMenu_C"))
  (bind _output_get (Variables|Default|SetMainMenuWidget _returnvalue_2))
  (UserInterface|Viewport|AddtoViewport _output_get 0)
  (Input|SetInputModeGameandUI _returnvalue _output_get "LockAlways" false false)
  (Variables|/Script/Engine.PlayerController|SetbShowMouseCursor _returnvalue true))

(event EventTick
  (params (DeltaSeconds :type Float%20%28single-precision%29))
  ;[1 1 1] Show debug button (§)
  (if (Game|Player|IsInputKeyDown (Game|GetPlayerController 0) "Section")
    (Utilities|FlowControl|DoOnce false
      (:Completed
        (Widget|SetVisibility (Variables|/Game/Blueprints/UI/Menus/WBP_MainMenu.WBP_MainMenu_C|GetTestMap (Variables|Default|GetMainMenuWidget)) "Visible")))))

(fn ConstructionScript)