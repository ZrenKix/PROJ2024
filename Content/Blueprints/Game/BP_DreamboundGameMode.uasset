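; Game mode that runs transitions between exploration and turn-based arena combat.
; CreateArena fades to black, has the ArenaManager build the fight, then starts turn order, boss-dependent music, combat widgets and optional dialogue.
; Possession changes and action ends re-apply the tagged arena camera during combat.
; When combat finishes or creation fails, it repossesses the old pawn, saves and closes the arena; the hero buff loop applies nothing.
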(event Custom|OnPossessedPawnChanged_Event
  (params (OldPawn :type Pawn%20Object%20Reference) (NewPawn :type Pawn%20Object%20Reference))
  (bind _returnvalue (Game|GetPlayerController 0))
  (Utilities|FlowControl|Sequence
    (:then_0
      (Utilities|FlowControl|DelayUntilNextTick)
      (bind _returnvalue_2 (Actor|GetActorOfClass "/Script/Engine.PlayerStart"))
      (Pawn|SetControlRotation _returnvalue (Transformation|GetActorRotation _returnvalue_2)))
    (:then_1
      (if (Variables|Default|GetIsInCombat)
        (Game|Player|SetViewTargetwithBlend _returnvalue (Variables|Default|GetArena%20Camera) 0.0 "VTBlend_Linear" 0.0 false)))))

(event Custom|Create%20Arena
  (params (Enemies :type Array%20of%20Unit%20Base%20Class%20References) (Heroes :type Array%20of%20Unit%20Base%20Class%20References) (BossfightTyoe :type EBossfightType%20Enum :default "None") (NumOfHeroes :type Integer) (Dialogue%20Data :type Dialogue%20Data%20Asset%20Class%20Reference))
  (bind _returnvalue (Game|GetPlayerController 0))
  (bind _returnvalue_2 (Subsystems|GetArenaManager))
  (bind _index (Variables|Default|GetIndex))
  (bind _currentuuid (Variables|Default|GetCurrentUUID))
  (bind _returnvalue_3 (== _index _currentuuid))
  (Variables|Default|SetHeroes Heroes)
  (bind _returnvalue_4 (|Check))
  (Variables|Default|SetIsInCombat true)
  (|FadeWidget _returnvalue_4)
  (Input|DisableInput _returnvalue 0)
  (Utilities|FlowControl|Delay 1.5)
  (bind _returnvalue_5 (Class|ArenaManager|CreateArena _returnvalue_2 Enemies Heroes "ArenaScene" BossfightTyoe NumOfHeroes))
  (Utilities|FlowControl|Delay 1.6)
  (Audio|Components|Audio|FadeIn)
  (Input|EnableInput _returnvalue 0)
  (if _returnvalue_5
    (Utilities|FlowControl|Sequence
      (:then_0
        (EventDispatchers|AssignOnCombatFinished _returnvalue_2 (delegate Custom|OnCombatFinished_Event))
        (EventDispatchers|AssignOnActionEndEvent _returnvalue_2 (delegate Custom|OnActionEndEvent_Event))
        (|SetArenaCamera
          (:Completed
            (Class|ArenaManager|NextinTurnOrder _returnvalue_2)
            (if (Utilities|IsValidClass Dialogue%20Data)
              ;[0.4104 0.4301 1] Create Dialogue
              (bind _returnvalue_6 (UserInterface|CreateWidget "/Game/Blueprints/Arena/Widgets/WBP_DialogueWindow.WBP_DialogueWindow_C"))
              (Widget|SetVisibility _returnvalue_6 "Hidden")
              (Class|ArenaDialogueLogic|InitializDialogue (Variables|/Script/PROJ.ArenaManager|GetDialogueLogic (Subsystems|GetArenaManager)) Dialogue%20Data _returnvalue_6))
            (bind _returnvalue_7 (UserInterface|CreateWidget "/Game/Blueprints/Arena/Widgets/BP_StatsContainer.BP_StatsContainer_C"))
            (bind _returnvalue_8 (UserInterface|CreateWidget "/Game/Blueprints/Arena/Widgets/BP_QueueOrderWidget.BP_QueueOrderWidget_C"))
            (UserInterface|Viewport|AddtoViewport _returnvalue_7 0)
            (CallFunction|ApplyBuffs (Variables|Default|GetHeroes)))))
      (:then_1
        (switch Utilities|FlowControl|Switch|SwitchonEBossfightType BossfightTyoe
          (:None
            (bind _returnvalue_9 (Class|FMODBlueprintStatics|PlayEvent2D "/Game/FMOD/Events/Music/CombatMusic.CombatMusic")))
          (:Erebus
            (Class|FMODBlueprintStatics|PlayEvent2D "/Game/FMOD/Events/Music/CombatMusic.CombatMusic"))
          (:DarkBob
            (Class|FMODBlueprintStatics|PlayEvent2D "/Game/FMOD/Events/Music/DarkBobMusic.DarkBobMusic")))))
    (else
      (Variables|Default|SetIsInCombat false)
      (Class|FMODBlueprintStatics|EventInstanceStop _returnvalue_9 false)
      (Utilities|FlowControl|Delay 0.2)
      (|Possesoldpawn
        (:output
          (CallFunction|SaveGame true)
          (Default|CallCloseArena (Math|Integer|SelectInt _index 0 _returnvalue_3))
          (if _returnvalue_3
            (Math|Integer|IncrementInt _currentuuid)))))))

(event Custom|OnCombatFinished_Event
  (bind _index (Variables|Default|GetIndex))
  (bind _currentuuid (Variables|Default|GetCurrentUUID))
  (bind _returnvalue (== _index _currentuuid))
  (Variables|Default|SetIsInCombat false)
  (Class|FMODBlueprintStatics|EventInstanceStop (stale Custom|Create%20Arena _returnvalue_9) false)
  (Utilities|FlowControl|Delay 0.2)
  (|Possesoldpawn
    (:output
      (CallFunction|SaveGame true)
      (Default|CallCloseArena (Math|Integer|SelectInt _index 0 _returnvalue))
      (if _returnvalue
        (Math|Integer|IncrementInt _currentuuid)))))

(event Custom|OnActionEndEvent_Event
  (Utilities|FlowControl|DelayUntilNextTick)
  (Utilities|FlowControl|DelayUntilNextTick)
  (Class|ArenaDialogueLogic|CheckandDisplayEntries (Variables|/Script/PROJ.ArenaManager|GetDialogueLogic (Subsystems|GetArenaManager)))
  (if (Variables|Default|GetIsInCombat)
    (Game|Player|SetViewTargetwithBlend (Game|GetPlayerController 0) (Variables|Default|GetArena%20Camera) 0.0 "VTBlend_Linear" 0.0 false)))

(event EventBeginPlay
  (EventDispatchers|AssignOnPossessedPawnChanged (Game|GetPlayerController 0) (delegate Custom|OnPossessedPawnChanged_Event)))

(event EventTick
  (params (DeltaSeconds :type Float%20%28single-precision%29)))

(fn ConstructionScript)

(fn SaveComplete
  (params (SaveGameRef :type BP%20Save%20Game%20Object%20Reference))
  (Utilities|IsValid SaveGameRef
    (:Is%20Valid
      (bind _returnvalue (UserInterface|CreateWidget "/Game/Blueprints/Save/WBP_SaveComplete.WBP_SaveComplete_C"))
      (UserInterface|Viewport|AddtoViewport _returnvalue 0))))

(fn SaveGame
  (params (Async :type Boolean))
  (bind _asbp_game_instance (Utilities|Casting|CastToBP_GameInstance (Game|GetGameInstance)))
  (EventDispatchers|BindEventtoGameSaved _asbp_game_instance (EventDispatchers|CreateEvent :!event SaveComplete))
  (Class|BPIPersistence|RequestSave(Message) _asbp_game_instance Async))

(fn ApplyBuffs
  (params (Heroes :type Array%20of%20Unit%20Base%20Class%20References))
  (bind _asbp_player_hero (Utilities|Casting|CastToBP_PlayerHero (Game|GetPlayerCharacter 0)))
  (for _array_element (Class|ArenaManager|GetHeroes (Subsystems|GetArenaManager))
    (for _index (range 0 (Variables|/Game/Blueprints/Characters/Player/BP_PlayerHero.BP_PlayerHero_C|GetBuffAmount _asbp_player_hero))
      _)))

(fn CreateArena
  (params (Heros :type Array%20of%20Unit%20Base%20Class%20References) (Enemies :type Array%20of%20Unit%20Base%20Class%20References) (BossfightType :type EBossfightType%20Enum :default "None") (Num%20Of%20Heroes :type Integer) (Dialogue%20Data :type Dialogue%20Data%20Asset%20Class%20Reference))
  (CallFunction|CreateArena Enemies Heros BossfightType Num%20Of%20Heroes Dialogue%20Data)
  (bind _result (Math|Integer|IncrementInt (Variables|Default|GetIndex))
    (:%20%20
      (return _result))))