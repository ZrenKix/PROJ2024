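; Tutorial game mode that tracks the bedtime objectives and hands the player on to the hub level.
; BeginPlay locks player movement and interaction, and a separate PlayIntroCutscene function shows the diary intro widget.
; Tick polls for all lamps off and wardrobe closed, then going to bed.
; Completion fires once, chaining input lock, fade to black, sequence playback and a GameInstance save through finish callbacks before opening TheHub.
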(event Custom|SaveCompleted
  (params (SaveGameRef :type BP%20Save%20Game%20Object%20Reference))
  ;[1 1 1] Play cutscene when animation is done
  (Game|OpenLevel(byObjectReference) "/Game/Maps/TheHub.TheHub"))

(event Custom|OnFinished_Event
  ;[1 1 1] Play cutscene when animation is done
  (bind _asbp_game_instance (Utilities|Casting|CastToBP_GameInstance (Game|GetGameInstance)))
  (EventDispatchers|BindEventtoGameSaved _asbp_game_instance (delegate Custom|SaveCompleted))
  (Class|BPIPersistence|RequestSave(Message) _asbp_game_instance false))

(event Custom|FadeToBlack
  ;[1 1 1] Fade to black
  (bind _returnvalue (UserInterface|CreateWidget "/Game/Blueprints/UI/Tutorial/WBP_FadeBlack.WBP_FadeBlack_C"))
  (bind _output_get (Variables|Default|SetFadeToBlackWidget _returnvalue))
  (UserInterface|Viewport|AddtoViewport _output_get 0)
  (Class|UserWidget|BindtoAnimationFinished (Variables|Default|GetFadeToBlackWidget) (Variables|/Game/Blueprints/UI/Tutorial/WBP_FadeBlack.WBP_FadeBlack_C|GetFadeToBlack (Variables|Default|GetFadeToBlackWidget)) (delegate Custom|Play%20cutscene%20then%20load%20level))
  (UserInterface|Animation|PlayAnimation (Variables|Default|GetFadeToBlackWidget) (Variables|/Game/Blueprints/UI/Tutorial/WBP_FadeBlack.WBP_FadeBlack_C|GetFadeToBlack (Variables|Default|GetFadeToBlackWidget)) 0.0 1 "Forward" 1.0 false)
  (Class|FMODBlueprintStatics|PlayEvent2D "/Game/FMOD/Events/Jingles/Rest.Rest"))

(event Custom|Play%20cutscene%20then%20load%20level
  ;[1 1 1] Play cutscene when animation is done
  (bind _cutsceneactor (Variables|Default|GetCutsceneActor)
    (:then
      (Sequencer|Player|Play (Variables|/Script/LevelSequence.LevelSequenceActor|GetSequencePlayer _cutsceneactor) :!class /Script/MovieScene.MovieSceneSequencePlayer)
      (EventDispatchers|AssignOnFinished (Variables|/Script/LevelSequence.LevelSequenceActor|GetSequencePlayer _cutsceneactor) (delegate Custom|OnFinished_Event))
      (Utilities|FlowControl|Delay 0.2)
      (Viewport|RemoveAllWidgets) ; Mainly to remove fade to black widget
    )
    (:else)))

(event EventBeginPlay
  ;[1 1 1] Show intro text and disable interaction until text is complete
  (bind _asbp_player_hero (Utilities|Casting|CastToBP_PlayerHero (Game|GetPlayerCharacter 0)))
  (bind _output_get (Variables|Default|SetPlayerRef _asbp_player_hero))
  (Variables|/Game/Blueprints/Characters/Player/BP_PlayerHero.BP_PlayerHero_C|SetInteractEnabled _output_get false)
  (Pawn|Components|CharacterMovement|DisableMovement (Variables|/Script/Engine.Character|GetCharacterMovement _asbp_player_hero)))

(event EventTick
  (params (DeltaSeconds :type Float%20%28single-precision%29))
  ;[1 1 1] Check objective status
  (CallFunction|CheckObjectives)
  (if (Variables|Default|GetFirstObjectivesComplete?) ; 1st objectives complete?
    (if (Variables|Default|GetSecondObjectivesComplete?) ; 2nd objectives complete?
      (Utilities|FlowControl|DoOnce false
        (:Completed
          (Input|DisableInput (Variables|Default|GetPlayerRef) 0)
          (bind _objectivewidget (Variables|Default|GetObjectiveWidget)
            (:then
              (Widget|RemovefromParent _objectivewidget)
              (Utilities|FlowControl|Delay 0.2)
              (CallFunction|FadetoBlack)
              (Variables|/Game/Blueprints/Characters/Player/BP_PlayerHero.BP_PlayerHero_C|SetInteractEnabled (Variables|Default|GetPlayerRef) false))
            (:else)))))))

(fn ConstructionScript)

(fn CheckObjectives
  (bind _output_get (Variables|Default|SetTurnedOffLamps? (>= (Variables|Default|GetTurnedOffLamps) (Utilities|Array|Length (Variables|Default|GetLamps)))))
  (if (and _output_get (Variables|Default|GetClosedWardrobe?))
    (Variables|Default|SetFirstObjectivesComplete? true)
    (if (Variables|Default|GetGoToBed?)
      (Variables|Default|SetSecondObjectivesComplete? true))))

(fn PlayIntroCutscene
  (bind _returnvalue (UserInterface|CreateWidget "/Game/Blueprints/UI/Tutorial/WBP_NewGameIntro.WBP_NewGameIntro_C" 0 "Dear diary, 
 
I’m scared. When it gets dark the shadows look like they’re moving. I want to keep my lights on but mommy says I have to turn them off at night. Yesterday, after I turned off the lights, I saw glowing eyes in my wardrobe. I could feel them staring at me when I tried to sleep. 
 
I tried to tell mommy about the monsters, but she doesn’t believe me. She says it’s all in my imagination, but what if it isn’t? What if they are real and just come out in the dark? 
 
I wish I could be brave, but everything just feels so… wrong. I hope tomorrow I can tell mommy it’s all okay, but I don’t know. Maybe the monsters will be gone by then. Or maybe they will get me. I hope they won’t. 
 
xx Edith 
 
E to continue..."))
  (UserInterface|Viewport|AddtoViewport _returnvalue 0)
  (return))