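; BP_VincentRocks is an actor whose presence in the level persists through the save system.
; On BeginPlay it requests a load from BP_GameInstance, then destroys itself if ShouldSpawn is false.
; Its save and load events write and read that flag in the save game's SpawnableActors map, keyed by a GUID the construction script generates when none is valid.
; Nothing in this graph changes ShouldSpawn apart from loading.
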(event EventBeginPlay
  (bind _asbp_game_instance (Utilities|Casting|CastToBP_GameInstance (Game|GetGameInstance)))
  (Default|RequestLoad _asbp_game_instance self)
  (if (not (Variables|Default|GetShouldSpawn?))
    (Actor|DestroyActor)))

(event EventLoadData
  (params (SaveGameRef :type BP%20Save%20Game%20Object%20Reference))
  (bind _guid (Variables|Default|GetGuid))
  (bind _spawnableactors (Variables|/Game/Assets/Save/BP_SaveGame.BP_SaveGame_C|GetSpawnableActors SaveGameRef))
  (bind (_value _returnvalue) (Utilities|Map|Find _spawnableactors _guid))
  (if _returnvalue
    (Variables|Default|SetShouldSpawn? _value)))

(event EventSaveData
  (params (SaveGameRef :type BP%20Save%20Game%20Object%20Reference))
  (Utilities|Map|Add (Variables|/Game/Assets/Save/BP_SaveGame.BP_SaveGame_C|GetSpawnableActors SaveGameRef) (Variables|Default|GetGuid) (Variables|Default|GetShouldSpawn?)))

(fn ConstructionScript
  (CallFunction|HandleGUID))

(fn HandleGUID
  (if (not (Guid|IsValidGuid (Variables|Default|GetGuid)))
    (Variables|Default|SetGuid (Guid|NewGuid))))