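; BP_LightLantern is an examinable interactable that lights a group of lanterns when used.
; Interact loops over its Lanterns array, casts each to BP_LanternTut to call LightUp, and switches its own PaperSprite to the default lit material.
; It then shows a WBP_TextPopup remarking on the lanterns and reports success.
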(event EventBeginPlay)

(event Collision|EventActorBeginOverlap
  (params (OtherActor :type Actor%20Object%20Reference)))

(event EventTick
  (params (DeltaSeconds :type Float%20%28single-precision%29)))

(fn ConstructionScript)

(fn GetInteractPrompt
  (return "Examine"))

(fn Interact
  (for _array_element (Variables|Default|GetLanterns)
    (bind _asbp_lantern_tut (Utilities|Casting|CastToBP_LanternTut _array_element))
    (Default|LightUp _asbp_lantern_tut)
    (Rendering|Material|SetMaterial (Variables|Default|GetPaperSprite) 0 "/Paper2D/DefaultLitSpriteMaterial.DefaultLitSpriteMaterial"))
  (bind _returnvalue (UserInterface|CreateWidget "/Game/Blueprints/UI/Interaction/WBP_TextPopup.WBP_TextPopup_C" 0 "*Wow, did those lanters just light up?"))
  (UserInterface|Viewport|AddtoViewport _returnvalue 0)
  (return true))