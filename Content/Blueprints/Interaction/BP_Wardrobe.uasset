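; BP_Wardrobe is an interactable wardrobe for the tutorial, which the player can close once.
; It shows its prompt only while interactable; Interact starts the close animation and then disables further interaction.
; A timeline rotates the left door, then on finish plays an attached closing sound event and sets ClosedWardrobe on the tutorial game mode cached at BeginPlay.
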(event Custom|PlayAnimation
  (bind _door_left (Variables|Default|GetDoor_Left))
  ;[1 1 1] Handle Interaction
  (bind _doorrotation (Timeline|CloseDoorTimeline Play)
    (:Update
      (Transformation|SetRelativeRotation _door_left (Math|Rotator|MakeRotator 0.0 0.0 _doorrotation) false false))
    (:Finished
      ;[1 1 1] Play sound
      (Class|FMODBlueprintStatics|PlayEventAttached "/Game/FMOD/Events/TutorialRoom/Close_Closet.Close_Closet" _door_left "None" "0, 0, 0" "KeepRelativeOffset")
      ;[1 1 1] Update wardrobe condition
      (bind _gamemode (Variables|Default|GetGameMode)
        (:then
          (Variables|/Game/Blueprints/Game/BP_TutorialGameMode.BP_TutorialGameMode_C|SetClosedWardrobe? _gamemode true))
        (:else)))))

(event EventBeginPlay
  (bind _asbp_tutorial_game_mode (Utilities|Casting|CastToBP_TutorialGameMode (Game|GetGameMode)))
  (Variables|Default|SetGameMode _asbp_tutorial_game_mode))

(fn ConstructionScript)

(fn GetInteractPrompt
  (if (Variables|Default|GetisInteractable?)
    (return (Variables|Default|GetInteract%20Text))
    (else
      (return ""))))

(fn Interact
  (if (Variables|Default|GetisInteractable?)
    (CallFunction|PlayAnimation)
    (Variables|Default|SetisInteractable? false)
    (return false)))