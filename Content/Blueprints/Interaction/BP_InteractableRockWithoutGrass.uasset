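; BP_InteractableRockWithoutGrass is an interactable rock that shows a text popup with Edith's character portrait when the player interacts with it.
; It enables interaction on BeginPlay and supplies an empty interact prompt.
; Interact creates a WBP_TextPopup, randomly fills it with Prompt01 or Prompt02, adds it to the viewport and returns false.
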(event EventBeginPlay
  (CallFunction|SetInteractable true))

(event Collision|EventActorBeginOverlap
  (params (OtherActor :type Actor%20Object%20Reference)))

(event EventTick
  (params (DeltaSeconds :type Float%20%28single-precision%29)))

(fn ConstructionScript)

(fn GetInteractPrompt
  (return ""))

(fn Interact
  (bind _returnvalue (UserInterface|CreateWidget "/Game/Blueprints/UI/Interaction/WBP_TextPopup.WBP_TextPopup_C" 0 "" "Edith" "/Game/Assets/UI/NewUI/T_UI_Card_Character_Edith.T_UI_Card_Character_Edith"))
  (switch int (Math|Random|RandomInteger 2)
    (:0
      (Variables|/Game/Blueprints/UI/Interaction/WBP_TextPopup.WBP_TextPopup_C|SetFullText _returnvalue (Variables|Default|GetPrompt_01)))
    (:1
      (Variables|/Game/Blueprints/UI/Interaction/WBP_TextPopup.WBP_TextPopup_C|SetFullText _returnvalue (Variables|Default|GetPrompt_02))))
  (UserInterface|Viewport|AddtoViewport _returnvalue 0)
  (return false))