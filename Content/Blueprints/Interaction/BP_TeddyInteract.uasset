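; BP_TeddyInteract is a one-time interactable teddy that the player says goodnight to as an objective.
; It offers a "Goodnight Teddy" prompt until used, then disables itself and shows a widget playing a heart animation, with a delegate bound to the animation's finish.
; The same interaction calls TeddyDone on the objectives manager found at BeginPlay.
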(event EventBeginPlay
  (bind _returnvalue (Actor|GetActorOfClass "/Game/Blueprints/ObjectiveManager/BP_ObjectivesManager.BP_ObjectivesManager_C"))
  (Variables|Default|SetObjectivesManager _returnvalue))

(fn ConstructionScript)

(fn HandleWidget
  (CallFunction|ShowWidget)
  (bind _aswbp_heart (Utilities|Casting|CastToWBP_Heart (UserInterface|GetWidget (Variables|Default|GetWidget))))
  (LocalVariables|SetHeartWidget _aswbp_heart)
  (Utilities|FlowControl|Sequence
    (:then_0
      (Class|UserWidget|BindtoAnimationFinished (LocalVariables|GetHeartWidget) (Variables|/Game/Blueprints/UI/Tutorial/WBP_Heart.WBP_Heart_C|GetHeart (LocalVariables|GetHeartWidget)) (EventDispatchers|CreateEvent :!event HideWidget)))
    (:then_1
      (UserInterface|Animation|PlayAnimation (LocalVariables|GetHeartWidget) (Variables|/Game/Blueprints/UI/Tutorial/WBP_Heart.WBP_Heart_C|GetHeart (LocalVariables|GetHeartWidget)) 0.0 1 "Forward" 1.0 true)
      (return))))

(fn ShowWidget
  (Rendering|SetVisibility (Variables|Default|GetWidget) true false))

(fn HideWidget
  (Rendering|SetVisibility (Variables|Default|GetWidget) false false))

(fn GetInteractPrompt
  (if (Variables|Default|GetisInteractable)
    (return "Goodnight Teddy")
    (else
      (return ""))))

(fn Interact
  (if (Variables|Default|GetisInteractable)
    (Variables|Default|SetisInteractable false)
    (CallFunction|HandleWidget)
    (bind _objectivesmanager (Variables|Default|GetObjectivesManager)
      (:then
        (Default|TeddyDone _objectivesmanager)
        (return false))
      (:else))))