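; BP_Bed is an interactable bed that lets the player go to sleep once the objectives manager allows it.
; It finds BP_ObjectivesManager on BeginPlay, then each Tick refreshes its prompt and becomes interactable while CanGoToBed is set.
; The first interaction calls FirstTimeBed on the manager, and later ones start the sleep cutscene, each clearing the interactable flag.
; It also defines helpers to disable and restore player movement.
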(event EventBeginPlay
  ;[1 1 1] Begin Play
  (bind _returnvalue (Actor|GetActorOfClass "/Game/Blueprints/BP_ObjectivesManager.BP_ObjectivesManager_C"))
  (Variables|Default|SetObjectivesManager _returnvalue))

(event EventTick
  (params (DeltaSeconds :type Float%20%28single-precision%29))
  ;[1 1 1] Tick
  (CallFunction|HandleInteract)
  (bind _objectivesmanager (Variables|Default|GetObjectivesManager)
    (:then
      (if (Variables|/Game/Blueprints/BP_ObjectivesManager.BP_ObjectivesManager_C|GetCanGoToBed _objectivesmanager)
        (Variables|Default|SetisInteractable true)))
    (:else)))

(fn ConstructionScript)

(fn DisablePlayerMovement
  (Pawn|Components|CharacterMovement|DisableMovement (Variables|/Script/Engine.Character|GetCharacterMovement (Game|GetPlayerCharacter 0))))

(fn EnablePlayerMovement
  (Pawn|Components|CharacterMovement|SetMovementMode (Variables|/Script/Engine.Character|GetCharacterMovement (Game|GetPlayerCharacter 0)) "MOVE_Walking" 0))

(fn HandleInteract
  (if (Variables|Default|GetisInteractable)
    (Variables|Default|SetInteract%20Text "Go to sleep.")
    (else
      (Variables|Default|SetInteract%20Text ""))))

(fn GetInteractPrompt
  (if (Variables|Default|GetisInteractable)
    (return (Variables|Default|GetInteract%20Text))
    (else
      (return ""))))

(fn Interact
  (if (Variables|Default|GetisInteractable)
    (if (Variables|Default|GetfirstTime)
      ;[1 1 1] First time trying to sleep
      (Variables|Default|SetisInteractable false)
      (Variables|Default|SetfirstTime false)
      (Default|FirstTimeBed (Variables|Default|GetObjectivesManager))
      (return false)
      (else
        ;[1 1 1] Start sleep cutscene
        (Default|StartSleepCutscene (Variables|Default|GetObjectivesManager))
        (Variables|Default|SetisInteractable false)
        (return false)))))