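; Interactable Vincent brush pickup that shows a text popup once and relates to the find-the-portal objective.
; Interact opens the popup with a bound completion callback, then disables further interaction and clears ShouldSpawn; UpdateObjective calls FindThePortal on the objectives manager.
; ShouldSpawn saves under a construction-time GUID; BeginPlay requests a load from the game instance and destroys the actor when the flag is false.
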(event EventBeginPlay
  (bind _asbp_game_instance (Utilities|Casting|CastToBP_GameInstance (Game|GetGameInstance)))
  (Default|RequestLoad _asbp_game_instance self)
  ;[1 1 1] Get objective manager
  (bind _returnvalue (Actor|GetActorOfClass "/Game/Blueprints/ObjectiveManager/BP_ObjectivesManager.BP_ObjectivesManager_C"))
  (Variables|Default|SetObjectiveManager _returnvalue)
  ;[1 1 1] handle spawning
  (if (not (Variables|Default|GetShouldSpawn?))
    (Actor|DestroyActor)))

(event EventLoadData
  (params (SaveGameRef :type BP%20Save%20Game%20Object%20Reference))
  (bind _guid (Variables|Default|GetGuid))
  (bind _spawnableactors (Variables|/Game/Assets/Save/BP_SaveGame.BP_SaveGame_C|GetSpawnableActors SaveGameRef))
  (bind (_value _returnvalue) (Utilities|Map|Find _spawnableactors _guid))
  (if _returnvalue
    (Variables|Default|SetShouldSpawn? _value)))

(event EventSetInteractable
  (params (bIsInteractable :type Boolean)))

(event EventSaveData
  (params (SaveGameRef :type BP%20Save%20Game%20Object%20Reference))
  (Utilities|Map|Add (Variables|/Game/Assets/Save/BP_SaveGame.BP_SaveGame_C|GetSpawnableActors SaveGameRef) (Variables|Default|GetGuid) (Variables|Default|GetShouldSpawn?)))

(event EventTick
  (params (DeltaSeconds :type Float%20%28single-precision%29)))

(fn ConstructionScript
  (CallFunction|HandleGUID))

(fn HandleGUID
  (if (not (Guid|IsValidGuid (Variables|Default|GetGuid)))
    (Variables|Default|SetGuid (Guid|NewGuid))))

(fn UpdateObjective
  (bind _objectivemanager (Variables|Default|GetObjectiveManager)
    (:then
      (Default|FindthePortal _objectivemanager))
    (:else)))

(fn GetInteractPrompt
  (if (Variables|Default|GetIsInteractable)
    (return "Interact")
    (else
      (return ""))))

(fn Interact
  (if (Variables|Default|GetIsInteractable)
    (bind _returnvalue (UserInterface|CreateWidget "/Game/Blueprints/UI/Interaction/WBP_TextPopup.WBP_TextPopup_C" 0 (Variables|Default|GetFull%20Text) (Variables|Default|GetDisplay%20Name) (Variables|Default|GetUnit%20Image%20Texture)))
    (EventDispatchers|BindEventtoOnDone _returnvalue (EventDispatchers|CreateEvent :!event UpdateObjective))
    (UserInterface|Viewport|AddtoViewport _returnvalue 0)
    (Variables|Default|SetIsInteractable false)
    (Variables|Default|SetShouldSpawn? false)
    (return true)))