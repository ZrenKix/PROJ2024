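; BP_PaintingPiece is a spinning, interactable collectible that shows one of three Vincent painting images in a widget when picked up.
; Pickup updates the ObjectivesManager and saves through the game mode, though piece three skips both once the loaded piece count reaches three.
; The construction script randomises spin speed and direction.
; Spawn state persists by actor GUID, so pieces flagged to destroy after pickup remove themselves on later loads.
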(event EventBeginPlay
  (Class|BPIPersistence|RequestLoad(Message) (Game|GetGameInstance) self)
  (if (Variables|Default|GetshouldSpawn)
    (bind _returnvalue (Actor|GetActorOfClass "/Game/Blueprints/ObjectiveManager/BP_ObjectivesManager.BP_ObjectivesManager_C"))
    (Variables|Default|SetObjectivesManager _returnvalue)
    (Variables|Default|GetObjectivesManager
      (:then)
      (:else
        (Development|PrintString "No objectives manager found!" true true "(R=1.000000,G=0.961084,B=0.000000,A=1.000000)")))
    (else
      (Actor|DestroyActor))))

(event EventSaveData
  (params (SaveGameRef :type BP%20Save%20Game%20Object%20Reference))
  (Utilities|Map|Add (Variables|/Game/Assets/Save/BP_SaveGame.BP_SaveGame_C|GetPaintingPieces SaveGameRef) (Variables|Default|GetActorGuid) (Variables|Default|GetshouldSpawn)))

(event EventLoadData
  (params (SaveGameRef :type BP%20Save%20Game%20Object%20Reference))
  (bind _paintingpieces (Variables|/Game/Assets/Save/BP_SaveGame.BP_SaveGame_C|GetPaintingPieces SaveGameRef))
  (bind _actorguid (Variables|Default|GetActorGuid))
  (bind (_value _returnvalue) (Utilities|Map|Find _paintingpieces _actorguid))
  (if _returnvalue
    (Variables|Default|SetshouldSpawn _value)
    (Variables|Default|SetCurrentPieceNr (Variables|/Game/Assets/Save/BP_SaveGame.BP_SaveGame_C|GetPaintingPieceNr SaveGameRef))))

(fn ConstructionScript
  (CallFunction|RandomiseRotation))

(fn RandomiseRotation
  (Variables|/Script/Engine.RotatingMovementComponent|SetRotationRate (Variables|Default|GetRotatingMovement) (Math|Rotator|MakeRotator 0.0 0.0 (* (Math|Random|RandomFloatinRange 45.0 65.0) (Math|Integer|SelectInt -1 1 (Math|Random|RandomBool))))))

(fn GetInteractPrompt
  (if (Variables|Default|GetisInteractable)
    (return "Pick up")
    (else
      (return ""))))

(fn Interact
  (if (Variables|Default|GetisInteractable)
    (if (Variables|Default|GetDestroyAfterPickup)
      (Variables|Default|SetshouldSpawn false))
    (bind _returnvalue (UserInterface|CreateWidget "/Game/Blueprints/UI/Interaction/PaintingPieces/WBP_PaintingPiece.WBP_PaintingPiece_C"))
    (Variables|Default|SetPaintingWidget _returnvalue)
    (switch int (Variables|Default|GetPieceNr)
      (:Default)
      (:1
        (Variables|/Game/Blueprints/UI/Interaction/PaintingPieces/WBP_PaintingPiece.WBP_PaintingPiece_C|SetImage (Variables|Default|GetPaintingWidget) "/Game/Assets/VincentPainting_1.VincentPainting_1")
        (UserInterface|Viewport|AddtoViewport (Variables|Default|GetPaintingWidget) 0)
        (Default|UpdatePaintingPiece (Variables|Default|GetObjectivesManager) :!label _label)
        (bind _asbp_dreambound_game_mode (Utilities|Casting|CastToBP_DreamboundGameMode (Game|GetGameMode)))
        (Default|SaveGame _asbp_dreambound_game_mode true)
        (if (Variables|Default|GetDestroyAfterPickup)
          (Actor|DestroyActor)
          (return false)
          (else
            (return false))))
      (:2
        (Variables|/Game/Blueprints/UI/Interaction/PaintingPieces/WBP_PaintingPiece.WBP_PaintingPiece_C|SetImage (Variables|Default|GetPaintingWidget) "/Game/Assets/VincentPainting_2.VincentPainting_2")
        (UserInterface|Viewport|AddtoViewport (Variables|Default|GetPaintingWidget) 0)
        (goto _label))
      (:3
        (Variables|/Game/Blueprints/UI/Interaction/PaintingPieces/WBP_PaintingPiece.WBP_PaintingPiece_C|SetImage (Variables|Default|GetPaintingWidget) "/Game/Assets/VincentPainting_3.VincentPainting_3")
        (UserInterface|Viewport|AddtoViewport (Variables|Default|GetPaintingWidget) 0)
        (if (not (>= (Variables|Default|GetCurrentPieceNr) 3))
          (goto _label))))))