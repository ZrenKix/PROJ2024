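; Trigger-box cutscene actor that plays a level sequence once when the hero overlaps it while active.
; Playback deactivates hero movement, and the skip input jumps the sequence to its end frame.
; CutsceneFinished restores movement, reveals a portal, sets any companion following, moves listed companions to the player, then destroys the actor.
; The done flag, set only with a valid companion, saves and loads by sequence name.
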(event OnComponentBeginOverlap(Box)
  (params (OverlappedComponent :type Primitive%20Component%20Object%20Reference) (OtherActor :type Actor%20Object%20Reference) (OtherComp :type Primitive%20Component%20Object%20Reference) (OtherBodyIndex :type Integer) (bFromSweep :type Boolean) (SweepResult :type Hit%20Result%20Structure%20%28by%20ref%29))
  (bind _levelsequencer (Variables|Default|GetLevelSequencer))
  (bind _sequenceplayer (Variables|/Script/LevelSequence.LevelSequenceActor|GetSequencePlayer _levelsequencer))
  (if (not (Variables|Default|GetCutsceneDone))
    (if (Variables|Default|GetIsActive)
      (Utilities|FlowControl|DoOnce false
        (:Completed
          (bind _asbp_player_hero (Utilities|Casting|CastToBP_PlayerHero OtherActor))
          (Variables|Default|SetPlayerRef _asbp_player_hero)
          (EventDispatchers|BindEventtoOnPlay (Variables|/Script/LevelSequence.LevelSequenceActor|GetSequencePlayer (Variables|Default|GetLevelSequencer)) (delegate Custom|SetIsPlaying))
          (Sequencer|Player|Play _sequenceplayer :!class /Script/MovieScene.MovieSceneSequencePlayer)
          (Components|Activation|Deactivate (Variables|/Script/Engine.Character|GetCharacterMovement (Variables|Default|GetPlayerRef)))
          (EventDispatchers|BindEventtoOnFinished _sequenceplayer (EventDispatchers|CreateEvent :!event CutsceneFinished)))))))

(event Custom|Start%20Sequence
  (bind _levelsequencer (Variables|Default|GetLevelSequencer))
  (bind _sequenceplayer (Variables|/Script/LevelSequence.LevelSequenceActor|GetSequencePlayer _levelsequencer))
  (Utilities|FlowControl|DoOnce false
    (:Completed
      (bind _asbp_player_hero (Utilities|Casting|CastToBP_PlayerHero (stale OnComponentBeginOverlap(Box) OtherActor)))
      (Variables|Default|SetPlayerRef _asbp_player_hero)
      (EventDispatchers|BindEventtoOnPlay (Variables|/Script/LevelSequence.LevelSequenceActor|GetSequencePlayer (Variables|Default|GetLevelSequencer)) (delegate Custom|SetIsPlaying))
      (Sequencer|Player|Play _sequenceplayer :!class /Script/MovieScene.MovieSceneSequencePlayer)
      (Components|Activation|Deactivate (Variables|/Script/Engine.Character|GetCharacterMovement (Variables|Default|GetPlayerRef)))
      (EventDispatchers|BindEventtoOnFinished _sequenceplayer (EventDispatchers|CreateEvent :!event CutsceneFinished)))))

(event Custom|SetIsPlaying
  (Variables|Default|SetisPlaying true))

(event Input|EnhancedActionEvents|EnhancedInputActionIA_SkipCutscene
  (params (ActionValue :type Boolean) (ElapsedSeconds :type Float%20%28double-precision%29) (TriggeredSeconds :type Float%20%28double-precision%29) (InputAction :type Input%20Action%20Object%20Reference :default "/Game/Blueprints/Input/InputActions/IA_SkipCutscene.IA_SkipCutscene"))
  (if (Variables|Default|GetisPlaying)
    (CallFunction|SkipCutscene)))

(event EventSaveData
  (params (SaveGameRef :type BP%20Save%20Game%20Object%20Reference))
  ;[1 1 1] Save data
  (Utilities|Map|Add (Variables|/Game/Assets/Save/BP_SaveGame.BP_SaveGame_C|GetCutscenes SaveGameRef) (Utilities|GetSequenceName) (Variables|Default|GetCutsceneDone)))

(event EventLoadData
  (params (SaveGameRef :type BP%20Save%20Game%20Object%20Reference))
  ;[1 1 1] Load data
  (Variables|Default|SetCutsceneDone (.Value (Utilities|Map|Find (Variables|/Game/Assets/Save/BP_SaveGame.BP_SaveGame_C|GetCutscenes SaveGameRef) (Utilities|GetSequenceName)))))

(event EventBeginPlay
  ;[1 1 1] BeginPlay
  (Class|BPIPersistence|RequestLoad(Message) (Game|GetGameInstance) self))

(fn ConstructionScript)

(fn CutsceneFinished
  (Rendering|SetActorHiddenInGame (Variables|Default|GetPortalToOtherLevel) false)
  (Variables|Default|GetCompanion
    (:then
      (Collision|SetCollisionEnabled (Variables|Default|GetBox) "NoCollision")
      (bind _followtarget (Variables|Default|GetFollowTarget)
        (:then
          (Class|CompanionCharacter|SetFollowTarget (Variables|Default|GetCompanion) _followtarget))
        (:else
          (Class|CompanionCharacter|SetFollowTarget (Variables|Default|GetCompanion) (Game|GetPlayerCharacter 0))))
      (Variables|/Script/PROJ.CompanionCharacter|SetbCanFollow (Variables|Default|GetCompanion) true)
      (Rendering|SetActorHiddenInGame (Variables|Default|GetCompanion) false)
      (Variables|Default|SetCutsceneDone true))
    (:else
      _))
  (Components|Activation|Activate (Variables|/Script/Engine.Character|GetCharacterMovement (Variables|Default|GetPlayerRef)) false)
  (for _array_element (Variables|Default|GetCompanionsToMove)
    (Transformation|SetActorLocation _array_element (Transformation|GetActorLocation (Game|Player|GetPlayerPawn 0)) false false))
  (Actor|DestroyActor))

(fn SkipCutscene
  (bind _levelsequencer (Variables|Default|GetLevelSequencer))
  (bind _sequenceplayer (Variables|/Script/LevelSequence.LevelSequenceActor|GetSequencePlayer _levelsequencer))
  (bind _returnvalue (Class|MovieSceneSequencePlayer|GetEndTime _sequenceplayer))
  (bind (_frame _framerate _subframe) (Utilities|TimeManagement|BreakQualifiedFrameTime _returnvalue))
  (Components|Timeline|SetPlaybackPosition _sequenceplayer (Utilities|Struct|MakeMovieSceneSequencePlaybackParams (Utilities|Struct|MakeFrameTime _frame _subframe) 0.0 "" "(Hours=0,Minutes=0,Seconds=0,Frames=0,bDropFrameFormat=False)" "Frame" "Play")))