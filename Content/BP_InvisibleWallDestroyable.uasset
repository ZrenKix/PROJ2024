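; An invisible wall actor whose presence persists through save data via a ShouldSpawn flag.
; The construction script assigns a GUID when none is valid, giving the wall a key in the save game's SpawnableActors map.
; Save events write the flag to that map and load events restore it.
; BeginPlay requests a load from the game instance, then destroys the actor if the flag is false.
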(event EventBeginPlay
  (Class|BPIPersistence|RequestLoad(Message) (Game|GetGameInstance) self)
  (if (not (Variables|Default|GetShouldSpawn))
    (Actor|DestroyActor)))

(event EventSaveData
  (params (SaveGameRef :type BP%20Save%20Game%20Object%20Reference))
  (Utilities|Map|Add (Variables|/Game/Assets/Save/BP_SaveGame.BP_SaveGame_C|GetSpawnableActors SaveGameRef) (Variables|Default|GetGuid) (Variables|Default|GetShouldSpawn)))

(event EventLoadData
  (params (SaveGameRef :type BP%20Save%20Game%20Object%20Reference))
  (bind _guid (Variables|Default|GetGuid))
  (bind _spawnableactors (Variables|/Game/Assets/Save/BP_SaveGame.BP_SaveGame_C|GetSpawnableActors SaveGameRef))
  (bind (_value _returnvalue) (Utilities|Map|Find _spawnableactors _guid))
  (if _returnvalue
    (Variables|Default|SetShouldSpawn _value)))

(fn ConstructionScript
  (CallFunction|HandleGUID))

(fn HandleGUID
  (if (not (Guid|IsValidGuid (Variables|Default|GetGuid)))
    (Variables|Default|SetGuid (Guid|NewGuid))))