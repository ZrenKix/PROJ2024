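; BP_Interact is an interactable that shows a WBP_TextPopup with its text, display name and unit image.
; Interact creates the widget on every call but adds it to the viewport only while HasRan is false, then sets that flag.
; Tick watches the flag and, through a DoOnce, waits Duration before clearing it to allow another popup.
; The SetInteractable event is empty, and RerollRotator's random-rotation logic is unconnected.
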(event EventBeginPlay)

(event EventTick
  (params (DeltaSeconds :type Float%20%28single-precision%29))
  (if (Variables|Default|GetHasRan)
    (Utilities|FlowControl|DoOnce false :!label _label
      (:Completed
        (Utilities|FlowControl|Delay (Variables|Default|GetDuration))
        (Variables|Default|SetHasRan false)
        (goto _label Reset)))))

(event EventSetInteractable
  (params (bIsInteractable :type Boolean)))

(fn ConstructionScript)

(fn RerollRotator)

(fn GetInteractPrompt
  (return "Interact"))

(fn Interact
  (bind _returnvalue (UserInterface|CreateWidget "/Game/Blueprints/UI/Interaction/WBP_TextPopup.WBP_TextPopup_C" 0 (Variables|Default|GetFull%20Text) (Variables|Default|GetDisplay%20Name) (Variables|Default|GetUnit%20Image%20Texture)))
  (if (not (Variables|Default|GetHasRan))
    (Variables|Default|SetHasRan true)
    (UserInterface|Viewport|AddtoViewport _returnvalue 0)
    (return false)))